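; BP_EyeMove is an environment eye actor that turns to watch the player character and plays audio while it rotates.
; BeginPlay caches the ThirdPersonCharacter, and Tick rapidly interpolates the actor's rotation toward it using a look-at rotation.
; A looping timer samples rotation across a short delay, playing the audio from the start when it changes and stopping it when it does not.
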(event Custom|Sound
  (Variables|Default|Setrotation%20before (Transformation|GetActorRotation))
  (Utilities|FlowControl|Delay 0.1)
  (Variables|Default|Setrotation%20now (Transformation|GetActorRotation))
  (if (Utilities|Operators|EqualEqual (Variables|Default|Getrotation%20before) (Variables|Default|Getrotation%20now) 0.0)
    (Audio|Components|Audio|Stop (Variables|Default|GetAudio))
    (elif true
      (Audio|Components|Audio|Play (Variables|Default|GetAudio) 0.0))))

(event EventTick
  (params (DeltaSeconds :type Float%20%28single-precision%29))
  (Transformation|SetActorRotation (Math|Interpolation|RInterpTo (Transformation|GetActorRotation) (Math|Rotator|FindLookatRotation (Transformation|GetActorLocation) (Transformation|GetActorLocation (Variables|Default|GetCharacter))) DeltaSeconds 8e+01)))

(event EventBeginPlay
  (bind _asthird_person_character (Utilities|Casting|CastToThirdPersonCharacter (Game|GetPlayerCharacter 0)))
  (Variables|Default|SetCharacter _asthird_person_character)
  (Utilities|Time|SetTimerbyEvent (delegate Custom|Sound) 0.2 true))

(fn ConstructionScript)