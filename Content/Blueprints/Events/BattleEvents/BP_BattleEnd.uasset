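; Arena battle-end actor that tracks remaining enemies and, once none are left, opens its linked doors and clears the player's HadUlt flag.
; It then hides the HUD, disables input and plays level sequences between fade widgets, with flagged fence and meat moves plus dialogue.
; Its collision registers it as the player's LastArena, and UseUlt recounts enemies from overlaps.
; Initial counting and enemy back-reference wiring are disconnected.
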(event OnComponentBeginOverlap(arenaCollision)
  (params (OverlappedComponent :type Primitive%20Component%20Object%20Reference) (OtherActor :type Actor%20Object%20Reference) (OtherComp :type Primitive%20Component%20Object%20Reference) (OtherBodyIndex :type Integer) (bFromSweep :type Boolean) (SweepResult :type Hit%20Result%20Structure%20%28by%20ref%29))
  (bind _asthird_person_character (Utilities|Casting|CastToThirdPersonCharacter OtherActor))
  (Variables|/Game/ThirdPersonBP/Blueprints/ThirdPersonCharacter.ThirdPersonCharacter_C|SetLastArena _asthird_person_character self)
  (Development|PrintString "i am inside" true true "(R=0.000000,G=0.660000,B=1.000000,A=1.000000)" 1e+03))

(event Custom|SequencePlay
  (Development|PrintString "sequence plays" true true "(R=0.000000,G=0.660000,B=1.000000,A=1.000000)" 1002.0)
  (Utilities|FlowControl|Delay 1.0)
  (Widget|SetVisibility (Variables|/Game/ThirdPersonBP/Blueprints/ThirdPersonCharacter.ThirdPersonCharacter_C|GetInterfaceREF (Variables|Default|GetRef)) "Hidden")
  (Input|DisableInput (Variables|Default|GetRef) (Game|GetPlayerController 0))
  (bind _returnvalue (UserInterface|CreateWidget "/Game/Cinematics/W_FadeSequence.W_FadeSequence_C"))
  (UserInterface|Viewport|AddtoViewport _returnvalue 0)
  (Utilities|FlowControl|Delay 1.0)
  (Widget|RemovefromParent _returnvalue)
  (for _array_element (Variables|Default|GetsequenceToPlay)
    (bind _outactor (Sequencer|Player|CreateLevelSequencePlayer _array_element))
    (Sequencer|Player|Play (Variables|/Script/LevelSequence.LevelSequenceActor|GetSequencePlayer _outactor) :!class /Script/MovieScene.MovieSceneSequencePlayer)
    (Utilities|FlowControl|Delay 4.0)
    (bind _returnvalue_2 (UserInterface|CreateWidget "/Game/Cinematics/W_FadeSequence.W_FadeSequence_C"))
    (UserInterface|Viewport|AddtoViewport _returnvalue_2 0)
    (Utilities|FlowControl|Delay 1.0)
    (Input|EnableInput (Variables|Default|GetRef) (Game|GetPlayerController 0))
    (Widget|SetVisibility (Variables|/Game/ThirdPersonBP/Blueprints/ThirdPersonCharacter.ThirdPersonCharacter_C|GetInterfaceREF (Variables|Default|GetRef)) "Hidden")
    (if (Variables|Default|GetDoorMoved?)
      (if (Variables|Default|GetMeatMoved?)
        (if (not (Variables|Default|GetOranTalk?))
          (bind _returnvalue_3 (AddComponent|AddDialogueComponent))
          (Class|IInteraction|Talk(Message) _returnvalue_3))
        (else
          (Variables|Default|SetMeatMoved? true)
          (bind _returnvalue_4 (Actor|GetActorOfClass "/Game/Cinematics/SequencesFightScene/BP_Meat.BP_Meat_C"))
          (Transformation|SetActorLocation _returnvalue_4 "2089.667969,5910.800293,-1861.583618" false false)))
      (else
        (Variables|Default|SetDoorMoved? true)
        (bind _returnvalue_5 (Actor|GetActorOfClass "/Game/Cinematics/SequencesFightScene/BP_Fence.BP_Fence_C"))
        (Transformation|SetActorRotation _returnvalue_5 "0,-165.165756, 0")
        (bind _returnvalue_6 (AddComponent|AddDialogueComponent))
        (Class|IInteraction|Talk(Message) _returnvalue_6)))))

(event Custom|MinusEnemy
  (Math|Integer|DecrementInt (Variables|Default|GetenemiesAmount)
    (:%20%20
      (if (<= (Variables|Default|GetenemiesAmount) 0)
        (CallFunction|OpenDoor)
        (CallFunction|SequencePlay)
        (Variables|/Game/ThirdPersonBP/Blueprints/ThirdPersonCharacter.ThirdPersonCharacter_C|SetHadUlt (Variables|Default|GetRef) false)))))

(event Custom|OpenDoor
  (for _array_element (Variables|Default|GetdoorsToOpen)
    (Default|OpenDoor _array_element)))

(event EventBeginPlay
  (bind _asthird_person_character (Utilities|Casting|CastToThirdPersonCharacter (Game|GetPlayerCharacter 0)))
  (Variables|Default|SetRef _asthird_person_character))

(event EventUseUlt
  (bind _output_get (Variables|Default|SetenemiesAmount (Utilities|Array|Length (Collision|GetOverlappingActors (Variables|Default|GetarenaCollision) "/Game/Blueprints/Enemies/BaseEnemy/BP_BaseEnemy.BP_BaseEnemy_C" :!class /Script/Engine.PrimitiveComponent))))
  (Development|PrintString (Utilities|String|ToString(Integer) _output_get) true true "(R=0.000000,G=0.660000,B=1.000000,A=1.000000)" 1e+03))

(fn ConstructionScript)