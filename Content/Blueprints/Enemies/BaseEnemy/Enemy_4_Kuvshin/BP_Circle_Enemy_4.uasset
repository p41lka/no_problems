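; Telegraphed lightning area attack for Enemy 4 (Kuvshin) that runs on spawn and damages everything in its radius except BaseEnemy actors.
; A first timeline scales the whole actor with a lightning effect.
; After a short pause, a second timeline scales the flat cylinder as a warning indicator, with play rate derived from DelayTime.
; When it finishes, the actor applies full radial damage at the arrow's location, spawns an explosion effect and destroys itself.
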(event Custom|Explosion
  (Effects|SpawnEmitteratLocation "/Game/VFX/Stylized_FX_Collection_02/ParticleSystem/StylizedFX_05/Lightning_Shot/P_LightningShot_02.P_LightningShot_02" (Transformation|GetActorLocation) "0, 0, 0" "0.500000,0.500000,0.500000")
  (bind _newtrack_1 (Timeline|Timeline_1 PlayFromStart)
    (:Update
      (Transformation|SetActorScale3D (Math|Vector|MakeVector _newtrack_1 _newtrack_1 _newtrack_1)))
    (:Finished
      (Utilities|FlowControl|Delay 0.2)
      (Components|Timeline|SetPlayRate (Variables|Default|GetTimeline_0) (/ 1.0 (Variables|Default|GetDelayTime)))
      (bind _newtrack_1_2 (Timeline|Timeline_0 PlayFromStart)
        (:Update
          (Transformation|SetWorldScale3D (Variables|Default|GetCylinder) (Math|Vector|MakeVector _newtrack_1_2 _newtrack_1_2 0.1)))
        (:Finished
          (bind _outactors (Actor|GetAllActorsOfClass "/Game/Blueprints/Enemies/BaseEnemy/BP_BaseEnemy.BP_BaseEnemy_C"))
          (Game|Damage|ApplyRadialDamage (Variables|Default|GetDamage) (Transformation|GetWorldLocation (Variables|Default|GetArrow)) 2.5e+02 0 _outactors self 0 true "ECC_Visibility")
          (Effects|SpawnEmitteratLocation "/Game/VFX/Stylized_FX_Collection_02/ParticleSystem/StylizedFX_05/Lightning_Shot/P_LightningBall_Explosion_02.P_LightningBall_Explosion_02" (Transformation|GetActorLocation))
          (Actor|DestroyActor))))))

(event EventBeginPlay
  (CallFunction|Explosion)
  (Transformation|SetWorldScale3D (Variables|Default|GetCylinder) "0, 0, 0"))

(fn ConstructionScript)