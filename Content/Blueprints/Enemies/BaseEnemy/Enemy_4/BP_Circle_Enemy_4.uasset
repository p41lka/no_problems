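; BP_Circle_Enemy_4 is a telegraphed area attack for Enemy 4 that starts its explosion sequence as soon as it spawns.
; After a delay, it switches its cylinder to the enemy emissive material as a warning, then waits the same delay again.
; It then applies full radial damage at the arrow's location, ignoring all BP_BaseEnemy actors, spawns a lightning slash Niagara effect, and destroys itself.
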(event Custom|Explosion
  (bind _delaytime (Variables|Default|GetDelayTime))
  (Utilities|FlowControl|Delay _delaytime)
  (Rendering|Material|SetMaterial (Variables|Default|GetCylinder) 0 "/Game/Materials/M_Enemies/M_Emissive_Enemy.M_Emissive_Enemy")
  (Utilities|FlowControl|Delay _delaytime)
  (bind _outactors (Actor|GetAllActorsOfClass "/Game/Blueprints/Enemies/BaseEnemy/BP_BaseEnemy.BP_BaseEnemy_C"))
  (Game|Damage|ApplyRadialDamage (Variables|Default|GetDamage) (Transformation|GetWorldLocation (Variables|Default|GetArrow)) 5e+02 0 _outactors self 0 true "ECC_Visibility")
  (Niagara|SpawnSystematLocation "/Game/VFX/Hack_And_Slash_FX/VFX_Niagara/Slashes/NS_Lightning_Slash.NS_Lightning_Slash" (Transformation|GetActorLocation))
  (Utilities|FlowControl|Delay 0.2)
  (Actor|DestroyActor))

(event EventBeginPlay
  (CallFunction|Explosion))

(fn ConstructionScript)