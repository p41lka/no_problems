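; BP_Enemy_4_Projectile_2 is an Enemy 4 projectile that leaves a BP_Circle_Enemy_4 where it lands.
; When projectile movement stops, it destroys itself if it hit a BP_BaseEnemy.
; Otherwise it spawns the circle at the impact location and passes EnemyDamage to it, without destroying itself in this graph.
; A BP_AttackProjectile overlapping Sphere1 also destroys it, so it can be shot down.
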(event OnComponentBeginOverlap(Sphere1)
  (params (OverlappedComponent :type Primitive%20Component%20Object%20Reference) (OtherActor :type Actor%20Object%20Reference) (OtherComp :type Primitive%20Component%20Object%20Reference) (OtherBodyIndex :type Integer) (bFromSweep :type Boolean) (SweepResult :type Hit%20Result%20Structure%20%28by%20ref%29))
  (Utilities|Casting|CastToBP_AttackProjectile OtherActor)
  (Actor|DestroyActor))

(event OnProjectileStop(ProjectileMovement)
  (params (ImpactResult :type Hit%20Result%20Structure%20%28by%20ref%29))
  (bind (_bblockinghit _binitialoverlap _time _distance _location _impactpoint _normal _impactnormal _physmat _hitactor) (Collision|BreakHitResult ImpactResult))
  (Utilities|Casting|CastToBP_BaseEnemy _hitactor
    (:then
      (Actor|DestroyActor))
    (:CastFailed
      (bind _returnvalue (Game|SpawnActorfromClass "/Game/Blueprints/Enemies/BaseEnemy/Enemy_4/BP_Circle_Enemy_4.BP_Circle_Enemy_4_C" (Math|Transform|MakeTransform _location "0, 0, 0" "1.000000,1.000000,1.000000") "Undefined" 0 0))
      ;[0 0 0] Set circle Damage
      (Variables|/Game/Blueprints/Enemies/BaseEnemy/Enemy_4/BP_Circle_Enemy_4.BP_Circle_Enemy_4_C|SetDamage _returnvalue (Variables|Default|GetEnemyDamage)))))

(event EventBeginPlay
  (|CallParentFunction) ; This node is disabled and will not be called.\nDrag off pins to build functionality.
)

(fn ConstructionScript
  (|CallParentFunction))