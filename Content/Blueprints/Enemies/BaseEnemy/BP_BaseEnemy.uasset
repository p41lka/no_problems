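; Base enemy Blueprint with a health bar widget, a brief hit stun and a BP_Capsule spawn on death.
; Overlapping BP_AttackProjectile actors apply fixed damage to it, attributed to the player character, and are destroyed.
; Damage updates health and the widget, then either triggers death or plays a lightning impact effect and disables movement for StanTime.
; The logic initializing current health and widget values from MaxHealth is unconnected and never runs.
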(event OnComponentBeginOverlap(CapsuleComponent)
  (params (OverlappedComponent :type Primitive%20Component%20Object%20Reference) (OtherActor :type Actor%20Object%20Reference) (OtherComp :type Primitive%20Component%20Object%20Reference) (OtherBodyIndex :type Integer) (bFromSweep :type Boolean) (SweepResult :type Hit%20Result%20Structure%20%28by%20ref%29))
  (bind _asbp_attack_projectile (Utilities|Casting|CastToBP_AttackProjectile OtherActor))
  (Game|Damage|ApplyDamage self 1e+01 0 (Variables|Default|GetCharacterREF))
  (Actor|DestroyActor _asbp_attack_projectile))

(event Custom|Death
  (Game|SpawnActorfromClass "/Game/Blueprints/Capsules/BP_Capsule.BP_Capsule_C" (Math|Transform|MakeTransform (Transformation|GetActorLocation) "0, 0, 0" "1.000000,1.000000,1.000000") "AlwaysSpawn" 0 0)
  (Actor|DestroyActor))

(event EventBeginPlay
  (bind _asthird_person_character (Utilities|Casting|CastToThirdPersonCharacter (Game|GetPlayerCharacter 0)))
  (Variables|Default|SetCharacterREF _asthird_person_character)
  (bind _asw_enemy_health (Utilities|Casting|CastToW_EnemyHealth (UserInterface|GetUserWidgetObject (Variables|Default|GetHealthBar))))
  (Variables|Default|SetEnemyUIREF _asw_enemy_health))

(event Game|Damage|EventAnyDamage
  (params (Damage :type Float%20%28single-precision%29) (DamageType :type Damage%20Type%20Object%20Reference) (InstigatedBy :type Controller%20Object%20Reference) (DamageCauser :type Actor%20Object%20Reference))
  (bind _charactermovement (Variables|Character|GetCharacterMovement))
  (bind _output_get (Variables|Default|SetCurrentHealth (- (Variables|Default|GetCurrentHealth) Damage)))
  (Variables|/Game/Widgets/W_EnemyHealth.W_EnemyHealth_C|SetCurrentHealthUI (Variables|Default|GetEnemyUIREF) _output_get)
  (if (<= _output_get 0.0)
    (CallFunction|Death)
    (else
      ;[0 0 0] Stan
      (Pawn|Components|CharacterMovement|DisableMovement _charactermovement)
      (Niagara|SpawnSystematLocation "/Game/VFX/Hack_And_Slash_FX/VFX_Niagara/Impacts/NS_Lightning_Slash_Impact_2.NS_Lightning_Slash_Impact_2" (Transformation|GetActorLocation))
      (Utilities|FlowControl|Delay (Variables|Default|GetStanTime))
      (Pawn|Components|CharacterMovement|SetMovementMode _charactermovement "MOVE_Walking" 0))))

(fn ConstructionScript)

(fn IsGeneratorReloading
  (params (IsReloading :type Boolean))
  (return false))