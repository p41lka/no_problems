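; Grom enemy that absorbs damage as a visible charge and performs a dash attack.
; Hits briefly halt movement, swap body materials by remaining health, light emissive slots by accumulated damage and add to the GromDamage Blackboard value.
; Dash plays a wind-up, resets both damage counters, then timeline-lerps to a forward trace's player hit or endpoint, clearing the glow on landing.
; A separate Attack event applies damage directly to the player.
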(event Custom|Dash
  (bind _returnvalue (Transformation|GetActorLocation))
  (bind _runemitter (Variables|Default|GetRunEmitter))
  ;[0 0 0] Dash
  (if (not (Variables|Default|GetIsAttacking))
    (Animation|Montage|PlayMontage (Variables|Character|GetMesh) "/Game/Animations/Enemies/6_Grom/Grom_Before_Montage.Grom_Before_Montage"
      (:then
        (Components|Activation|SetActive _runemitter true false))
      (:OnCompleted
        (Components|Activation|Deactivate _runemitter :!label _label)
        (Variables|Default|SetIsAttacking true)
        (Variables|Default|SetCurrentDamageEaten 0.0)
        (AI|Components|Blackboard|SetValueasFloat (AI|GetBlackboard (Pawn|GetController)) (Utilities|Name|MakeLiteralName "GromDamage") 0.0)
        (Variables|Dash|SetStartDashPosition _returnvalue)
        (bind _outhit (Collision|LineTraceByChannel _returnvalue (+ _returnvalue (* (Transformation|GetActorForwardVector) (Variables|Dash|GetDashDistance))) "TraceTypeQuery1" false 0 "None"))
        (if (.bBlockingHit (Collision|BreakHitResult _outhit))
          (Utilities|Casting|CastToThirdPersonCharacter (.HitActor (Collision|BreakHitResult _outhit))
            (:then
              (Variables|Dash|SetEndDashPosition (.Location (Collision|BreakHitResult _outhit))))
            (:CastFailed
              (Variables|Dash|SetEndDashPosition (.TraceEnd (Collision|BreakHitResult _outhit)) :!label _label_2)))
          (else
            (goto _label_2)))
        (Components|Timeline|SetPlayRate (Variables|Default|GetDash_timeline) (/ 1.0 (Variables|Dash|GetDashDuration)))
        (Pawn|Components|CharacterMovement|DisableMovement (Variables|Character|GetCharacterMovement))
        (Animation|Montage|PlayMontage (Variables|Character|GetMesh) "/Game/Animations/Enemies/6_Grom/Grom_Attack_Anim_Montage.Grom_Attack_Anim_Montage"
          (:then
            (Rendering|SetVisibility (Variables|Default|GetDashEmitter) true false)
            (bind _alpha (Timeline|Dash_Timeline PlayFromStart)
              (:Update
                (Transformation|SetActorLocation (Math|Vector|Lerp(Vector) (Variables|Dash|GetStartDashPosition) (Variables|Dash|GetEndDashPosition) _alpha) false false))
              (:Finished
                (Effects|SpawnEmitteratLocation "/Game/VFX/Stylized_FX_Collection_02/ParticleSystem/StylizedFX_04/LandBullet/P_Land_Hit.P_Land_Hit" (Transformation|GetWorldLocation (Variables|Default|GetArrow1)) (Transformation|GetActorRotation))
                (Rendering|SetVisibility (Variables|Default|GetDashEmitter) false false)
                (CallFunction|CleanDamage)
                (Utilities|FlowControl|Delay 0.4)
                (Variables|Default|SetIsAttacking false)
                (Pawn|Components|CharacterMovement|SetMovementMode (Variables|Character|GetCharacterMovement) "MOVE_Walking" 0))))))
      (:OnBlendOut
        (goto _label)))))

(event Custom|Attack
  ;[0 0 0] Attack
  (Game|Damage|ApplyDamage (Game|GetPlayerCharacter 0) (Utilities|Struct|BreakEnemyInfo_Struct (Variables|Default|GetEnemyInfo_Struct)) 0 self))

(event Custom|CheckDamage
  (bind _mesh (Variables|Character|GetMesh))
  (bind _currentdamageeaten (Variables|Default|GetCurrentDamageEaten))
  (bind _mesh_2 (Variables|Character|GetMesh))
  (bind _currentdamageeaten_2 (Variables|Default|GetCurrentDamageEaten))
  ;[0 0 0] Charge
  (if (>= _currentdamageeaten (Variables|Default|GetMaxDamageEaten))
    (Rendering|Material|SetMaterial _mesh 1 "/Game/Materials/M_Enemies/M_Emissive_Blue_Enemy.M_Emissive_Blue_Enemy")
    (elif (>= _currentdamageeaten 3e+01)
      (Rendering|Material|SetMaterial _mesh 2 "/Game/Materials/M_Enemies/M_Emissive_Blue_Enemy.M_Emissive_Blue_Enemy")
      (elif (>= _currentdamageeaten_2 2e+01)
        (Rendering|Material|SetMaterial _mesh_2 3 "/Game/Materials/M_Enemies/M_Emissive_Blue_Enemy.M_Emissive_Blue_Enemy")
        (elif (>= _currentdamageeaten_2 1e+01)
          (Rendering|Material|SetMaterial _mesh_2 4 "/Game/Materials/M_Enemies/M_Emissive_Blue_Enemy.M_Emissive_Blue_Enemy"))))))

(event Custom|CleanDamage
  (bind _mesh (Variables|Character|GetMesh))
  ;[0 0 0] Charge
  (Rendering|Material|SetMaterial _mesh 1 "/Game/Materials/M_Enemies/MI_GrayEnemy.MI_GrayEnemy")
  (Rendering|Material|SetMaterial _mesh 2 "/Game/Materials/M_Enemies/MI_GrayEnemy.MI_GrayEnemy")
  (Rendering|Material|SetMaterial _mesh 3 "/Game/Materials/M_Enemies/MI_GrayEnemy.MI_GrayEnemy")
  (Rendering|Material|SetMaterial _mesh 4 "/Game/Materials/M_Enemies/MI_GrayEnemy.MI_GrayEnemy"))

(event EventBeginPlay
  (bind _enemyinfo_struct (Variables|Default|GetEnemyInfo_Struct))
  (bind _enemyuiref (Variables|Default|GetEnemyUIREF))
  (bind (_maxhealth _maxspeed) (Utilities|Struct|BreakEnemyInfo_Struct _enemyinfo_struct))
  (|CallParentFunction)
  (Variables|/Script/Engine.CharacterMovementComponent|SetMaxWalkSpeed (Variables|Character|GetCharacterMovement) _maxspeed)
  (bind _output_get (Variables|Default|SetCurrentHealth _maxhealth))
  (bind _output_get_2 (Variables|/Game/Widgets/W_EnemyHealth.W_EnemyHealth_C|SetCurrentHealthUI _enemyuiref _output_get))
  (Variables|/Game/Widgets/W_EnemyHealth.W_EnemyHealth_C|SetMaxHealthUI _enemyuiref _output_get_2))

(event Game|Damage|EventAnyDamage
  (params (Damage :type Float%20%28single-precision%29) (DamageType :type Damage%20Type%20Object%20Reference) (InstigatedBy :type Controller%20Object%20Reference) (DamageCauser :type Actor%20Object%20Reference))
  (bind _returnvalue (Pawn|GetController))
  (bind _returnvalue_2 (Utilities|Name|MakeLiteralName "GromDamage"))
  (bind _currenthealth (Variables|Default|GetCurrentHealth))
  (bind _charactermovement (Variables|Character|GetCharacterMovement))
  (bind _mesh (Variables|Character|GetMesh))
  (bind _enemyinfo_struct (Variables|Default|GetEnemyInfo_Struct))
  (bind _maxhealth (Utilities|Struct|BreakEnemyInfo_Struct _enemyinfo_struct))
  (bind _returnvalue_3 (AI|GetBlackboard _returnvalue))
  (bind _returnvalue_4 (/ _currenthealth _maxhealth))
  ;[0 0 0] Damage
  (Variables|Default|SetCurrentDamageEaten (+ Damage (Variables|Default|GetCurrentDamageEaten)))
  (CallFunction|CheckDamage)
  (|CallParentFunction Damage DamageType InstigatedBy DamageCauser)
  (Utilities|IsValid self
    (:Is%20Valid
      (Pawn|Components|CharacterMovement|DisableMovement _charactermovement)
      (Animation|Montage|PlayMontage (Variables|Character|GetMesh) "/Game/Animations/Enemies/6_Grom/Grom_Damage_Anim_Montage.Grom_Damage_Anim_Montage"
        (:then
          (AI|Components|Blackboard|SetValueasFloat _returnvalue_3 _returnvalue_2 (+ (Class|BlackboardComponent|GetValueasFloat _returnvalue_3 _returnvalue_2) Damage))
          ;[0 0 0] Damage material
          (CallFunction|Splatter 5e+01)
          (if (<= _returnvalue_4 0.25)
            (Rendering|Material|SetMaterial _mesh 0 "/Game/Materials/M_Enemy_Damage/Grom/MI_Grom_3.MI_Grom_3")
            (elif (<= _returnvalue_4 0.5)
              (Rendering|Material|SetMaterial _mesh 0 "/Game/Materials/M_Enemy_Damage/Grom/MI_Grom_2.MI_Grom_2")
              (elif (<= _returnvalue_4 0.75)
                (Rendering|Material|SetMaterial _mesh 0 "/Game/Materials/M_Enemy_Damage/Grom/MI_Grom_1.MI_Grom_1")))))
        (:OnCompleted
          (Pawn|Components|CharacterMovement|SetMovementMode _charactermovement "MOVE_Walking" 0))))))

(event EventDeath
  (|CallParentFunction)
  (Audio|PlaySoundatLocation "/Game/Sound/Grom/Death/C_Grom_Death.C_Grom_Death" (Transformation|GetActorLocation) "0, 0, 0" 1.0 1.0 0.0 0 0 0 0))

(fn ConstructionScript
  (|CallParentFunction))