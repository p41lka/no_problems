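; Turret enemy that faces the player every tick and alternates attack waves with hiding and relocating.
; Each attack plays a montage and reloads; after the maximum waves, timelines move the mesh to hide it, then reveal it at a random reachable point near the player.
; It is invulnerable while hidden, and damage plays a reaction montage before resuming the cycle.
; The timer driving the ammo countdown is disconnected.
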(event Custom|Hide
  (bind _mesh (Variables|Character|GetMesh))
  (bind _relativelocation (Variables|/Script/Engine.SceneComponent|GetRelativeLocation _mesh))
  ;[0 0 0] Hide
  (Utilities|FlowControl|Delay (Variables|Default|GetBeforeHidingPauseTime))
  (Variables|Default|SetCanBeDamaged false)
  (Variables|/Script/Engine.PrimitiveComponent|SetbGenerateOverlapEvents (Variables|Default|GetCapsuleComponent) false)
  (Rendering|SetVisibility (Variables|Default|GetHealthBar) false true)
  (bind _newtrack_0 (Timeline|Timeline_0 PlayFromStart)
    (:Update
      (Transformation|SetRelativeLocation _mesh (Math|Vector|MakeVector (.x _relativelocation) (.y _relativelocation) _newtrack_0) false false))
    (:Finished
      (Utilities|FlowControl|Delay (Variables|Default|GetHidingTime))
      (CallFunction|Unhide))))

(event Custom|Attack
  ;[0 0 0] Spawn Projectiles
  (Math|Integer|IncrementInt (Variables|Default|GetCurrentWave)
    (:%20%20
      (Animation|Montage|PlayMontage (Variables|Character|GetMesh) "/Game/Animations/Enemies/2_Turrel/Turrel_Attack_Anim_Montage.Turrel_Attack_Anim_Montage"
        (:OnCompleted
          (CallFunction|Reload))))))

(event Custom|AttackSpawn
  ;[1 1 1] previous timer
  (if (> (Variables|Default|GetCurrentAmmoInWave) 0)
    (Math|Integer|DecrementInt (Variables|Default|GetCurrentAmmoInWave))))

(event Custom|Reload
  ;[0 0 0] Reload and set waves
  (Utilities|FlowControl|Delay (Variables|Default|GetReloadTime))
  (if (< (Variables|Default|GetCurrentWave) (Variables|Default|GetMaxWaves))
    (CallFunction|Attack)
    (else
      (CallFunction|Hide))))

(event Custom|Unhide
  (bind _returnvalue (Game|GetPlayerCharacter 0))
  (bind _mesh (Variables|Character|GetMesh))
  (bind _radius (Variables|Default|GetRadius))
  (bind _returnvalue_2 (Transformation|GetActorLocation _returnvalue))
  (bind _relativelocation (Variables|/Script/Engine.SceneComponent|GetRelativeLocation _mesh))
  (bind _randomlocation (AI|Navigation|GetRandomReachablePointinRadius _returnvalue_2 _radius 0 0))
  ;[0 0 0] Unhide
  (Transformation|SetActorLocation (Math|Vector|MakeVector (.x _randomlocation) (.y _randomlocation) (.z (Transformation|GetActorLocation))) false true)
  (bind _newtrack_0 (Timeline|Timeline_1 ReverseFromEnd)
    (:Update
      (Transformation|SetRelativeLocation _mesh (Math|Vector|MakeVector (.x _relativelocation) (.y _relativelocation) _newtrack_0) false false))
    (:Finished
      (Variables|Default|SetCanBeDamaged true)
      (Rendering|SetVisibility (Variables|Default|GetHealthBar) true true)
      (Utilities|FlowControl|Delay (Variables|Default|GetBeforeAttackPauseTime))
      (Variables|Default|SetCurrentWave 0)
      (Variables|/Script/Engine.PrimitiveComponent|SetbGenerateOverlapEvents (Variables|Default|GetCapsuleComponent) true)
      (CallFunction|Attack))))

(event EventBeginPlay
  (bind _enemyinfo_struct (Variables|Default|GetEnemyInfo_Struct))
  (bind _enemyuiref (Variables|Default|GetEnemyUIREF))
  (bind (_maxhealth _maxspeed) (Utilities|Struct|BreakEnemyInfo_Struct _enemyinfo_struct))
  (|CallParentFunction)
  (Variables|/Script/Engine.CharacterMovementComponent|SetMaxWalkSpeed (Variables|Character|GetCharacterMovement) _maxspeed)
  (bind _output_get (Variables|Default|SetCurrentHealth _maxhealth))
  (bind _output_get_2 (Variables|/Game/Widgets/W_EnemyHealth.W_EnemyHealth_C|SetCurrentHealthUI _enemyuiref _output_get))
  (Variables|/Game/Widgets/W_EnemyHealth.W_EnemyHealth_C|SetMaxHealthUI _enemyuiref _output_get_2)
  (Variables|Default|SetCurrentAmmoInWave (Variables|Default|GetMaxAmmoInWave))
  (CallFunction|Attack))

(event EventTick
  (params (DeltaSeconds :type Float%20%28single-precision%29))
  ;[0 0 0] Rotation
  (Transformation|SetActorRotation (Math|Rotator|MakeRotator 0.0 0.0 (.yaw (Math|Rotator|FindLookatRotation (Transformation|GetActorLocation) (Transformation|GetWorldLocation (Variables|/Script/Engine.Character|GetMesh (Game|GetPlayerCharacter 0))))))))

(event Game|Damage|EventAnyDamage
  (params (Damage :type Float%20%28single-precision%29) (DamageType :type Damage%20Type%20Object%20Reference) (InstigatedBy :type Controller%20Object%20Reference) (DamageCauser :type Actor%20Object%20Reference))
  ;[0 0 0] EventDamage
  (if (Variables|Default|GetCanBeDamaged)
    (|CallParentFunction Damage DamageType InstigatedBy DamageCauser)
    (Animation|Montage|PlayMontage (Variables|Character|GetMesh) "/Game/Animations/Enemies/2_Turrel/Turrel_Damage_Anim_Montage.Turrel_Damage_Anim_Montage"
      (:OnCompleted
        (if (< (Variables|Default|GetCurrentWave) (Variables|Default|GetMaxWaves))
          (CallFunction|Attack)
          (else
            (CallFunction|Reload)))))))

(fn ConstructionScript
  (|CallParentFunction))