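; BP_Enemy_1 is the Imp enemy, a child of a base enemy that attacks by firing projectiles.
; BeginPlay applies max speed and health from EnemyInfoStruct to movement and the enemy UI.
; Attack starts a looping timer that spawns a scaled-down projectile at ProjectilesSpawn and passes it the struct's damage.
; Damage disables movement while the hit montage plays, restoring walking when it completes.
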(event Custom|Attack
  ;[0 0 0] Spawn Projectiles
  (bind _returnvalue (Utilities|Time|SetTimerbyEvent (delegate Custom|PassiveAttackSpawn) (Utilities|Struct|BreakEnemyInfo_Struct (Variables|Default|GetEnemyInfo_Struct)) true))
  (Variables|Default|SetAttackTimer _returnvalue))

(event Custom|PassiveAttackSpawn
  (bind _projectilesspawn (Variables|Default|GetProjectilesSpawn))
  ;[0 0 0] Spawn Projectiles
  (bind _returnvalue (Game|SpawnActorfromClass "/Game/Blueprints/Enemies/BaseEnemy/Enemy_1_Imp/BP_Enemy_1_Projectile.BP_Enemy_1_Projectile_C" (Math|Transform|MakeTransform (Transformation|GetWorldLocation _projectilesspawn) (Transformation|GetWorldRotation _projectilesspawn) "0.200000,0.200000,0.200000") "Undefined" 0 0))
  ;[0 0 0] Set projectile Damage
  (Variables|/Game/Blueprints/Enemies/BaseEnemy/BP_EnemyProjectiles.BP_EnemyProjectiles_C|SetEnemyDamage _returnvalue (Utilities|Struct|BreakEnemyInfo_Struct (Variables|Default|GetEnemyInfo_Struct))))

(event EventBeginPlay
  (bind _enemyinfo_struct (Variables|Default|GetEnemyInfo_Struct))
  (bind _enemyuiref (Variables|Default|GetEnemyUIREF))
  (bind (_maxhealth _maxspeed) (Utilities|Struct|BreakEnemyInfo_Struct _enemyinfo_struct))
  (|CallParentFunction)
  (Variables|/Script/Engine.CharacterMovementComponent|SetMaxWalkSpeed (Variables|Character|GetCharacterMovement) _maxspeed)
  (bind _output_get (Variables|Default|SetCurrentHealth _maxhealth))
  (bind _output_get_2 (Variables|/Game/Widgets/W_EnemyHealth.W_EnemyHealth_C|SetCurrentHealthUI _enemyuiref _output_get))
  (Variables|/Game/Widgets/W_EnemyHealth.W_EnemyHealth_C|SetMaxHealthUI _enemyuiref _output_get_2))

(event EventDamage
  (bind _charactermovement (Variables|Character|GetCharacterMovement))
  (|CallParentFunction)
  (Pawn|Components|CharacterMovement|DisableMovement _charactermovement)
  (Animation|Montage|PlayMontage (Variables|Character|GetMesh) "/Game/Animations/Enemies/1_Imp/Imp_Damage_Anim_Montage.Imp_Damage_Anim_Montage"
    (:OnCompleted
      (Pawn|Components|CharacterMovement|SetMovementMode _charactermovement "MOVE_Walking" 0))))

(fn ConstructionScript
  (|CallParentFunction))