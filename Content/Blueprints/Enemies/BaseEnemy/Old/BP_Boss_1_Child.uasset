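; Boss enemy that cycles a tentacle slam with radial damage, minion spawning and a tentacle spin on a delay loop.
; It tracks health in the enemy UI and dies at zero.
; Faith, Destruction and Renewal boxes rotate while the player is inside the sphere.
; Standing in a box while not using an ability runs a looping resonance timer that grants that aspect's ability when full, resetting on exit.
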(event OnComponentBeginOverlap(Faith_Box)
  (params (OverlappedComponent :type Primitive%20Component%20Object%20Reference) (OtherActor :type Actor%20Object%20Reference) (OtherComp :type Primitive%20Component%20Object%20Reference) (OtherBodyIndex :type Integer) (bFromSweep :type Boolean) (SweepResult :type Hit%20Result%20Structure%20%28by%20ref%29))
  ;[0 0 0] Faith
  (bind _asthird_person_character (Utilities|Casting|CastToThirdPersonCharacter OtherActor))
  (if (not (Variables|/Game/ThirdPersonBP/Blueprints/ThirdPersonCharacter.ThirdPersonCharacter_C|GetIsUsingAbility _asthird_person_character))
    (CallFunction|Overlap "NewEnumerator0")
    (CallFunction|StartResonating)))

(event OnComponentEndOverlap(Faith_Box)
  (params (OverlappedComponent :type Primitive%20Component%20Object%20Reference) (OtherActor :type Actor%20Object%20Reference) (OtherComp :type Primitive%20Component%20Object%20Reference) (OtherBodyIndex :type Integer))
  ;[0 0 0] Faith
  (Utilities|Casting|CastToThirdPersonCharacter OtherActor)
  (CallFunction|EndResonating))

(event OnComponentBeginOverlap(Destruction_Box)
  (params (OverlappedComponent :type Primitive%20Component%20Object%20Reference) (OtherActor :type Actor%20Object%20Reference) (OtherComp :type Primitive%20Component%20Object%20Reference) (OtherBodyIndex :type Integer) (bFromSweep :type Boolean) (SweepResult :type Hit%20Result%20Structure%20%28by%20ref%29))
  ;[0 0 0] Destruction
  (bind _asthird_person_character (Utilities|Casting|CastToThirdPersonCharacter OtherActor))
  (if (not (Variables|/Game/ThirdPersonBP/Blueprints/ThirdPersonCharacter.ThirdPersonCharacter_C|GetIsUsingAbility _asthird_person_character))
    (CallFunction|Overlap "NewEnumerator1")
    (CallFunction|StartResonating)))

(event OnComponentEndOverlap(Destruction_Box)
  (params (OverlappedComponent :type Primitive%20Component%20Object%20Reference) (OtherActor :type Actor%20Object%20Reference) (OtherComp :type Primitive%20Component%20Object%20Reference) (OtherBodyIndex :type Integer))
  ;[0 0 0] Destruction
  (Utilities|Casting|CastToThirdPersonCharacter OtherActor)
  (CallFunction|EndResonating))

(event OnComponentBeginOverlap(Renewal_Box)
  (params (OverlappedComponent :type Primitive%20Component%20Object%20Reference) (OtherActor :type Actor%20Object%20Reference) (OtherComp :type Primitive%20Component%20Object%20Reference) (OtherBodyIndex :type Integer) (bFromSweep :type Boolean) (SweepResult :type Hit%20Result%20Structure%20%28by%20ref%29))
  ;[0 0 0] Renewal
  (bind _asthird_person_character (Utilities|Casting|CastToThirdPersonCharacter OtherActor))
  (if (not (Variables|/Game/ThirdPersonBP/Blueprints/ThirdPersonCharacter.ThirdPersonCharacter_C|GetIsUsingAbility _asthird_person_character))
    (CallFunction|Overlap "NewEnumerator3")
    (CallFunction|StartResonating)))

(event OnComponentEndOverlap(Renewal_Box)
  (params (OverlappedComponent :type Primitive%20Component%20Object%20Reference) (OtherActor :type Actor%20Object%20Reference) (OtherComp :type Primitive%20Component%20Object%20Reference) (OtherBodyIndex :type Integer))
  ;[0 0 0] Renewal
  (Utilities|Casting|CastToThirdPersonCharacter OtherActor)
  (CallFunction|EndResonating))

(event OnComponentBeginOverlap(Sphere)
  (params (OverlappedComponent :type Primitive%20Component%20Object%20Reference) (OtherActor :type Actor%20Object%20Reference) (OtherComp :type Primitive%20Component%20Object%20Reference) (OtherBodyIndex :type Integer) (bFromSweep :type Boolean) (SweepResult :type Hit%20Result%20Structure%20%28by%20ref%29))
  ;[0 0 0] Rotate Aspests
  (Utilities|Casting|CastToThirdPersonCharacter OtherActor)
  (bind _addrotation (Timeline|Rotate Play)
    (:Update
      (Transformation|AddWorldRotation (Variables|Default|GetBoxes) (Math|Rotator|MakeRotator 0.0 0.0 _addrotation) false false))))

(event OnComponentEndOverlap(Sphere)
  (params (OverlappedComponent :type Primitive%20Component%20Object%20Reference) (OtherActor :type Actor%20Object%20Reference) (OtherComp :type Primitive%20Component%20Object%20Reference) (OtherBodyIndex :type Integer))
  ;[0 0 0] Rotate Aspests
  (Utilities|Casting|CastToThirdPersonCharacter OtherActor)
  (bind _addrotation (Timeline|Rotate Stop)
    (:Update
      (Transformation|AddWorldRotation (Variables|Default|GetBoxes) (Math|Rotator|MakeRotator 0.0 0.0 _addrotation) false false))))

(event Custom|Resonance
  (bind _characterref (Variables|Default|GetCharacterREF))
  ;[0 0 0] Resonance
  ;;[0 0 0] Resonance Timer
  (if (Variables|Default|GetIsBossResonating)
    (if (< (Variables|Default|GetCurrentTime) (Variables|Default|GetResonanceTime))
      (bind _result (Math|Float|IncrementFloat (Variables|Default|GetCurrentTime))
        (:%20%20
          (Variables|/Game/Widgets/W_CharacterInterface.W_CharacterInterface_C|SetCurrentResonanceTime (Variables|/Game/ThirdPersonBP/Blueprints/ThirdPersonCharacter.ThirdPersonCharacter_C|GetInterfaceREF (Variables|Default|GetCharacterREF)) _result)
          (if (>= (Variables|Default|GetCurrentTime) (Variables|Default|GetResonanceTime))
            (Variables|/Game/ThirdPersonBP/Blueprints/ThirdPersonCharacter.ThirdPersonCharacter_C|SetIsUsingAbility (Variables|Default|GetCharacterREF) true)
            ;;;[0 0 0] Set ability from enemy aspect
            (switch Utilities|FlowControl|Switch|SwitchonEnemyAspects_Enum (Variables|Default|GetCurrentAspect)
              (:NewEnumerator0
                (Default|SetFaithAbility _characterref))
              (:NewEnumerator1
                (Default|SetDestructionAbility _characterref))
              (:NewEnumerator3
                (Default|SetRenewalAbility _characterref)))
            (Variables|Default|SetIsBossResonating false)))))))

(event Custom|Attack_1
  ;[0 0 0] Attack_1
  (bind _add_rotation (Timeline|Attack1 PlayFromStart)
    (:Update
      (Transformation|AddRelativeRotation (Variables|Default|GetTentacle_1) (Math|Rotator|MakeRotator 0.0 _add_rotation 0.0) false false))
    (:Finished
      (Transformation|SetRelativeRotation (Variables|Default|GetTentacle_1) "0, 0, 0" false false)
      (Transformation|SetRelativeRotation (Variables|Default|GetTentacle_2) "0,180.000000, 0" false false)
      (Transformation|SetRelativeRotation (Variables|Default|GetTentacle_3) "0,90.000000, 0" false false)
      (Transformation|SetRelativeRotation (Variables|Default|GetTentacle_4) "0,-90.000000, 0" false false)
      (Game|Damage|ApplyRadialDamage 25.0 (Transformation|GetActorLocation) 6e+02 0 0 self 0 true "ECC_Visibility"))))

(event Custom|Overlap
  (params (Aspect :type EnemyAspects_Enum%20Enum :default "NewEnumerator0"))
  (bind _characterref (Variables|Default|GetCharacterREF))
  ;[0 0 0] Set Aspect
  (Variables|Default|SetCurrentAspect Aspect)
  (Default|SetLatestGenerator _characterref Aspect)
  (Variables|/Game/Widgets/W_CharacterInterface.W_CharacterInterface_C|SetDisplayAspect (Variables|/Game/ThirdPersonBP/Blueprints/ThirdPersonCharacter.ThirdPersonCharacter_C|GetInterfaceREF _characterref) Aspect))

(event Custom|StartResonating
  ;[0 0 0] Resonance
  ;;[0 0 0] Resonance Timer
  (Variables|Default|SetIsBossResonating true)
  (bind _returnvalue (Utilities|Time|SetTimerbyEvent (delegate Custom|Resonance) 0.5 true))
  (Variables|Default|SetResTimer _returnvalue))

(event Custom|EndResonating
  ;[0 0 0] Resonance
  (Utilities|Time|ClearandInvalidateTimerbyHandle (Variables|Default|GetResTimer))
  (Variables|Default|SetCurrentTime 0.0)
  (Variables|/Game/Widgets/W_CharacterInterface.W_CharacterInterface_C|SetCurrentResonanceTime (Variables|/Game/ThirdPersonBP/Blueprints/ThirdPersonCharacter.ThirdPersonCharacter_C|GetInterfaceREF (Variables|Default|GetCharacterREF)) 0.0))

(event Custom|SpawnMinions
  ;[0 0 0] Spawn Minions
  (bind _returnvalue (Utilities|Time|SetTimerbyEvent (delegate Custom|Minions) 1.0 true))
  (Variables|Default|SetSpawnMinionsTimer _returnvalue))

(event Custom|Minions
  (bind _returnvalue (Transformation|GetActorLocation))
  ;[0 0 0] Spawn Minions
  (if (> (Variables|Default|GetMinionsAmount) 0)
    (Game|SpawnActorfromClass "/Game/Blueprints/Enemies/BaseEnemy/Old/BP_Minion_Child.BP_Minion_Child_C" (Math|Transform|MakeTransform (Math|Vector|MakeVector (.x _returnvalue) (.y _returnvalue) (+ (.z _returnvalue) 1e+02)) "0, 0, 0" "1.000000,1.000000,1.000000") "Undefined" 0 0)
    (Math|Integer|DecrementInt (Variables|Default|GetMinionsAmount))
    (else
      (Utilities|Time|ClearandInvalidateTimerbyHandle (Variables|Default|GetSpawnMinionsTimer)))))

(event Custom|Attack_2
  ;[0 0 0] Attack2
  (bind _newtrack_0 (Timeline|Attack2 PlayFromStart)
    (:Update
      (Transformation|AddWorldRotation (Variables|Default|GetTentacles) (Math|Rotator|MakeRotator 0.0 0.0 _newtrack_0) false false))))

(event EventBeginPlay
  (bind _enemyuiref (Variables|Default|GetEnemyUIREF))
  (|CallParentFunction)
  (bind _output_get (Variables|Default|SetCurrentHealth 1e+02))
  (bind _output_get_2 (Variables|/Game/Widgets/W_EnemyHealth.W_EnemyHealth_C|SetMaxHealthUI _enemyuiref _output_get))
  (Variables|/Game/Widgets/W_EnemyHealth.W_EnemyHealth_C|SetCurrentHealthUI _enemyuiref _output_get_2)
  (Utilities|FlowControl|Delay 2.0)
  (CallFunction|Attack1 :!label _label)
  (Utilities|FlowControl|Delay 6.0)
  (CallFunction|SpawnMinions)
  (Utilities|FlowControl|Delay 6.0)
  (CallFunction|Attack1)
  (Utilities|FlowControl|Delay 6.0)
  (CallFunction|Attack2)
  (Utilities|FlowControl|Delay 6.0)
  (goto _label))

(event Collision|EventActorBeginOverlap
  (params (OtherActor :type Actor%20Object%20Reference)))

(event EventTick
  (params (DeltaSeconds :type Float%20%28single-precision%29)))

(event Game|Damage|EventAnyDamage
  (params (Damage :type Float%20%28single-precision%29) (DamageType :type Damage%20Type%20Object%20Reference) (InstigatedBy :type Controller%20Object%20Reference) (DamageCauser :type Actor%20Object%20Reference))
  (bind _output_get (Variables|Default|SetCurrentHealth (- (Variables|Default|GetCurrentHealth) Damage)))
  (Variables|/Game/Widgets/W_EnemyHealth.W_EnemyHealth_C|SetCurrentHealthUI (Variables|Default|GetEnemyUIREF) _output_get)
  (if (<= _output_get 0.0)
    (CallFunction|Death)))

(fn ConstructionScript
  (|CallParentFunction))

(fn IsGeneratorReloading
  (params (IsReloading :type Boolean))
  (return false))