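; BP_Minion_Child is a minion enemy that chases the player and carries a shield that drops while the player uses an ability.
; Tick moves it toward the player and toggles the shield's visibility, collision and overlaps from the ThirdPersonCharacter's IsUsingAbility flag.
; Damage applies only with the shield down, updating the enemy health UI and calling Death at zero health.
; On destruction it has the player character delete its destruction marks.
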(event EventBeginPlay
  (bind _enemyuiref (Variables|Default|GetEnemyUIREF))
  (|CallParentFunction)
  (bind _output_get (Variables|Default|SetCurrentHealth 4e+01))
  (bind _output_get_2 (Variables|/Game/Widgets/W_EnemyHealth.W_EnemyHealth_C|SetCurrentHealthUI _enemyuiref _output_get))
  (Variables|/Game/Widgets/W_EnemyHealth.W_EnemyHealth_C|SetMaxHealthUI _enemyuiref _output_get_2)
  (bind _asthird_person_character (Utilities|Casting|CastToThirdPersonCharacter (Game|GetPlayerCharacter 0)))
  (Variables|Default|SetCharacterREF _asthird_person_character))

(event EventTick
  (params (DeltaSeconds :type Float%20%28single-precision%29))
  (bind _characterref (Variables|Default|GetCharacterREF))
  (bind _shield (Variables|Default|GetShield))
  (bind _shield_2 (Variables|Default|GetShield))
  (AI|Navigation|SimpleMovetoActor (Pawn|GetController) (Game|GetPlayerCharacter 0))
  (Utilities|IsValid _characterref
    (:Is%20Valid
      (if (Variables|/Game/ThirdPersonBP/Blueprints/ThirdPersonCharacter.ThirdPersonCharacter_C|GetIsUsingAbility _characterref)
        (Rendering|SetVisibility _shield_2 false true)
        (Collision|SetCollisionEnabled _shield_2 "NoCollision")
        (Variables|/Script/Engine.PrimitiveComponent|SetbGenerateOverlapEvents _shield_2 false)
        (Variables|Default|SetIsShieldActive false)
        (else
          (Rendering|SetVisibility _shield true true)
          (Collision|SetCollisionEnabled _shield "QueryAndPhysics")
          (Variables|/Script/Engine.PrimitiveComponent|SetbGenerateOverlapEvents _shield true)
          (Variables|Default|SetIsShieldActive true))))))

(event Game|Damage|EventAnyDamage
  (params (Damage :type Float%20%28single-precision%29) (DamageType :type Damage%20Type%20Object%20Reference) (InstigatedBy :type Controller%20Object%20Reference) (DamageCauser :type Actor%20Object%20Reference))
  (if (not (Variables|Default|GetIsShieldActive))
    (bind _output_get (Variables|Default|SetCurrentHealth (- (Variables|Default|GetCurrentHealth) Damage)))
    (Variables|/Game/Widgets/W_EnemyHealth.W_EnemyHealth_C|SetCurrentHealthUI (Variables|Default|GetEnemyUIREF) _output_get)
    (if (<= _output_get 0.0)
      (CallFunction|Death))))

(event EventDestroyed
  (bind _characterref (Variables|Default|GetCharacterREF))
  ;[0 0 0] Delete DestructionMarks after death
  (Utilities|IsValid _characterref
    (:Is%20Valid
      (Default|DeleteMarks _characterref))))

(fn ConstructionScript
  (|CallParentFunction))