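; BP_Enemy_3 is a ranged enemy (Shiz) that turns its yaw toward the player every tick and fires projectiles.
; BeginPlay copies speed and health from its info struct into movement and UI.
; Attack starts a looping timer spawning damage-carrying projectiles until ammo runs out, then reloads after a delay; its only call in this graph is disconnected.
; Taking damage pauses movement during a hit montage and forwards to the parent.
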(event Custom|Attack
  ;[0 0 0] Spawn Projectiles
  (bind _returnvalue (Utilities|Time|SetTimerbyEvent (delegate Custom|PassiveAttackSpawn) (Utilities|Struct|BreakEnemyInfo_Struct (Variables|Default|GetEnemyInfo_Struct)) true))
  (Variables|Default|SetAttackTimer _returnvalue))

(event Custom|PassiveAttackSpawn
  ;[0 0 0] Spawn Projectiles
  (if (> (Variables|Default|GetCurrentShootAmount) 0)
    (bind _returnvalue (Game|SpawnActorfromClass "/Game/Blueprints/Enemies/BaseEnemy/Enemy_3_Shiz/BP_Enemy_3_Projectile.BP_Enemy_3_Projectile_C" (Math|Transform|MakeTransform (Transformation|GetWorldLocation (Variables|Default|GetProjectilesSpawn)) (Transformation|GetActorRotation) "0.200000,0.200000,0.200000") "Undefined" 0 0))
    ;[0 0 0] Set projectile Damage
    (Variables|/Game/Blueprints/Enemies/BaseEnemy/BP_EnemyProjectiles.BP_EnemyProjectiles_C|SetEnemyDamage _returnvalue (Utilities|Struct|BreakEnemyInfo_Struct (Variables|Default|GetEnemyInfo_Struct)))
    (Math|Integer|DecrementInt (Variables|Default|GetCurrentShootAmount))
    (else
      ;[0 0 0] Reload
      (Utilities|FlowControl|Delay (Variables|Default|GetRecoilTime))
      (Variables|Default|SetCurrentShootAmount (Variables|Default|GetMaxShootAmount)))))

(event EventBeginPlay
  (bind _enemyinfo_struct (Variables|Default|GetEnemyInfo_Struct))
  (bind _enemyuiref (Variables|Default|GetEnemyUIREF))
  (bind (_maxhealth _maxspeed) (Utilities|Struct|BreakEnemyInfo_Struct _enemyinfo_struct))
  (|CallParentFunction)
  (Variables|/Script/Engine.CharacterMovementComponent|SetMaxWalkSpeed (Variables|Character|GetCharacterMovement) _maxspeed)
  (bind _output_get (Variables|Default|SetCurrentHealth _maxhealth))
  (bind _output_get_2 (Variables|/Game/Widgets/W_EnemyHealth.W_EnemyHealth_C|SetCurrentHealthUI _enemyuiref _output_get))
  (Variables|/Game/Widgets/W_EnemyHealth.W_EnemyHealth_C|SetMaxHealthUI _enemyuiref _output_get_2)
  (Variables|Default|SetCurrentShootAmount (Variables|Default|GetMaxShootAmount)))

(event EventTick
  (params (DeltaSeconds :type Float%20%28single-precision%29))
  ;[0 0 0] Rotation
  (Transformation|SetActorRotation (Math|Rotator|MakeRotator 0.0 0.0 (.yaw (Math|Rotator|FindLookatRotation (Transformation|GetActorLocation) (Transformation|GetWorldLocation (Variables|/Script/Engine.Character|GetMesh (Game|GetPlayerCharacter 0))))))))

(event Game|Damage|EventAnyDamage
  (params (Damage :type Float%20%28single-precision%29) (DamageType :type Damage%20Type%20Object%20Reference) (InstigatedBy :type Controller%20Object%20Reference) (DamageCauser :type Actor%20Object%20Reference))
  (bind _charactermovement (Variables|Character|GetCharacterMovement))
  (Pawn|Components|CharacterMovement|DisableMovement _charactermovement)
  (Animation|Montage|PlayMontage (Variables|Default|GetSkeletalMesh) "/Game/Animations/Enemies/3_Shiz/Shiz_Damage_Anim_Montage.Shiz_Damage_Anim_Montage"
    (:then
      (|CallParentFunction Damage DamageType InstigatedBy DamageCauser))
    (:OnCompleted
      (Pawn|Components|CharacterMovement|SetMovementMode _charactermovement "MOVE_Walking" 0 :!label _label))
    (:OnInterrupted
      (goto _label))))

(fn ConstructionScript
  (|CallParentFunction))