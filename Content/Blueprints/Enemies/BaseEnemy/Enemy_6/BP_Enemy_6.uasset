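; Enemy 6 is a charging melee enemy, built on a parent enemy class, that sets speed, health and UI from its info struct.
; One trigger box starts a brief, extreme speed boost when the player enters, and a second deals damage during attacks.
; A separate Dash event line-traces forward and lerps the actor there on a timeline.
; Accumulated damage past a threshold changes a cylinder's material, and Dash resets that tally.
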(event OnComponentBeginOverlap(Box)
  (params (OverlappedComponent :type Primitive%20Component%20Object%20Reference) (OtherActor :type Actor%20Object%20Reference) (OtherComp :type Primitive%20Component%20Object%20Reference) (OtherBodyIndex :type Integer) (bFromSweep :type Boolean) (SweepResult :type Hit%20Result%20Structure%20%28by%20ref%29))
  (Utilities|Casting|CastToThirdPersonCharacter OtherActor)
  (Variables|Default|SetIsAttacking true)
  (Variables|/Script/Engine.CharacterMovementComponent|SetMaxWalkSpeed (Variables|Character|GetCharacterMovement) (* (Utilities|Struct|BreakEnemyInfo_Struct (Variables|Default|GetEnemyInfo_Struct)) 5e+01))
  (Utilities|FlowControl|Delay 2.0)
  (Variables|Default|SetIsAttacking false)
  (Variables|/Script/Engine.CharacterMovementComponent|SetMaxWalkSpeed (Variables|Character|GetCharacterMovement) (Utilities|Struct|BreakEnemyInfo_Struct (Variables|Default|GetEnemyInfo_Struct)))
  (Utilities|FlowControl|DoOnce false ; enters at Reset
    (:Completed
      (Game|Damage|ApplyDamage (stale OnComponentBeginOverlap(Box1) _asthird_person_character) (Utilities|Struct|BreakEnemyInfo_Struct (Variables|Default|GetEnemyInfo_Struct)) 0 self))))

(event OnComponentBeginOverlap(Box1)
  (params (OverlappedComponent :type Primitive%20Component%20Object%20Reference) (OtherActor :type Actor%20Object%20Reference) (OtherComp :type Primitive%20Component%20Object%20Reference) (OtherBodyIndex :type Integer) (bFromSweep :type Boolean) (SweepResult :type Hit%20Result%20Structure%20%28by%20ref%29))
  (bind _asthird_person_character (Utilities|Casting|CastToThirdPersonCharacter OtherActor))
  (if (Variables|Default|GetIsAttacking)
    (Game|Damage|ApplyDamage _asthird_person_character (Utilities|Struct|BreakEnemyInfo_Struct (Variables|Default|GetEnemyInfo_Struct)) 0 self)))

(event Custom|Dash
  (bind _returnvalue (Transformation|GetActorLocation))
  ;[0 0 0] Dash
  (if (not (Variables|Default|GetIsAttacking))
    (Variables|Default|SetIsAttacking true)
    (Variables|Default|SetCurrentDamageEaten 0.0)
    (Variables|Dash|SetStartDashPosition _returnvalue)
    (bind _outhit (Collision|LineTraceByChannel _returnvalue (+ _returnvalue (* (Transformation|GetActorForwardVector) (Variables|Dash|GetDashDistance))) "TraceTypeQuery1" false 0 "ForDuration"))
    (if (.bBlockingHit (Collision|BreakHitResult _outhit))
      (Utilities|Casting|CastToThirdPersonCharacter (.HitActor (Collision|BreakHitResult _outhit))
        (:then
          (Variables|Dash|SetEndDashPosition (.Location (Collision|BreakHitResult _outhit))))
        (:CastFailed
          (Variables|Dash|SetEndDashPosition (.TraceEnd (Collision|BreakHitResult _outhit)) :!label _label)))
      (else
        (goto _label)))
    (Components|Timeline|SetPlayRate (Variables|Default|GetDash_timeline) (/ 1.0 (Variables|Dash|GetDashDuration)))
    (bind _alpha (Timeline|Dash_Timeline PlayFromStart)
      (:Update
        (Transformation|SetActorLocation (Math|Vector|Lerp(Vector) (Variables|Dash|GetStartDashPosition) (Variables|Dash|GetEndDashPosition) _alpha) false false))
      (:Finished
        (Utilities|FlowControl|Delay 0.2)
        (Variables|Default|SetIsAttacking false)))))

(event EventBeginPlay
  (bind _enemyinfo_struct (Variables|Default|GetEnemyInfo_Struct))
  (bind _enemyuiref (Variables|Default|GetEnemyUIREF))
  (bind (_maxhealth _maxspeed) (Utilities|Struct|BreakEnemyInfo_Struct _enemyinfo_struct))
  (|CallParentFunction)
  (Variables|/Script/Engine.CharacterMovementComponent|SetMaxWalkSpeed (Variables|Character|GetCharacterMovement) _maxspeed)
  (bind _output_get (Variables|Default|SetCurrentHealth _maxhealth))
  (bind _output_get_2 (Variables|/Game/Widgets/W_EnemyHealth.W_EnemyHealth_C|SetCurrentHealthUI _enemyuiref _output_get))
  (Variables|/Game/Widgets/W_EnemyHealth.W_EnemyHealth_C|SetMaxHealthUI _enemyuiref _output_get_2))

(event Game|Damage|EventAnyDamage
  (params (Damage :type Float%20%28single-precision%29) (DamageType :type Damage%20Type%20Object%20Reference) (InstigatedBy :type Controller%20Object%20Reference) (DamageCauser :type Actor%20Object%20Reference))
  (bind _output_get (Variables|Default|SetCurrentDamageEaten (+ Damage (Variables|Default|GetCurrentDamageEaten))))
  (|CallParentFunction Damage DamageType InstigatedBy DamageCauser)
  (if (>= _output_get (Variables|Default|GetMaxDamageEaten))
    (Rendering|Material|SetMaterial (Variables|Default|GetCylinder_1) 0 0)))

(fn ConstructionScript
  (|CallParentFunction))