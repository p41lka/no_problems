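; Blueprint for the first boss enemy, extending a parent class whose BeginPlay and construction script it calls.
; On BeginPlay it takes max health from EnemyInfo, starts current health at that value, and copies both into the enemy UI reference.
; After a short delay it plays a non-looping sit animation on the mesh; it has no other active logic of its own.
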(event EventBeginPlay
  (bind _enemyuiref (Variables|Default|GetEnemyUIREF))
  (|CallParentFunction)
  (bind _output_get (Variables|Default|SetMaxHealth (.MaxHealth (Utilities|Struct|BreakEnemyInfo_Struct (Variables|Default|GetEnemy_Info)))))
  (bind _output_get_2 (Variables|Default|SetCurrentHealth _output_get))
  (bind _output_get_3 (Variables|/Game/Widgets/W_EnemyHealth.W_EnemyHealth_C|SetCurrentHealthUI _enemyuiref _output_get_2))
  (Variables|/Game/Widgets/W_EnemyHealth.W_EnemyHealth_C|SetMaxHealthUI _enemyuiref _output_get_3)
  (Utilities|FlowControl|Delay 1.0)
  (Components|Animation|PlayAnimation (Variables|Character|GetMesh) "/Game/Animations/Boss_1/Boss_1_Sit_Anim.Boss_1_Sit_Anim" false))

(event Collision|EventActorBeginOverlap
  (params (OtherActor :type Actor%20Object%20Reference)))

(event EventTick
  (params (DeltaSeconds :type Float%20%28single-precision%29)))

(fn ConstructionScript
  (|CallParentFunction))