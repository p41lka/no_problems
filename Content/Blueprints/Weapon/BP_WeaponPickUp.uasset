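; Weapon pickup actor whose Weapon enum (Gun, Sickle or Three) selects its mesh in the construction script.
; Timelines bob and spin the mesh, and a sphere overlap toggles the E prompt's visibility for the third-person character.
; Interact grants the weapon if the character lacks it, sets it as current and refreshes weapon visibility.
; It then hides the mesh, plays particles and a sound, and destroys itself after a short delay.
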(event OnComponentBeginOverlap(Sphere)
  (params (OverlappedComponent :type Primitive%20Component%20Object%20Reference) (OtherActor :type Actor%20Object%20Reference) (OtherComp :type Primitive%20Component%20Object%20Reference) (OtherBodyIndex :type Integer) (bFromSweep :type Boolean) (SweepResult :type Hit%20Result%20Structure%20%28by%20ref%29))
  (Utilities|Casting|CastToThirdPersonCharacter OtherActor)
  (Rendering|SetVisibility (Variables|Default|GetE) true false))

(event OnComponentEndOverlap(Sphere)
  (params (OverlappedComponent :type Primitive%20Component%20Object%20Reference) (OtherActor :type Actor%20Object%20Reference) (OtherComp :type Primitive%20Component%20Object%20Reference) (OtherBodyIndex :type Integer))
  (Utilities|Casting|CastToThirdPersonCharacter OtherActor)
  (Rendering|SetVisibility (Variables|Default|GetE) false false))

(event EventBeginPlay
  (bind _mesh (Variables|Default|GetMesh))
  (bind _asthird_person_character (Utilities|Casting|CastToThirdPersonCharacter (Game|GetPlayerCharacter 0)))
  (Variables|Default|SetCharREF _asthird_person_character)
  (Utilities|FlowControl|Sequence
    (:then_0
      (bind _newtrack_0 (Timeline|Floating%20in%20the%20air Play)
        (:Update
          (Transformation|AddLocalOffset _mesh (Math|Vector|MakeVector 0.0 0.0 (Math|Float|Lerp 1.0 -1.0 _newtrack_0)) false false))))
    (:then_1
      (bind _newtrack_0_2 (Timeline|Rotation Play)
        (:Update
          (Transformation|SetRelativeRotation _mesh (Math|Rotator|MakeRotator 0.0 0.0 _newtrack_0_2) false false))))))

(event EventInteract
  (bind _charref (Variables|Default|GetCharREF))
  (bind _charref_2 (Variables|Default|GetCharREF))
  (bind _charref_3 (Variables|Default|GetCharREF))
  (switch Utilities|FlowControl|Switch|SwitchonWeapon_Enum (Variables|Default|GetWeapon)
    (:NewEnumerator0
      (if (not (Variables|/Game/ThirdPersonBP/Blueprints/ThirdPersonCharacter.ThirdPersonCharacter_C|GetHasGun _charref_2))
        (Variables|/Game/ThirdPersonBP/Blueprints/ThirdPersonCharacter.ThirdPersonCharacter_C|SetHasGun _charref_3 true)
        (Variables|/Game/ThirdPersonBP/Blueprints/ThirdPersonCharacter.ThirdPersonCharacter_C|SetCurrentWeapon _charref_3 "NewEnumerator0")
        (Variables|/Game/ThirdPersonBP/Blueprints/ThirdPersonCharacter.ThirdPersonCharacter_C|SetWeaponIndex _charref 0)
        (Default|SetWeaponVisibility _charref :!label _label)
        (Rendering|SetVisibility (Variables|Default|GetMesh) false false)
        (Components|Activation|Activate (Variables|Default|GetParticleSystem) true)
        (Audio|PlaySound2D "/Game/Sound/Sams_sound/zapsplat_science_fiction_cyberpunk_weapon_on_high_pitched_power_up_003_89942_pick_up_01.zapsplat_science_fiction_cyberpunk_weapon_on_high_pitched_power_up_003_89942_pick_up_01" 1.0 1.0 0.2 0 0)
        (Utilities|FlowControl|Delay 0.5)
        (Actor|DestroyActor)))
    (:NewEnumerator1
      (if (not (Variables|/Game/ThirdPersonBP/Blueprints/ThirdPersonCharacter.ThirdPersonCharacter_C|GetHasSickle _charref_2))
        (Variables|/Game/ThirdPersonBP/Blueprints/ThirdPersonCharacter.ThirdPersonCharacter_C|SetHasSickle _charref_3 true)
        (Variables|/Game/ThirdPersonBP/Blueprints/ThirdPersonCharacter.ThirdPersonCharacter_C|SetCurrentWeapon _charref_3 "NewEnumerator1")
        (Variables|/Game/ThirdPersonBP/Blueprints/ThirdPersonCharacter.ThirdPersonCharacter_C|SetWeaponIndex _charref 1)
        (goto _label)))
    (:NewEnumerator2
      (if (not (Variables|/Game/ThirdPersonBP/Blueprints/ThirdPersonCharacter.ThirdPersonCharacter_C|GetHasThree _charref_2))
        (Variables|/Game/ThirdPersonBP/Blueprints/ThirdPersonCharacter.ThirdPersonCharacter_C|SetHasThree _charref_3 true)
        (Variables|/Game/ThirdPersonBP/Blueprints/ThirdPersonCharacter.ThirdPersonCharacter_C|SetCurrentWeapon _charref_3 "NewEnumerator2")
        (Variables|/Game/ThirdPersonBP/Blueprints/ThirdPersonCharacter.ThirdPersonCharacter_C|SetWeaponIndex _charref 2)
        (goto _label)))))

(fn ConstructionScript
  (bind _mesh (Variables|Default|GetMesh))
  (switch Utilities|FlowControl|Switch|SwitchonWeapon_Enum (Variables|Default|GetWeapon)
    (:NewEnumerator0
      (Components|StaticMesh|SetStaticMesh _mesh "/Game/Meshes/Weapons/SM_Gun.SM_Gun"))
    (:NewEnumerator1
      (Components|StaticMesh|SetStaticMesh _mesh "/Game/Meshes/Weapons/SM_Sickle.SM_Sickle"))
    (:NewEnumerator2
      (Components|StaticMesh|SetStaticMesh _mesh "/Game/Meshes/Weapons/SM_Three.SM_Three"))))