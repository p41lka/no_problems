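; Enemy actor that continuously fires projectiles and hurts the player on contact.
; On BeginPlay it fills its health and starts a looping timer that spawns scaled-down BP_EnemyProjectiles at the AttackSpawn component.
; Overlapping its Sphere applies damage to a ThirdPersonCharacter.
; Incoming damage reduces health and destroys the actor once it reaches zero.
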(event OnComponentBeginOverlap(Sphere)
  (params (OverlappedComponent :type Primitive%20Component%20Object%20Reference) (OtherActor :type Actor%20Object%20Reference) (OtherComp :type Primitive%20Component%20Object%20Reference) (OtherBodyIndex :type Integer) (bFromSweep :type Boolean) (SweepResult :type Hit%20Result%20Structure%20%28by%20ref%29))
  ;[0 0 0] Damage when overlap with character
  (bind _asthird_person_character (Utilities|Casting|CastToThirdPersonCharacter OtherActor))
  (Game|Damage|ApplyDamage _asthird_person_character 1e+01 0 0))

(event Custom|PassiveAttack
  ;[0 0 0] Spawn Projectiles
  (bind _returnvalue (Utilities|Time|SetTimerbyEvent (delegate Custom|PassiveAttackSpawn) 0.2 true))
  (Variables|Default|SetAttackTimer _returnvalue))

(event Custom|PassiveAttackSpawn
  (bind _attackspawn (Variables|Default|GetAttackSpawn))
  ;[0 0 0] Spawn Projectiles
  (Game|SpawnActorfromClass "/Game/Blueprints/Projectiles/BP_EnemyProjectiles.BP_EnemyProjectiles_C" (Math|Transform|MakeTransform (Transformation|GetWorldLocation _attackspawn) (Transformation|GetWorldRotation _attackspawn) "0.200000,0.200000,0.200000") "Undefined" 0 0))

(event Game|Damage|EventAnyDamage
  (params (Damage :type Float%20%28single-precision%29) (DamageType :type Damage%20Type%20Object%20Reference) (InstigatedBy :type Controller%20Object%20Reference) (DamageCauser :type Actor%20Object%20Reference))
  ;[0 0 0] Damage
  (bind _output_get (Variables|Default|SetCurrentHealth (- (Variables|Default|GetCurrentHealth) Damage)))
  (if (not (> _output_get 0.0))
    (Actor|DestroyActor)))

(event EventBeginPlay
  (Variables|Default|SetCurrentHealth (Variables|Default|GetMaxHealth))
  (CallFunction|PassiveAttack))

(fn ConstructionScript)