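; BP_Destruction_1Projectiles is a short-lived projectile for the first Destruction boost.
; On BeginPlay it sets a brief lifespan and caches the player's ThirdPersonCharacter.
; The sphere's first hit, if on a BP_BaseEnemy, spawns an impact effect below the enemy's origin, calls the character's Destruction1Overlap with that enemy, and destroys the projectile.
; When projectile movement stops, it spawns a smaller impact effect and destroys itself.
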(event OnProjectileStop(ProjectileMovement)
  (params (ImpactResult :type Hit%20Result%20Structure%20%28by%20ref%29))
  (Effects|SpawnEmitteratLocation "/Game/VFX/Stylized_FX_Collection_02/ParticleSystem/StylizedFX_05/Sci_Fi_Bullet/P_SF_Bullet_Hit_03.P_SF_Bullet_Hit_03" (.Location (Collision|BreakHitResult ImpactResult)) "0, 0, 0" "0.400000,0.400000,0.400000")
  (Actor|DestroyActor))

(event OnComponentHit(Sphere1)
  (params (HitComponent :type Primitive%20Component%20Object%20Reference) (OtherActor :type Actor%20Object%20Reference) (OtherComp :type Primitive%20Component%20Object%20Reference) (NormalImpulse :type Vector :default "0, 0, 0") (Hit :type Hit%20Result%20Structure%20%28by%20ref%29))
  (Utilities|FlowControl|DoOnce false
    (:Completed
      (bind _asbp_base_enemy (Utilities|Casting|CastToBP_BaseEnemy OtherActor))
      (bind _output_get (Variables|Default|SetEnemyREF _asbp_base_enemy))
      (Effects|SpawnEmitteratLocation "/Game/VFX/Stylized_FX_Collection_02/ParticleSystem/StylizedFX_05/Sci_Fi_Bullet/P_SF_Bullet_Hit_03.P_SF_Bullet_Hit_03" (Math|Vector|MakeVector (.x (Transformation|GetActorLocation _output_get)) (.y (Transformation|GetActorLocation _output_get)) (- (.z (Transformation|GetActorLocation _output_get)) 5e+01)))
      (Default|Destruction1Overlap (Variables|Default|GetCharacterREF) _output_get)
      (Actor|DestroyActor))))

(event EventBeginPlay
  (Actor|SetLifeSpan 1.5)
  (bind _asthird_person_character (Utilities|Casting|CastToThirdPersonCharacter (Game|GetPlayerCharacter 0)))
  (Variables|Default|SetCharacterREF _asthird_person_character))

(fn ConstructionScript)