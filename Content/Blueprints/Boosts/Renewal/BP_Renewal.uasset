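; BP_Renewal is a short-lived hit actor in the Boosts folder that damages enemies on impact and expires after about a second.
; On BeginPlay it caches the player's ThirdPersonCharacter to use as damage causer.
; Its first hit, guarded by DoOnce, applies fixed damage to a BP_BaseEnemy with an impact emitter below the enemy's origin.
; Other hits show a smaller emitter at the impact point; either way it destroys itself.
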(event EventBeginPlay
  (Actor|SetLifeSpan 1.2)
  (bind _asthird_person_character (Utilities|Casting|CastToThirdPersonCharacter (Game|GetPlayerCharacter 0)))
  (Variables|Default|SetCharacterREF _asthird_person_character))

(event Collision|EventHit
  (params (MyComp :type Primitive%20Component%20Object%20Reference) (Other :type Actor%20Object%20Reference) (OtherComp :type Primitive%20Component%20Object%20Reference) (bSelfMoved :type Boolean) (HitLocation :type Vector :default "0, 0, 0") (HitNormal :type Vector :default "0, 0, 0") (NormalImpulse :type Vector :default "0, 0, 0") (Hit :type Hit%20Result%20Structure%20%28by%20ref%29))
  (Utilities|FlowControl|DoOnce false
    (:Completed
      (bind _asbp_base_enemy (Utilities|Casting|CastToBP_BaseEnemy Other)
        (:then
          (Effects|SpawnEmitteratLocation "/Game/VFX/Stylized_FX_Collection_02/ParticleSystem/StylizedFX_05/Sci_Fi_Bullet/P_SF_Bullet_Hit_04.P_SF_Bullet_Hit_04" (Math|Vector|MakeVector (.x (Transformation|GetActorLocation _asbp_base_enemy)) (.y (Transformation|GetActorLocation _asbp_base_enemy)) (- (.z (Transformation|GetActorLocation _asbp_base_enemy)) 5e+01)))
          (Game|Damage|ApplyDamage _asbp_base_enemy 1e+01 0 (Variables|Default|GetCharacterREF))
          (Utilities|IsValid _asbp_base_enemy
            (:Is%20Valid
              _)
            (:Is%20Not%20Valid
              _))
          (Actor|DestroyActor))
        (:CastFailed
          (Effects|SpawnEmitteratLocation "/Game/VFX/Stylized_FX_Collection_02/ParticleSystem/StylizedFX_05/Sci_Fi_Bullet/P_SF_Bullet_Hit_04.P_SF_Bullet_Hit_04" HitLocation "0, 0, 0" "0.400000,0.400000,0.400000")
          (Actor|DestroyActor))))))

(fn ConstructionScript)