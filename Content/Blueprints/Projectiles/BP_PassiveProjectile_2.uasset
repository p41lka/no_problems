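; Homing passive projectile that seeks the nearest BP_Enemy and damages it.
; Tick refreshes the nearest target, while a timeline started on BeginPlay lerps the projectile from its sphere's current location toward it, destroying it if no target is valid.
; Overlapping an enemy's Sphere component applies PassiveDamage and destroys the projectile.
; The FindNearestEnemy function is an unfinished stub; targeting uses FindNearestActor.
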(event OnComponentBeginOverlap(SphereCollision)
  (params (OverlappedComponent :type Primitive%20Component%20Object%20Reference) (OtherActor :type Actor%20Object%20Reference) (OtherComp :type Primitive%20Component%20Object%20Reference) (OtherBodyIndex :type Integer) (bFromSweep :type Boolean) (SweepResult :type Hit%20Result%20Structure%20%28by%20ref%29))
  (bind _asbp_enemy (Utilities|Casting|CastToBP_Enemy OtherActor))
  (if (== OtherComp (Variables|/Game/Blueprints/BaseEnemy/BP_Enemy.BP_Enemy_C|GetSphere _asbp_enemy))
    (Game|Damage|ApplyDamage _asbp_enemy (Variables|Default|GetPassiveDamage) 0 0)
    (Actor|DestroyActor)))

(event EventBeginPlay
  (bind _distance_normalized_ (Timeline|Alpha Play)
    (:Update
      (Utilities|IsValid (Variables|Default|GetNearest%20Actor)
        (:Is%20Valid
          (Transformation|SetActorLocation (Math|Vector|Lerp(Vector) (Transformation|GetWorldLocation (Variables|Default|GetSphere)) (Transformation|GetActorLocation (Variables|Default|GetNearest%20Actor)) _distance_normalized_) false false))
        (:Is%20Not%20Valid
          (Actor|DestroyActor))))))

(event EventTick
  (params (DeltaSeconds :type Float%20%28single-precision%29))
  (bind _nearestactor (CallFunction|FindNearestActor "/Game/Blueprints/BaseEnemy/BP_Enemy.BP_Enemy_C" (Transformation|GetActorLocation)))
  (Variables|Default|SetNearest%20Actor _nearestactor))

(fn ConstructionScript)

(fn FindNearestEnemy
  (params (Class :type Actor%20Class%20Reference) (Target%20Location :type Vector)))