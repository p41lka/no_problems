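; BP_PassiveProjectile is a homing projectile that seeks the nearest BP_Generator and deals PassiveDamage to it.
; Tick refreshes the nearest generator, while a timeline started on BeginPlay lerps the actor from its Sphere's current world location toward that target, destroying it if the target is invalid.
; Overlapping a generator's Sphere component with SphereCollision applies the damage and destroys the projectile.
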(event OnComponentBeginOverlap(SphereCollision)
  (params (OverlappedComponent :type Primitive%20Component%20Object%20Reference) (OtherActor :type Actor%20Object%20Reference) (OtherComp :type Primitive%20Component%20Object%20Reference) (OtherBodyIndex :type Integer) (bFromSweep :type Boolean) (SweepResult :type Hit%20Result%20Structure%20%28by%20ref%29))
  ;[1 1 1] base enemy
  (bind _asbp_generator (Utilities|Casting|CastToBP_Generator OtherActor))
  (if (== OtherComp (Variables|/Game/Blueprints/Generator/BP_Generator.BP_Generator_C|GetSphere _asbp_generator))
    (Game|Damage|ApplyDamage _asbp_generator (Variables|Default|GetPassiveDamage) 0 0)
    (Actor|DestroyActor)))

(event EventBeginPlay
  (bind _distance_normalized_ (Timeline|Alpha Play)
    (:Update
      (Utilities|IsValid (Variables|Default|GetNearest%20Actor)
        (:Is%20Valid
          (Transformation|SetActorLocation (Math|Vector|Lerp(Vector) (Transformation|GetWorldLocation (Variables|Default|GetSphere)) (Transformation|GetActorLocation (Variables|Default|GetNearest%20Actor)) _distance_normalized_) false false))
        (:Is%20Not%20Valid
          (Actor|DestroyActor))))))

(event EventTick
  (params (DeltaSeconds :type Float%20%28single-precision%29))
  (bind _nearestactor (CallFunction|FindNearestActor "/Game/Blueprints/Generator/BP_Generator.BP_Generator_C" (Transformation|GetActorLocation)))
  (Variables|Default|SetNearest%20Actor _nearestactor))

(fn ConstructionScript)