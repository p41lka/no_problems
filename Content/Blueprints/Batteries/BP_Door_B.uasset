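; Sliding double door that opens on OpenDoor with a 2D sound, then triggers its DialogueComponent three seconds later.
; Two timelines move SceneL and SceneR toward LocationLeft and LocationRight, lerping from each leaf's current relative location every update.
; BeginPlay scales the timeline play rates by the inverse of Time.
; CloseDoor is empty; partial closing logic for the left leaf is left unconnected.
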(event Custom|OpenDoor
  (bind _scene_l (Variables|Default|GetScene_L))
  (bind _scene_r (Variables|Default|GetScene_R))
  (Variables|Default|SetIsOpened true)
  (bind _returnvalue (Audio|CreateSound2D "/Game/Sound/243699__ertfelda__hidden-wall-opening_01.243699__ertfelda__hidden-wall-opening_01" 1.0 1.0 0.0 0))
  (Audio|Components|Audio|Play _returnvalue 0.0)
  (Utilities|FlowControl|Sequence
    (:then_0
      (bind _newtrack_0 (Timeline|Door_open_close PlayFromStart)
        (:Update
          (Transformation|SetRelativeLocation _scene_l (Math|Vector|Lerp(Vector) (Variables|/Script/Engine.SceneComponent|GetRelativeLocation _scene_l) (Variables|Default|GetLocation_Left) _newtrack_0) false false))))
    (:then_1
      (bind _newtrack_0_2 (Timeline|Timeline_0 PlayFromStart)
        (:Update
          (Transformation|SetRelativeLocation _scene_r (Math|Vector|Lerp(Vector) (Variables|/Script/Engine.SceneComponent|GetRelativeLocation _scene_r) (Variables|Default|GetLocation_Right) _newtrack_0_2) false false))))
    (:then_2
      ;[0 0 0] Dialogue
      (Utilities|FlowControl|Delay 3.0)
      (Default|Interact self))))

(event Custom|CloseDoor)

(event EventBeginPlay
  (bind _time (Variables|Default|GetTime))
  (bind _returnvalue (/ 1.0 _time))
  (Components|Timeline|SetPlayRate (Variables|Default|GetDoor_open_close) _returnvalue)
  (Components|Timeline|SetPlayRate (Variables|Default|GetTimeline_0) _returnvalue)
  (Components|Timeline|SetPlayRate (Variables|Default|GetTimeline_1) _returnvalue)
  (Components|Timeline|SetPlayRate (Variables|Default|GetTimeline_2) _returnvalue))

(event EventInteract
  ;[0 0 0] Dialogue
  (Default|Talk (Variables|Default|GetDialogueComponent)))

(fn ConstructionScript)