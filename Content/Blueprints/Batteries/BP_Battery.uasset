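; BP_Battery is an interactable battery station that powers either a door or a set of lights, chosen by its Type.
; Interact spends one of the player's CurrentAmmo charges to open the door or switch on each inactive light, and refunds one for each closed or switched off.
; A DoOnce also fires timelines that slide the High and Low components.
; An overlap volume toggles the interact prompt widget for the player character.
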(event OnComponentBeginOverlap(InteractCollision)
  (params (OverlappedComponent :type Primitive%20Component%20Object%20Reference) (OtherActor :type Actor%20Object%20Reference) (OtherComp :type Primitive%20Component%20Object%20Reference) (OtherBodyIndex :type Integer) (bFromSweep :type Boolean) (SweepResult :type Hit%20Result%20Structure%20%28by%20ref%29))
  ;[0 0 0] E to interact widget
  (Utilities|Casting|CastToThirdPersonCharacter OtherActor)
  (Rendering|SetVisibility (Variables|Default|GetWidget) true false))

(event OnComponentEndOverlap(InteractCollision)
  (params (OverlappedComponent :type Primitive%20Component%20Object%20Reference) (OtherActor :type Actor%20Object%20Reference) (OtherComp :type Primitive%20Component%20Object%20Reference) (OtherBodyIndex :type Integer))
  ;[0 0 0] E to interact widget
  (Utilities|Casting|CastToThirdPersonCharacter OtherActor)
  (Rendering|SetVisibility (Variables|Default|GetWidget) false false))

(event Custom|DoorInteract
  (bind _door (Variables|Default|GetDoor))
  ;[0 0 0] Door
  (if (Variables|/Game/Blueprints/Batteries/BP_Door_B.BP_Door_B_C|GetIsOpened _door)
    (Default|CloseDoor _door)
    (CallFunction|AddCharges)
    (elif (> (Variables|/Game/ThirdPersonBP/Blueprints/ThirdPersonCharacter.ThirdPersonCharacter_C|GetCurrentAmmo (Variables|Default|GetCharREF)) 0)
      (Default|OpenDoor _door)
      (CallFunction|MinusCharges))))

(event Custom|LightInteract
  ;[0 0 0] Light
  (for _array_element (Variables|Default|GetLightSource)
    (if (Variables|/Game/Blueprints/Batteries/BP_Light_B.BP_Light_B_C|GetIsActive _array_element)
      (Default|LightOff _array_element)
      (CallFunction|AddCharges)
      (elif (> (Variables|/Game/ThirdPersonBP/Blueprints/ThirdPersonCharacter.ThirdPersonCharacter_C|GetCurrentAmmo (Variables|Default|GetCharREF)) 0)
        (Default|Lighton _array_element)
        (CallFunction|MinusCharges)))))

(event Custom|MinusCharges
  ;[0 0 0] Charges
  (Math|Integer|DecrementInt (Variables|/Game/ThirdPersonBP/Blueprints/ThirdPersonCharacter.ThirdPersonCharacter_C|GetCurrentAmmo (Variables|Default|GetCharREF))))

(event Custom|AddCharges
  ;[0 0 0] Charges
  (Math|Integer|IncrementInt (Variables|/Game/ThirdPersonBP/Blueprints/ThirdPersonCharacter.ThirdPersonCharacter_C|GetCurrentAmmo (Variables|Default|GetCharREF))))

(event EventInteract
  (switch Utilities|FlowControl|Switch|SwitchonE_BatteryType (Variables|Default|GetType)
    (:NewEnumerator0
      (CallFunction|DoorInteract))
    (:NewEnumerator1
      (CallFunction|LightInteract)))
  (Utilities|FlowControl|DoOnce false
    (:Completed
      (bind _up (Timeline|Timeline_0 Play)
        (:Update
          (Transformation|SetRelativeLocation (Variables|Default|GetHigh) _up false false)
          (bind _down (Timeline|Timeline_1 Play)
            (:Update
              (Transformation|SetRelativeLocation (Variables|Default|GetLow) _down false false))))))))

(event EventBeginPlay
  (bind _asthird_person_character (Utilities|Casting|CastToThirdPersonCharacter (Game|GetPlayerCharacter 0)))
  (Variables|Default|SetCharREF _asthird_person_character))

(fn ConstructionScript)