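; BP_Capsule is an ammo pickup that adds to the player character's CurrentDopAmmo, capped at MaxDopAmmo, then destroys itself.
; Collection runs on overlap with PickupCollision or through the Interact event, and only while that ammo is below max.
; On BeginPlay it caches the player character and, after a short delay, switches off the capsule's physics simulation.
; InteractCollision overlap events are empty, and the widget visibility logic is disconnected.
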(event OnComponentBeginOverlap(InteractCollision)
  (params (OverlappedComponent :type Primitive%20Component%20Object%20Reference) (OtherActor :type Actor%20Object%20Reference) (OtherComp :type Primitive%20Component%20Object%20Reference) (OtherBodyIndex :type Integer) (bFromSweep :type Boolean) (SweepResult :type Hit%20Result%20Structure%20%28by%20ref%29))
  ;[0 0 0] E to collect
)

(event OnComponentEndOverlap(InteractCollision)
  (params (OverlappedComponent :type Primitive%20Component%20Object%20Reference) (OtherActor :type Actor%20Object%20Reference) (OtherComp :type Primitive%20Component%20Object%20Reference) (OtherBodyIndex :type Integer))
  ;[0 0 0] E to collect
)

(event OnComponentBeginOverlap(PickupCollision)
  (params (OverlappedComponent :type Primitive%20Component%20Object%20Reference) (OtherActor :type Actor%20Object%20Reference) (OtherComp :type Primitive%20Component%20Object%20Reference) (OtherBodyIndex :type Integer) (bFromSweep :type Boolean) (SweepResult :type Hit%20Result%20Structure%20%28by%20ref%29))
  ;[0 0 0] Overlap to collect
  (bind _asthird_person_character (Utilities|Casting|CastToThirdPersonCharacter OtherActor))
  (if (< (Variables|/Game/ThirdPersonBP/Blueprints/ThirdPersonCharacter.ThirdPersonCharacter_C|GetCurrentDopAmmo _asthird_person_character) (Variables|/Game/ThirdPersonBP/Blueprints/ThirdPersonCharacter.ThirdPersonCharacter_C|GetMaxDopAmmo _asthird_person_character))
    (CallFunction|AddAmmo)))

(event Custom|AddAmmo
  (bind _characterref (Variables|Default|GetCharacterREF))
  ;[0 0 0] Add ammo event
  (Variables|/Game/ThirdPersonBP/Blueprints/ThirdPersonCharacter.ThirdPersonCharacter_C|SetCurrentDopAmmo _characterref (Math|Integer|Clamp(Integer) (+ (Variables|/Game/ThirdPersonBP/Blueprints/ThirdPersonCharacter.ThirdPersonCharacter_C|GetCurrentDopAmmo _characterref) (Variables|Default|GetAmmo)) 0 (Variables|/Game/ThirdPersonBP/Blueprints/ThirdPersonCharacter.ThirdPersonCharacter_C|GetMaxDopAmmo _characterref)))
  (Actor|DestroyActor))

(event EventInteract
  (bind _characterref (Variables|Default|GetCharacterREF))
  ;[0 0 0] E to collect
  (if (< (Variables|/Game/ThirdPersonBP/Blueprints/ThirdPersonCharacter.ThirdPersonCharacter_C|GetCurrentDopAmmo _characterref) (Variables|/Game/ThirdPersonBP/Blueprints/ThirdPersonCharacter.ThirdPersonCharacter_C|GetMaxDopAmmo _characterref))
    (CallFunction|AddAmmo)))

(event EventBeginPlay
  (bind _asthird_person_character (Utilities|Casting|CastToThirdPersonCharacter (Game|GetPlayerCharacter 0)))
  (Variables|Default|SetCharacterREF _asthird_person_character)
  (Utilities|FlowControl|Delay 0.6)
  (Physics|SetSimulatePhysics (Variables|Default|GetCapsule) false))

(fn ConstructionScript)