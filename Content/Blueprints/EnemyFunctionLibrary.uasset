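; Enemy function library with FindNearestActor, which finds the closest actor of a given class to a target location.
; It scans every actor from GetAllActorsOfClass, tracking the smallest distance in local variables and skipping any actor within 200 units of the target.
; It returns both the nearest qualifying actor and its distance.
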(fn FindNearestActor
  (params (Class :type Actor%20Class%20Reference) (TargetLocation :type Vector))
  (bind _outactors (Actor|GetAllActorsOfClass 0 Class))
  (for _array_element _outactors
    (if (and (< (Math|Vector|Distance(Vector) (Transformation|GetActorLocation _array_element) TargetLocation) (LocalVariables|GetLoc_NearestDistance)) (> (Math|Vector|Distance(Vector) (Transformation|GetActorLocation _array_element) TargetLocation) 2e+02))
      (LocalVariables|SetLoc_NearestDistance (Math|Vector|Distance(Vector) (Transformation|GetActorLocation _array_element) TargetLocation))
      (LocalVariables|SetLoc_NearestActor _array_element)))
  (return (LocalVariables|GetLoc_NearestActor) (LocalVariables|GetLoc_NearestDistance)))