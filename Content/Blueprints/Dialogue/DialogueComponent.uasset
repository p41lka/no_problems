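; Dialogue component that runs a conversation as a behavior tree, using an AIController it spawns on BeginPlay.
; Talk shows a W_Dialogue widget, switches to UI-only input, disables player movement, then starts DialogueTree and puts the widget in the BB_Dialogue blackboard for the tree.
; The widget's OnExit event removes it, restores game input and walking, and stops the tree.
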(event Custom|OnExit_Event
  (bind _returnvalue (Game|GetPlayerController 0))
  (Input|SetInputModeGameOnly _returnvalue)
  (Variables|/Script/Engine.PlayerController|SetbShowMouseCursor _returnvalue false)
  (Widget|RemovefromParent (Variables|Default|GetDialogueWidget))
  (Pawn|Components|CharacterMovement|SetMovementMode (Variables|/Script/Engine.Character|GetCharacterMovement (Game|GetPlayerCharacter 0)) "MOVE_Walking" 0)
  (AI|Logic|StopLogic (Variables|/Script/AIModule.AIController|GetBrainComponent (Variables|Default|GetAIController)) ""))

(event EventBeginPlay
  (bind _returnvalue (Game|SpawnActorfromClass "/Script/AIModule.AIController" (Math|Transform|MakeTransform "0, 0, 0" "0, 0, 0" "1.000000,1.000000,1.000000") "Undefined" 0 0))
  (Variables|Default|SetAIController _returnvalue))

(event EventTalk
  (bind _returnvalue (Game|GetPlayerController 0))
  (bind _returnvalue_2 (UserInterface|CreateWidget "/Game/Widgets/W_Dialogue.W_Dialogue_C" (Game|GetPlayerController 0)))
  (bind _output_get (Variables|Default|SetDialogueWidget _returnvalue_2))
  (EventDispatchers|AssignOnExit _output_get (delegate Custom|OnExit_Event))
  (UserInterface|Viewport|AddtoViewport _output_get 0)
  (Input|SetInputModeUIOnly _returnvalue _output_get "DoNotLock")
  (Variables|/Script/Engine.PlayerController|SetbShowMouseCursor _returnvalue true)
  (Pawn|Components|CharacterMovement|DisableMovement (Variables|/Script/Engine.Character|GetCharacterMovement (Game|GetPlayerCharacter 0)))
  (AI|RunBehaviorTree (Variables|Default|GetAIController) (Variables|Default|GetDialogueTree))
  (bind _blackboardcomponent (Class|AIController|UseBlackboard (Variables|Default|GetAIController) "/Game/Blueprints/Dialogue/BB_Dialogue.BB_Dialogue"))
  (AI|Components|Blackboard|SetValueasObject _blackboardcomponent (Utilities|Name|MakeLiteralName "DialogueWidget") (Variables|Default|GetDialogueWidget)))