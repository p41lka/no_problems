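; BP_Talkable1 is an interactable actor, likely an NPC, that the player can talk to.
; An interaction sphere shows the E component, apparently a key prompt, while the third-person character overlaps it and hides it on exit.
; Interact starts DialogueComponent's Talk with the actor's Name, hides E and sets IsTalking on the player character.
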(event OnComponentBeginOverlap(InteractionSphere)
  (params (OverlappedComponent :type Primitive%20Component%20Object%20Reference) (OtherActor :type Actor%20Object%20Reference) (OtherComp :type Primitive%20Component%20Object%20Reference) (OtherBodyIndex :type Integer) (bFromSweep :type Boolean) (SweepResult :type Hit%20Result%20Structure%20%28by%20ref%29))
  (Utilities|Casting|CastToThirdPersonCharacter OtherActor)
  (Rendering|SetVisibility (Variables|Default|GetE) true false))

(event OnComponentEndOverlap(InteractionSphere)
  (params (OverlappedComponent :type Primitive%20Component%20Object%20Reference) (OtherActor :type Actor%20Object%20Reference) (OtherComp :type Primitive%20Component%20Object%20Reference) (OtherBodyIndex :type Integer))
  (Utilities|Casting|CastToThirdPersonCharacter OtherActor)
  (Rendering|SetVisibility (Variables|Default|GetE) false false))

(event EventBeginPlay
  (bind _asthird_person_character (Utilities|Casting|CastToThirdPersonCharacter (Game|GetPlayerCharacter 0)))
  (Variables|Default|SetCharREF _asthird_person_character))

(event EventInteract
  (Default|Talk (Variables|Default|GetDialogueComponent) (Variables|Default|GetName))
  (Rendering|SetVisibility (Variables|Default|GetE) false false)
  (bind _asthird_person_character (Utilities|Casting|CastToThirdPersonCharacter (Game|GetPlayerCharacter 0)))
  (Variables|/Game/ThirdPersonBP/Blueprints/ThirdPersonCharacter.ThirdPersonCharacter_C|SetIsTalking _asthird_person_character true))

(fn ConstructionScript)