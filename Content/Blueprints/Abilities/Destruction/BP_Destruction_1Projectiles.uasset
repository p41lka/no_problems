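; BP_Destruction_1Projectiles is the projectile actor for the first Destruction ability.
; On spawn it sets a short lifespan and caches the player's ThirdPersonCharacter.
; When its sphere overlaps a BP_BaseEnemy, it passes that enemy to the character's Destruction1Overlap and destroys itself, leaving the hit response to the character.
; It also destroys itself when its projectile movement stops.
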(event OnComponentBeginOverlap(Sphere1)
  (params (OverlappedComponent :type Primitive%20Component%20Object%20Reference) (OtherActor :type Actor%20Object%20Reference) (OtherComp :type Primitive%20Component%20Object%20Reference) (OtherBodyIndex :type Integer) (bFromSweep :type Boolean) (SweepResult :type Hit%20Result%20Structure%20%28by%20ref%29))
  (bind _asbp_base_enemy (Utilities|Casting|CastToBP_BaseEnemy OtherActor))
  (bind _output_get (Variables|Default|SetEnemyREF _asbp_base_enemy))
  (Default|Destruction1Overlap (Variables|Default|GetCharacterREF) _output_get)
  (Actor|DestroyActor))

(event OnProjectileStop(ProjectileMovement)
  (params (ImpactResult :type Hit%20Result%20Structure%20%28by%20ref%29))
  (Actor|DestroyActor))

(event EventBeginPlay
  (Actor|SetLifeSpan 1.5)
  (bind _asthird_person_character (Utilities|Casting|CastToThirdPersonCharacter (Game|GetPlayerCharacter 0)))
  (Variables|Default|SetCharacterREF _asthird_person_character))

(fn ConstructionScript)