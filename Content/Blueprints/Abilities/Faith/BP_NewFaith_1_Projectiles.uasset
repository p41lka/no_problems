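; Projectile actor for a Faith ability that damages enemies on contact and in an area around the impact.
; It caches the player character on BeginPlay as damage causer and expires after a short lifespan.
; When its sphere overlaps a BP_BaseEnemy, a tiny delay precedes fixed direct damage plus full radial damage sized by NewFaith1Struct, then it destroys itself.
; A radius debug draw is left unconnected.
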(event OnComponentBeginOverlap(Sphere)
  (params (OverlappedComponent :type Primitive%20Component%20Object%20Reference) (OtherActor :type Actor%20Object%20Reference) (OtherComp :type Primitive%20Component%20Object%20Reference) (OtherBodyIndex :type Integer) (bFromSweep :type Boolean) (SweepResult :type Hit%20Result%20Structure%20%28by%20ref%29))
  (bind _newfaith1struct (Variables|Default|GetnewFaith1Struct))
  (bind (_isactive _redius _damageaoe) (Utilities|Struct|BreakNewFaith_1_Struct _newfaith1struct))
  (bind _asbp_base_enemy (Utilities|Casting|CastToBP_BaseEnemy OtherActor))
  (Utilities|FlowControl|Delay 0.01)
  (Game|Damage|ApplyDamage _asbp_base_enemy 1e+01 0 (Variables|Default|GetCharacterREF))
  (Game|Damage|ApplyRadialDamage _damageaoe (Transformation|GetWorldLocation (Variables|Default|GetSphere)) _redius 0 0 (Variables|Default|GetCharacterREF) 0 true "ECC_Visibility")
  (Actor|DestroyActor))

(event EventBeginPlay
  (Actor|SetLifeSpan 1.5)
  (bind _asthird_person_character (Utilities|Casting|CastToThirdPersonCharacter (Game|GetPlayerCharacter 0)))
  (Variables|Default|SetCharacterREF _asthird_person_character))

(fn ConstructionScript)