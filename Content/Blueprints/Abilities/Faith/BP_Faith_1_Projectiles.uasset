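; Faith ability projectile that damages enemies it overlaps as it flies.
; Its sphere overlap applies fixed ability-typed damage to BP_BaseEnemy actors and counts hits, destroying the projectile once the count reaches its pierce limit.
; It also destroys itself when its projectile movement stops, or expires after a short lifespan set on BeginPlay, where it caches a player character reference.
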(event OnComponentBeginOverlap(Sphere1)
  (params (OverlappedComponent :type Primitive%20Component%20Object%20Reference) (OtherActor :type Actor%20Object%20Reference) (OtherComp :type Primitive%20Component%20Object%20Reference) (OtherBodyIndex :type Integer) (bFromSweep :type Boolean) (SweepResult :type Hit%20Result%20Structure%20%28by%20ref%29))
  (bind _asbp_base_enemy (Utilities|Casting|CastToBP_BaseEnemy OtherActor))
  (Game|Damage|ApplyDamage _asbp_base_enemy 1e+01 0 0 "/Game/Blueprints/Abilities/Ability_DT.Ability_DT_C")
  (bind _result (Math|Integer|IncrementInt (Variables|Default|GetEnemiesOverlapped))
    (:%20%20
      (if (>= _result 2)
        (Actor|DestroyActor)))))

(event OnProjectileStop(ProjectileMovement)
  (params (ImpactResult :type Hit%20Result%20Structure%20%28by%20ref%29))
  (Actor|DestroyActor))

(event EventBeginPlay
  (Actor|SetLifeSpan 1.5)
  (bind _asthird_person_character (Utilities|Casting|CastToThirdPersonCharacter (Game|GetPlayerCharacter 0)))
  (Variables|Default|SetCharacterREF _asthird_person_character))

(fn ConstructionScript)