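; Short-lived projectile for the Destruction 1 ability that builds marks on enemy hits and cashes them in for damage.
; Overlapping an enemy's Sphere below max marks raises the count on the player character's Destruction1Struct and spawns a mark above the enemy, higher per count.
; At max, the hit applies damage, resets the count and destroys all mark actors in the world, as the count is player-wide.
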(event OnComponentBeginOverlap(Sphere1)
  (params (OverlappedComponent :type Primitive%20Component%20Object%20Reference) (OtherActor :type Actor%20Object%20Reference) (OtherComp :type Primitive%20Component%20Object%20Reference) (OtherBodyIndex :type Integer) (bFromSweep :type Boolean) (SweepResult :type Hit%20Result%20Structure%20%28by%20ref%29))
  (bind _characterref (Variables|Default|GetCharacterREF))
  (bind _characterref_2 (Variables|Default|GetCharacterREF))
  (bind _destruction_1_struct (Variables|/Game/ThirdPersonBP/Blueprints/ThirdPersonCharacter.ThirdPersonCharacter_C|GetDestruction_1_Struct _characterref_2))
  (bind (_maxmarks _currentmarks _damage) (Utilities|Struct|BreakDestruction_1_Struct _destruction_1_struct))
  (bind _asbp_enemy (Utilities|Casting|CastToBP_Enemy OtherActor))
  (Variables|Default|SetEnemyREF _asbp_enemy)
  (if (== (Variables|/Game/Blueprints/BaseEnemy/BP_Enemy.BP_Enemy_C|GetSphere _asbp_enemy) OtherComp)
    (if (> _maxmarks _currentmarks)
      (bind _result (Math|Integer|IncrementInt _currentmarks)
        (:%20%20
          (Utilities|Struct|SetmembersinDestruction_1_Struct _destruction_1_struct _result)
          (Game|SpawnActorfromClass "/Game/Blueprints/Abilities/BP_DestructionMark_1.BP_DestructionMark_1_C" (Math|Transform|MakeTransform (Math|Vector|MakeVector (.x (Transformation|GetActorLocation (Variables|Default|GetEnemyREF))) (.y (Transformation|GetActorLocation (Variables|Default|GetEnemyREF))) (+ (.z (Transformation|GetActorLocation (Variables|Default|GetEnemyREF))) (+ (* _result 20) 1e+02))) "0, 0, 0" "1.000000,1.000000,1.000000") "Undefined" 0 0)
          (Actor|DestroyActor :!label _label)))
      (else
        (Game|Damage|ApplyDamage _asbp_enemy _damage 0 _characterref)
        (Utilities|Struct|SetmembersinDestruction_1_Struct (Variables|/Game/ThirdPersonBP/Blueprints/ThirdPersonCharacter.ThirdPersonCharacter_C|GetDestruction_1_Struct _characterref))
        (bind _outactors (Actor|GetAllActorsOfClass "/Game/Blueprints/Abilities/BP_DestructionMark_1.BP_DestructionMark_1_C"))
        (for _array_element _outactors
          (Actor|DestroyActor _array_element)
          (goto _label))))))

(event EventBeginPlay
  (Actor|SetLifeSpan 1.5)
  (bind _asthird_person_character (Utilities|Casting|CastToThirdPersonCharacter (Game|GetPlayerCharacter 0)))
  (Variables|Default|SetCharacterREF _asthird_person_character))

(fn ConstructionScript)