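; BP_Grenade is a short-lived grenade projectile that reports its impact to the player's ThirdPersonCharacter, which it caches on BeginPlay.
; On hit it plays a sound, then calls the character's GrenadeOverlap with either the struck BP_BaseEnemy actor or, for other surfaces, the hit location.
; Non-enemy hits also spawn a hole particle effect slightly above the impact point.
; The grenade destroys itself on impact or when its lifespan expires.
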(event EventBeginPlay
  (Actor|SetLifeSpan 3.0)
  (bind _asthird_person_character (Utilities|Casting|CastToThirdPersonCharacter (Game|GetPlayerCharacter 0)))
  (Variables|Default|SetCharREF _asthird_person_character))

(event Collision|EventHit
  (params (MyComp :type Primitive%20Component%20Object%20Reference) (Other :type Actor%20Object%20Reference) (OtherComp :type Primitive%20Component%20Object%20Reference) (bSelfMoved :type Boolean) (HitLocation :type Vector :default "0, 0, 0") (HitNormal :type Vector :default "0, 0, 0") (NormalImpulse :type Vector :default "0, 0, 0") (Hit :type Hit%20Result%20Structure%20%28by%20ref%29))
  (bind _charref (Variables|Default|GetCharREF))
  (Audio|PlaySound2D "/Game/Sound/Char/Abilities/grenade_mixdown_01.grenade_mixdown_01" 1.0 1.0 0.0 0 0)
  (Utilities|Casting|CastToBP_BaseEnemy Other
    (:then
      (Default|GrenadeOverlap _charref Other "0, 0, 0" true))
    (:CastFailed
      (Effects|SpawnEmitteratLocation "/Game/VFX/Stylized_FX_Collection_02/ParticleSystem/StylizedFX_04/Hole/P_Hole_01.P_Hole_01" (Math|Vector|MakeVector (.x HitLocation) (.y HitLocation) (+ (.z HitLocation) 5.0)))
      (Default|GrenadeOverlap _charref 0 (Math|Vector|MakeVector (.x HitLocation) (.y HitLocation) (.z HitLocation)) false)))
  (Actor|DestroyActor))

(fn ConstructionScript)