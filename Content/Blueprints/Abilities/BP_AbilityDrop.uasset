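; BP_AbilityDrop is a world pickup that grants the player a Shield or Grenade ability.
; The construction script colours its sphere material to match the configured Ability.
; An overlap sphere shows the E prompt while a ThirdPersonCharacter is inside it.
; Interact assigns the ability and destroys the drop only if the player has no current ability and is not reloading one.
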(event OnComponentBeginOverlap(Sphere1)
  (params (OverlappedComponent :type Primitive%20Component%20Object%20Reference) (OtherActor :type Actor%20Object%20Reference) (OtherComp :type Primitive%20Component%20Object%20Reference) (OtherBodyIndex :type Integer) (bFromSweep :type Boolean) (SweepResult :type Hit%20Result%20Structure%20%28by%20ref%29))
  (Utilities|Casting|CastToThirdPersonCharacter OtherActor)
  (Rendering|SetVisibility (Variables|Default|GetE) true false))

(event OnComponentEndOverlap(Sphere1)
  (params (OverlappedComponent :type Primitive%20Component%20Object%20Reference) (OtherActor :type Actor%20Object%20Reference) (OtherComp :type Primitive%20Component%20Object%20Reference) (OtherBodyIndex :type Integer))
  (Utilities|Casting|CastToThirdPersonCharacter OtherActor)
  (Rendering|SetVisibility (Variables|Default|GetE) false false))

(event EventInteract
  (bind _charref (Variables|Default|GetCharREF))
  (if (not (Variables|/Game/ThirdPersonBP/Blueprints/ThirdPersonCharacter.ThirdPersonCharacter_C|GetIsReloadingAbility _charref))
    (switch Utilities|FlowControl|Switch|SwitchonCurrentAbilities_Enum (Variables|/Game/ThirdPersonBP/Blueprints/ThirdPersonCharacter.ThirdPersonCharacter_C|GetCurrentAbility _charref)
      (:NewEnumerator2
        (Variables|/Game/ThirdPersonBP/Blueprints/ThirdPersonCharacter.ThirdPersonCharacter_C|SetCurrentAbility _charref (Variables|Default|GetAbility))
        (Actor|DestroyActor)))))

(event EventBeginPlay
  (bind _asthird_person_character (Utilities|Casting|CastToThirdPersonCharacter (Game|GetPlayerCharacter 0)))
  (Variables|Default|SetCharREF _asthird_person_character))

(fn ConstructionScript
  (CallFunction|SetColor))

(fn SetColor
  (bind _sphere (Variables|Default|GetSphere))
  (switch Utilities|FlowControl|Switch|SwitchonCurrentAbilities_Enum (Variables|Default|GetAbility)
    (:NewEnumerator2
      (Rendering|Material|SetMaterial _sphere 0 "/Game/Materials/M_Emissive/M_BaseEmissive.M_BaseEmissive"))
    (:NewEnumerator0
      (Rendering|Material|SetMaterial _sphere 0 "/Game/Materials/M_Emissive/MI_Emissive_Teal.MI_Emissive_Teal"))
    (:NewEnumerator1
      (Rendering|Material|SetMaterial _sphere 0 "/Game/Materials/M_Emissive/MI_Emissive_Red.MI_Emissive_Red"))))