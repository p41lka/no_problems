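; Ultimate ability actor that, on spawn, deals one burst of area damage to enemies and heals the player character.
; BeginPlay sizes a sphere from the ultimate struct, damages every overlapping BP_BaseEnemy with the player as causer, then raises health up to the maximum.
; A Super Awakening particle plays at the actor's location; after a short delay a timeline drives its scale before the emitter and actor are destroyed.
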(event Custom|FindEnemiesAndDamage
  (bind _output_get (Variables|Default|SetOverlapping%20Actors (Collision|GetOverlappingActors (Variables|Default|GetSphere) "/Game/Blueprints/Enemies/BaseEnemy/BP_BaseEnemy.BP_BaseEnemy_C" :!class /Script/Engine.PrimitiveComponent)))
  (for _array_element _output_get
    (Game|Damage|ApplyDamage _array_element (.Damage (Utilities|Struct|BreakUltimateSparks_Struct (Variables|Default|GetultimateStruct))) 0 (Variables|Default|GetCharRef))))

(event Custom|HealChar
  (bind _charref (Variables|Default|GetCharRef))
  (Variables|/Game/ThirdPersonBP/Blueprints/ThirdPersonCharacter.ThirdPersonCharacter_C|SetCurrentHealth _charref (Math|Float|Clamp(Float) (Variables|/Game/ThirdPersonBP/Blueprints/ThirdPersonCharacter.ThirdPersonCharacter_C|GetMaxHealth _charref) 0.0 (+ (.Heal (Utilities|Struct|BreakUltimateSparks_Struct (Variables|Default|GetultimateStruct))) (Variables|/Game/ThirdPersonBP/Blueprints/ThirdPersonCharacter.ThirdPersonCharacter_C|GetCurrentHealth _charref)))))

(event EventBeginPlay
  (bind _asthird_person_character (Utilities|Casting|CastToThirdPersonCharacter (Game|GetPlayerCharacter 0)))
  (Variables|Default|SetCharRef _asthird_person_character)
  (Components|Sphere|SetSphereRadius (Variables|Default|GetSphere) (.Radius (Utilities|Struct|BreakUltimateSparks_Struct (Variables|Default|GetultimateStruct))) true)
  (CallFunction|FindEnemiesandDamage)
  (CallFunction|HealChar)
  (bind _returnvalue (Effects|SpawnEmitteratLocation "/Game/VFX/Stylized_FX_Collection_02/ParticleSystem/StylizedFX_04/SuperAwakening/P_SuperAwakening_2.P_SuperAwakening_2" (Transformation|GetActorLocation) "0, 0, 0" "2.000000,2.000000,2.000000"))
  (Utilities|FlowControl|Delay 2.0)
  (bind _newtrack_0 (Timeline|HideParticle PlayFromStart)
    (:Update
      (Transformation|SetWorldScale3D _returnvalue (Math|Vector|MakeVector _newtrack_0 _newtrack_0 _newtrack_0)))
    (:Finished
      (Components|DestroyComponent _returnvalue)
      (Actor|DestroyActor))))

(fn ConstructionScript)