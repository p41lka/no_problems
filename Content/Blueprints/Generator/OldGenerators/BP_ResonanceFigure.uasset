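; Resonance figure actor for a generator, shown as a circle, line or cross that the player steps into to resonate.
; SpawnFigure stores the generator, then shows the chosen shape and enables only its overlap collision.
; Character overlaps tell the generator to start or end resonating.
; Start and end events swap the shape's material to emissive blue and back while timelines scale the circle or rotate the line and cross.
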(event OnComponentBeginOverlap(CircleCollision)
  (params (OverlappedComponent :type Primitive%20Component%20Object%20Reference) (OtherActor :type Actor%20Object%20Reference) (OtherComp :type Primitive%20Component%20Object%20Reference) (OtherBodyIndex :type Integer) (bFromSweep :type Boolean) (SweepResult :type Hit%20Result%20Structure%20%28by%20ref%29))
  (Utilities|Casting|CastToThirdPersonCharacter OtherActor)
  (Default|StartResonating (Variables|Default|GetGenerator)))

(event OnComponentEndOverlap(CircleCollision)
  (params (OverlappedComponent :type Primitive%20Component%20Object%20Reference) (OtherActor :type Actor%20Object%20Reference) (OtherComp :type Primitive%20Component%20Object%20Reference) (OtherBodyIndex :type Integer))
  (Utilities|Casting|CastToThirdPersonCharacter OtherActor)
  (Default|EndResonating (Variables|Default|GetGenerator) false))

(event OnComponentBeginOverlap(LineCollision)
  (params (OverlappedComponent :type Primitive%20Component%20Object%20Reference) (OtherActor :type Actor%20Object%20Reference) (OtherComp :type Primitive%20Component%20Object%20Reference) (OtherBodyIndex :type Integer) (bFromSweep :type Boolean) (SweepResult :type Hit%20Result%20Structure%20%28by%20ref%29))
  (Utilities|Casting|CastToThirdPersonCharacter OtherActor)
  (Default|StartResonating (Variables|Default|GetGenerator)))

(event OnComponentEndOverlap(LineCollision)
  (params (OverlappedComponent :type Primitive%20Component%20Object%20Reference) (OtherActor :type Actor%20Object%20Reference) (OtherComp :type Primitive%20Component%20Object%20Reference) (OtherBodyIndex :type Integer))
  (Utilities|Casting|CastToThirdPersonCharacter OtherActor)
  (Default|EndResonating (Variables|Default|GetGenerator) false))

(event OnComponentBeginOverlap(Cross1_Collision)
  (params (OverlappedComponent :type Primitive%20Component%20Object%20Reference) (OtherActor :type Actor%20Object%20Reference) (OtherComp :type Primitive%20Component%20Object%20Reference) (OtherBodyIndex :type Integer) (bFromSweep :type Boolean) (SweepResult :type Hit%20Result%20Structure%20%28by%20ref%29))
  (Utilities|Casting|CastToThirdPersonCharacter OtherActor)
  (Default|StartResonating (Variables|Default|GetGenerator)))

(event OnComponentEndOverlap(Cross1_Collision)
  (params (OverlappedComponent :type Primitive%20Component%20Object%20Reference) (OtherActor :type Actor%20Object%20Reference) (OtherComp :type Primitive%20Component%20Object%20Reference) (OtherBodyIndex :type Integer))
  (Utilities|Casting|CastToThirdPersonCharacter OtherActor)
  (Default|EndResonating (Variables|Default|GetGenerator) false))

(event OnComponentBeginOverlap(Cross2_Collision)
  (params (OverlappedComponent :type Primitive%20Component%20Object%20Reference) (OtherActor :type Actor%20Object%20Reference) (OtherComp :type Primitive%20Component%20Object%20Reference) (OtherBodyIndex :type Integer) (bFromSweep :type Boolean) (SweepResult :type Hit%20Result%20Structure%20%28by%20ref%29))
  (Utilities|Casting|CastToThirdPersonCharacter OtherActor)
  (Default|StartResonating (Variables|Default|GetGenerator)))

(event OnComponentEndOverlap(Cross2_Collision)
  (params (OverlappedComponent :type Primitive%20Component%20Object%20Reference) (OtherActor :type Actor%20Object%20Reference) (OtherComp :type Primitive%20Component%20Object%20Reference) (OtherBodyIndex :type Integer))
  (Utilities|Casting|CastToThirdPersonCharacter OtherActor)
  (Default|EndResonating (Variables|Default|GetGenerator) false))

(event EventSpawnFigure
  (params (Figure :type ResonanceFigures_Enum%20Enum :default "NewEnumerator0") (Generator :type BP%20New%20Generator%20Object%20Reference))
  (Variables|Default|SetGenerator Generator)
  (bind _output_get (Variables|Default|SetCurrentFigure Figure))
  (switch Utilities|FlowControl|Switch|SwitchonResonanceFigures_Enum _output_get
    (:NewEnumerator0
      (Rendering|SetVisibility (Variables|Default|GetCircle) true false)
      (Rendering|SetVisibility (Variables|Default|GetLine) false false)
      (Rendering|SetVisibility (Variables|Default|GetCross) false true)
      (Variables|/Script/Engine.PrimitiveComponent|SetbGenerateOverlapEvents (Variables|Default|GetCircleCollision) true)
      (Variables|/Script/Engine.PrimitiveComponent|SetbGenerateOverlapEvents (Variables|Default|GetLineCollision) false)
      (Variables|/Script/Engine.PrimitiveComponent|SetbGenerateOverlapEvents (Variables|Default|GetCross1_Collision) false)
      (Variables|/Script/Engine.PrimitiveComponent|SetbGenerateOverlapEvents (Variables|Default|GetCross2_Collision) false))
    (:NewEnumerator1
      (Rendering|SetVisibility (Variables|Default|GetCircle) false false)
      (Rendering|SetVisibility (Variables|Default|GetLine) true false)
      (Rendering|SetVisibility (Variables|Default|GetCross) false true)
      (Variables|/Script/Engine.PrimitiveComponent|SetbGenerateOverlapEvents (Variables|Default|GetCircleCollision) false)
      (Variables|/Script/Engine.PrimitiveComponent|SetbGenerateOverlapEvents (Variables|Default|GetLineCollision) true)
      (Variables|/Script/Engine.PrimitiveComponent|SetbGenerateOverlapEvents (Variables|Default|GetCross1_Collision) false)
      (Variables|/Script/Engine.PrimitiveComponent|SetbGenerateOverlapEvents (Variables|Default|GetCross2_Collision) false))
    (:NewEnumerator2
      (Rendering|SetVisibility (Variables|Default|GetCircle) false false)
      (Rendering|SetVisibility (Variables|Default|GetLine) false false)
      (Rendering|SetVisibility (Variables|Default|GetCross) true true)
      (Variables|/Script/Engine.PrimitiveComponent|SetbGenerateOverlapEvents (Variables|Default|GetCircleCollision) false)
      (Variables|/Script/Engine.PrimitiveComponent|SetbGenerateOverlapEvents (Variables|Default|GetLineCollision) false)
      (Variables|/Script/Engine.PrimitiveComponent|SetbGenerateOverlapEvents (Variables|Default|GetCross1_Collision) true)
      (Variables|/Script/Engine.PrimitiveComponent|SetbGenerateOverlapEvents (Variables|Default|GetCross2_Collision) true))))

(event EventStartResonatingFigure
  (switch Utilities|FlowControl|Switch|SwitchonResonanceFigures_Enum (Variables|Default|GetCurrentFigure)
    (:NewEnumerator0
      (Rendering|Material|SetMaterial (Variables|Default|GetCircle) 0 "/Game/Materials/M_Emissive/M_Emissive_Blue.M_Emissive_Blue")
      (bind _scalecircle (Timeline|ChangeCircle Play)
        (:Update
          (Transformation|SetWorldScale3D (Variables|Default|GetCircle) _scalecircle))))
    (:NewEnumerator1
      (Rendering|Material|SetMaterial (Variables|Default|GetLine) 0 "/Game/Materials/M_Emissive/M_Emissive_Blue.M_Emissive_Blue")
      (bind _addrotation (Timeline|RotateLine Play)
        (:Update
          (Transformation|AddWorldRotation (Variables|Default|GetLine) (Math|Rotator|MakeRotator 0.0 0.0 _addrotation) false false))))
    (:NewEnumerator2
      (Rendering|Material|SetMaterial (Variables|Default|GetCross1) 0 "/Game/Materials/M_Emissive/M_Emissive_Blue.M_Emissive_Blue")
      (bind _addrotation_2 (Timeline|Timeline_0 Play)
        (:Update
          (Transformation|AddWorldRotation (Variables|Default|GetCross) (Math|Rotator|MakeRotator 0.0 0.0 _addrotation_2) false false))))))

(event EventEndResonatingFigure
  (switch Utilities|FlowControl|Switch|SwitchonResonanceFigures_Enum (Variables|Default|GetCurrentFigure)
    (:NewEnumerator0
      (Rendering|Material|SetMaterial (Variables|Default|GetCircle) 0 "/Game/Materials/M_Enemies/M_Circle.M_Circle")
      (bind _scalecircle (Timeline|ChangeCircle Stop)
        (:Update
          (Transformation|SetWorldScale3D (Variables|Default|GetCircle) _scalecircle))))
    (:NewEnumerator1
      (Rendering|Material|SetMaterial (Variables|Default|GetLine) 0 "/Game/Materials/M_Enemies/M_Circle.M_Circle")
      (bind _addrotation (Timeline|RotateLine Stop)
        (:Update
          (Transformation|AddWorldRotation (Variables|Default|GetLine) (Math|Rotator|MakeRotator 0.0 0.0 _addrotation) false false))))
    (:NewEnumerator2
      (Rendering|Material|SetMaterial (Variables|Default|GetCross1) 0 "/Game/Materials/M_Enemies/M_Circle.M_Circle")
      (bind _addrotation_2 (Timeline|Timeline_0 Stop)
        (:Update
          (Transformation|AddWorldRotation (Variables|Default|GetCross) (Math|Rotator|MakeRotator 0.0 0.0 _addrotation_2) false false))))))

(fn ConstructionScript)

(fn IsGeneratorReloading
  (params (IsReloading :type Boolean))
  (return false))