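; Resonance generator that grants the player an ability matching its enemy aspect, plus ammo, once resonated long enough.
; On BeginPlay it spawns a resonance figure character, and a looping timer fills the UI progress while resonating.
; Failed attempts start a decay timer intended to drain progress and damage the player at zero.
; Success triggers a tick-counted reload with material swaps; the surface-trace check is unused and IsGeneratorReloading always returns false.
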(event Custom|Resonance
  (bind _characterref (Variables|Default|GetCharacterREF))
  (bind _characterref_2 (Variables|Default|GetCharacterREF))
  ;[0 0 0] Resonance Timer
  (if (Variables|Default|GetIsGeneratorResonating)
    (if (< (Variables|Default|GetCurrentTime) (Variables|Default|GetResonanceTime))
      (bind _result (Math|Float|IncrementFloat (Variables|Default|GetCurrentTime))
        (:%20%20
          (Variables|/Game/Widgets/W_CharacterInterface.W_CharacterInterface_C|SetCurrentResonanceTime (Variables|/Game/ThirdPersonBP/Blueprints/ThirdPersonCharacter.ThirdPersonCharacter_C|GetInterfaceREF (Variables|Default|GetCharacterREF)) _result)
          (if (>= (Variables|Default|GetCurrentTime) (Variables|Default|GetResonanceTime))
            (Variables|/Game/ThirdPersonBP/Blueprints/ThirdPersonCharacter.ThirdPersonCharacter_C|SetIsUsingBoost (Variables|Default|GetCharacterREF) true)
            ;;[0 0 0] Set ability from enemy aspect
            (switch Utilities|FlowControl|Switch|SwitchonEnemyAspects_Enum (Variables|Default|GetEnemyAspects)
              (:NewEnumerator0
                (Default|SetFaithAbility _characterref_2))
              (:NewEnumerator1
                (Default|SetDestructionAbility _characterref_2))
              (:NewEnumerator2
                (Default|SetBondAbility _characterref_2))
              (:NewEnumerator3
                (Default|SetRenewalAbility _characterref_2)))
            (CallFunction|EndResonating true)
            (Variables|Default|SetIsReloading true)
            ;[0 0 0] Add Ammo
            (Variables|/Game/ThirdPersonBP/Blueprints/ThirdPersonCharacter.ThirdPersonCharacter_C|SetCurrentDopAmmo _characterref (Math|Integer|Clamp(Integer) (+ (Variables|/Game/ThirdPersonBP/Blueprints/ThirdPersonCharacter.ThirdPersonCharacter_C|GetCurrentDopAmmo _characterref) (Variables|Default|GetAmmoAmount)) 0 (Variables|/Game/ThirdPersonBP/Blueprints/ThirdPersonCharacter.ThirdPersonCharacter_C|GetMaxDopAmmo _characterref)))
            (Niagara|SpawnSystematLocation "/Game/VFX/Hack_And_Slash_FX/VFX_Niagara/Impacts/NS_Cyber_Slash_Impact.NS_Cyber_Slash_Impact" (Transformation|GetActorLocation))
            (Rendering|Material|SetMaterial (Variables|Default|GetResonator) 0 "/Game/Materials/M_Unlit/M_LightBlue.M_LightBlue")))))))

(event Custom|StartResonating
  ;[0 0 0] Start and End Resonating
  (if (not (Variables|Default|GetIsReloading))
    (Utilities|Time|ClearandInvalidateTimerbyHandle (Variables|Default|GetdownResTimer))
    (if (not (Variables|/Game/ThirdPersonBP/Blueprints/ThirdPersonCharacter.ThirdPersonCharacter_C|GetIsUsingBoost (Variables|Default|GetCharacterREF)))
      (Default|SetLatestGenerator (Variables|Default|GetCharacterREF) (Variables|Default|GetEnemyAspects))
      (Default|StartResonatingFigure (Variables|Default|GetResonanceCharREF))
      (Variables|Default|SetIsGeneratorResonating true)
      ;[0 0 0] Resonance Timer
      (bind _returnvalue (Utilities|Time|SetTimerbyEvent (delegate Custom|Resonance) 0.5 true))
      (Variables|Default|SetResTimer _returnvalue))))

(event Custom|ResDown
  (bind _downres (Variables|Default|GetdownRes))
  (bind (_downtime _downamount _damage) (Utilities|Struct|BreakGeneratorDown_Struct _downres))
  ;[0 0 0] Fail Resonate Timer
  (bind _output_get (Variables|Default|SetCurrentTime (- (Variables|Default|GetCurrentTime) _downamount)))
  (Variables|/Game/Widgets/W_CharacterInterface.W_CharacterInterface_C|SetCurrentResonanceTime (Variables|/Game/ThirdPersonBP/Blueprints/ThirdPersonCharacter.ThirdPersonCharacter_C|GetInterfaceREF (Variables|Default|GetCharacterREF)) (Math|Float|Clamp(Float) _output_get 0.0 (Variables|Default|GetResonanceTime)))
  (if (not (> (Math|Float|Clamp(Float) _output_get 0.0 (Variables|Default|GetResonanceTime)) 0.0))
    (Game|Damage|ApplyDamage (Variables|Default|GetCharacterREF) _damage 0 self)
    (Utilities|Time|ClearandInvalidateTimerbyHandle (Variables|Default|GetdownResTimer))))

(event Custom|EndResonating
  (params (success :type Boolean))
  ;[0 0 0] Start and End Resonating
  (Default|EndResonatingFigure (Variables|Default|GetResonanceCharREF))
  (Utilities|Time|ClearandInvalidateTimerbyHandle (Variables|Default|GetResTimer))
  (Variables|Default|SetIsGeneratorResonating false)
  (if (or success (Variables|/Game/ThirdPersonBP/Blueprints/ThirdPersonCharacter.ThirdPersonCharacter_C|GetIsUsingBoost (Variables|Default|GetCharacterREF)))
    (Variables|Default|SetCurrentTime 0.0)
    (Variables|/Game/Widgets/W_CharacterInterface.W_CharacterInterface_C|SetCurrentResonanceTime (Variables|/Game/ThirdPersonBP/Blueprints/ThirdPersonCharacter.ThirdPersonCharacter_C|GetInterfaceREF (Variables|Default|GetCharacterREF)) 0.0)
    (else
      ;[0 0 0] Fail Resonate Timer
      (bind _returnvalue (Utilities|Time|SetTimerbyEvent (EventDispatchers|CreateEvent :!event Custom|ResDown) (.downTime (Utilities|Struct|BreakGeneratorDown_Struct (Variables|Default|GetdownRes))) true))
      (Variables|Default|SetdownResTimer _returnvalue))))

(event Custom|CheckMaterial
  ;[0 0 0] Check Step on Material // NOT IN USE
)

(event EventTick
  (params (DeltaSeconds :type Float%20%28single-precision%29))
  ;[0 0 0] Reloading
  (CallFunction|CheckMaterial)
  (if (Variables|Default|GetIsReloading)
    (bind _output_get (Variables|Default|SetCurrentGeneratorReloadTime (+ (Variables|Default|GetCurrentGeneratorReloadTime) 1.0)))
    (if (< _output_get (Variables|Default|GetGeneratorReloadTime))
      (Variables|Default|SetIsReloading true)
      (else
        (Variables|Default|SetIsReloading false)
        (Variables|Default|SetCurrentGeneratorReloadTime 0.0)
        (Rendering|Material|SetMaterial (Variables|Default|GetResonator) 0 "/Game/Materials/M_Emissive/M_Emissive_Blue.M_Emissive_Blue")))
    (else
      (Variables|Default|SetCurrentGeneratorReloadTime 0.0))))

(event EventBeginPlay
  (bind _returnvalue (Transformation|GetActorLocation))
  (bind _asthird_person_character (Utilities|Casting|CastToThirdPersonCharacter (Game|GetPlayerCharacter 0)))
  (Variables|Default|SetCharacterREF _asthird_person_character)
  ;[0 0 0] Set points
  (bind _output_get (Variables|Default|SetActorRelativeLocation (Transformation|GetActorLocation)))
  (Variables|Default|SetPoint1 (+ _output_get (Variables|Default|GetPoint1)))
  (Variables|Default|SetPoint2 (+ _output_get (Variables|Default|GetPoint2)))
  (Variables|Default|SetPoint3 (+ _output_get (Variables|Default|GetPoint3)))
  (Variables|Default|SetPoint4 (+ _output_get (Variables|Default|GetPoint4)))
  (Variables|Default|SetPoint5 (+ _output_get (Variables|Default|GetPoint5)))
  (Variables|Default|SetPoint6 (+ _output_get (Variables|Default|GetPoint6)))
  ;[0 0 0] Spawn Resonate Figure
  (bind _returnvalue_2 (Game|SpawnActorfromClass "/Game/Blueprints/Generator/OldGenerators/BP_Resonance_Fig_Char.BP_Resonance_Fig_Char_C" (Math|Transform|MakeTransform (Math|Vector|MakeVector (+ (.x _returnvalue) 2e+02) (+ (.y _returnvalue) 2e+02) (- (.z _returnvalue) 6e+01)) "0, 0, 0" "1.000000,1.000000,1.000000") "Undefined" 0 0))
  (bind _output_get_2 (Variables|Default|SetResonanceCharREF _returnvalue_2))
  (Default|SpawnFigure _output_get_2 (Variables|Default|GetResonanceFigure) self))

(fn ConstructionScript)

(fn IsGeneratorReloading
  (params (IsReloading :type Boolean))
  (return false))