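; Enemy generator actor that grants the player an aspect ability through resonance and constantly spawns enemy projectiles from BeginPlay.
; Overlapping ResonanceCollision without an active boost lights the figure and starts a looping timer that advances the UI's resonance counter.
; At the threshold it sets the boost flag and grants Faith, Destruction or Renewal by EnemyAspects.
; The floor physical-material trace that sets IsGeneratorResonating, which gates counting, and the reload countdown are unwired.
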(event OnComponentBeginOverlap(ResonanceCollision)
  (params (OverlappedComponent :type Primitive%20Component%20Object%20Reference) (OtherActor :type Actor%20Object%20Reference) (OtherComp :type Primitive%20Component%20Object%20Reference) (OtherBodyIndex :type Integer) (bFromSweep :type Boolean) (SweepResult :type Hit%20Result%20Structure%20%28by%20ref%29))
  (Utilities|Casting|CastToThirdPersonCharacter OtherActor)
  (if (not (Variables|/Game/ThirdPersonBP/Blueprints/ThirdPersonCharacter.ThirdPersonCharacter_C|GetIsUsingBoost (Variables|Default|GetCharacterREF)))
    (CallFunction|StartResonationg)
    ;[0 0 0] Resonance Timer
    (bind _returnvalue (Utilities|Time|SetTimerbyEvent (delegate Custom|Resonance) 0.5 true))
    (Variables|Resonance|SetResTimer _returnvalue)))

(event OnComponentEndOverlap(ResonanceCollision)
  (params (OverlappedComponent :type Primitive%20Component%20Object%20Reference) (OtherActor :type Actor%20Object%20Reference) (OtherComp :type Primitive%20Component%20Object%20Reference) (OtherBodyIndex :type Integer))
  (Utilities|Casting|CastToThirdPersonCharacter OtherActor)
  (CallFunction|EndResonatingFigure))

(event Custom|Resonance
  (bind _characterref (Variables|Default|GetCharacterREF))
  ;[0 0 0] Resonance Timer
  (if (not (Variables|Resonance|GetIsGeneratorReloading_0))
    (if (Variables|Resonance|GetIsGeneratorResonating)
      (if (< (Variables|Resonance|GetCurrentTime) (Variables|Resonance|GetResonanceTime))
        (bind _result (Math|Float|IncrementFloat (Variables|Resonance|GetCurrentTime))
          (:%20%20
            (Variables|/Game/Widgets/W_CharacterInterface.W_CharacterInterface_C|SetCurrentResonanceTime (Variables|/Game/ThirdPersonBP/Blueprints/ThirdPersonCharacter.ThirdPersonCharacter_C|GetInterfaceREF (Variables|Default|GetCharacterREF)) _result)
            (if (>= (Variables|Resonance|GetCurrentTime) (Variables|Resonance|GetResonanceTime))
              (Variables|/Game/ThirdPersonBP/Blueprints/ThirdPersonCharacter.ThirdPersonCharacter_C|SetIsUsingBoost (Variables|Default|GetCharacterREF) true)
              ;;[0 0 0] Set ability from enemy aspect
              (switch Utilities|FlowControl|Switch|SwitchonEnemyAspects_Enum (Variables|Aspects|GetEnemyAspects)
                (:NewEnumerator0
                  (Default|SetFaithAbility _characterref))
                (:NewEnumerator1
                  (Default|SetDestructionAbility _characterref))
                (:NewEnumerator3
                  (Default|SetRenewalAbility _characterref)))
              (CallFunction|EndResonatingFigure))))))))

(event Custom|StartResonationg
  (Rendering|Material|SetMaterial (Variables|Default|GetResonanceFigure) 0 "/Game/Materials/M_Enemies/M_Resonance_Emissive.M_Resonance_Emissive")
  (CallFunction|ChangeFigure))

(event Custom|PassiveAttack
  ;[0 0 0] don't need yet
  ;;[0 0 0] Spawn Projectiles
  (bind _returnvalue (Utilities|Time|SetTimerbyEvent (delegate Custom|PassiveAttackSpawn) 0.4 true))
  (Variables|Default|SetAttackTimer _returnvalue))

(event Custom|PassiveAttackSpawn
  (bind _attackspawn (Variables|Default|GetAttackSpawn))
  ;[0 0 0] don't need yet
  ;;[0 0 0] Spawn Projectiles
  (Game|SpawnActorfromClass "/Game/Blueprints/Enemies/BaseEnemy/BP_EnemyProjectiles.BP_EnemyProjectiles_C" (Math|Transform|MakeTransform (Transformation|GetWorldLocation _attackspawn) (Transformation|GetWorldRotation _attackspawn) "0.500000,0.500000,0.500000") "Undefined" 0 0))

(event Custom|EndResonating
  (Rendering|Material|SetMaterial (Variables|Default|GetResonanceFigure) 0 "/Game/Materials/M_Enemies/M_Circle.M_Circle")
  (Utilities|Time|ClearandInvalidateTimerbyHandle (Variables|Resonance|GetResTimer))
  (Variables|Resonance|SetCurrentTime 0.0)
  (Variables|/Game/Widgets/W_CharacterInterface.W_CharacterInterface_C|SetCurrentResonanceTime (Variables|/Game/ThirdPersonBP/Blueprints/ThirdPersonCharacter.ThirdPersonCharacter_C|GetInterfaceREF (Variables|Default|GetCharacterREF)) 0.0))

(event Custom|CheckMaterial
  (bind _returnvalue (Game|GetPlayerCharacter 0))
  (bind _returnvalue_2 (Transformation|GetActorLocation _returnvalue))
  (bind _outhit (Collision|LineTraceByChannel _returnvalue_2 (- _returnvalue_2 "0,0.000000,300.000000") "TraceTypeQuery1" false 0 "ForDuration" true "(R=1.000000,G=0.000000,B=0.000000,A=1.000000)" "(R=0.000000,G=1.000000,B=0.000000,A=1.000000)" 1.0))
  (Development|PrintString (Utilities|GetDisplayName (.HitActor (Collision|BreakHitResult _outhit))) true true "(R=0.000000,G=0.660000,B=1.000000,A=1.000000)" 0.0)
  (bind _output_get (Variables|Resonance|SetIsGeneratorResonating (Utilities|Select :Index (Variables|/Script/PhysicsCore.PhysicalMaterial|GetSurfaceType (.PhysMat (Collision|BreakHitResult _outhit))) :SurfaceType_Default false :SurfaceType1 true)))
  (Development|PrintString (Utilities|String|ToString(Boolean) _output_get) true true "(R=0.000000,G=0.660000,B=1.000000,A=1.000000)" 0.0))

(event Custom|ChangeFigure)

(event EventTick
  (params (DeltaSeconds :type Float%20%28single-precision%29)))

(event EventBeginPlay
  (Variables|Default|SetCurrentHealth (Variables|Default|GetMaxHealth))
  (bind _asthird_person_character (Utilities|Casting|CastToThirdPersonCharacter (Game|GetPlayerCharacter 0)))
  (Variables|Default|SetCharacterREF _asthird_person_character)
  ;[1 1 1] Enemy passive attack
  (CallFunction|PassiveAttack))

(fn ConstructionScript)

(fn IsGeneratorReloading
  (params (IsReloading :type Boolean))
  (return false))