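; Interactable generator tied to one of four aspects that, once activated, grants the player that aspect's boost inside its linked areas.
; Activation starts a work timer and, unless the player already has that Spark, spawns enemies at line-of-sight-checked navmesh points around them.
; Staying in the areas long enough awards the Spark.
; A looping timer handles boost handover between overlapping generators; timelines animate parts and aspect particles.
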(event OnComponentBeginOverlap(interactableCollision)
  (params (OverlappedComponent :type Primitive%20Component%20Object%20Reference) (OtherActor :type Actor%20Object%20Reference) (OtherComp :type Primitive%20Component%20Object%20Reference) (OtherBodyIndex :type Integer) (bFromSweep :type Boolean) (SweepResult :type Hit%20Result%20Structure%20%28by%20ref%29))
  ;[0 0 0] Interact Widget
  (Utilities|Casting|CastToThirdPersonCharacter OtherActor)
  (if (not (Variables|Default|GetisActive))
    (Rendering|SetVisibility (Variables|Default|GetInteractionWidget) true false)))

(event OnComponentEndOverlap(interactableCollision)
  (params (OverlappedComponent :type Primitive%20Component%20Object%20Reference) (OtherActor :type Actor%20Object%20Reference) (OtherComp :type Primitive%20Component%20Object%20Reference) (OtherBodyIndex :type Integer))
  ;[0 0 0] Interact Widget
  (Utilities|Casting|CastToThirdPersonCharacter OtherActor)
  (Rendering|SetVisibility (Variables|Default|GetInteractionWidget) false false))

(event Custom|Start
  ;[0 0 0] StartResonate
  (Variables|Default|SetisActive true)
  (CallFunction|FindOverlappingAreas)
  (Utilities|Time|SetTimerbyEvent (EventDispatchers|CreateEvent :!event Custom|Stop) (.workTime (Utilities|Struct|BreakNewNewGen_struct (Variables|Default|GetgenStruct))))
  (CallFunction|SetAreasActivation true)
  (if (CallFunction|CheckSpark)
    _
    (else
      (CallFunction|SpawnEnemies)))
  (if (CallFunction|CheckOverlappingZones)
    (CallFunction|SetCharSkill true)
    (CallFunction|StartTimerforSpark)))

(event Custom|Stop
  (bind _charref (Variables|Default|GetcharRef))
  ;[0 0 0] StopResonating
  (if (not (Variables|Default|GetgaveSpark))
    (Variables|Default|SetisActive false)
    (CallFunction|SetAreasActivation false)
    (Utilities|Array|Clear (Variables|Default|GetoverlappingAreas))
    (if (CallFunction|CheckSamePower)
      (CallFunction|SetCharSkill false))
    (Utilities|Time|ClearandInvalidateTimerbyHandle (Variables|Default|GettimerForGiveAbility))
    (CallFunction|ClearSparkTimer)
    (if (not (Variables|/Game/ThirdPersonBP/Blueprints/ThirdPersonCharacter.ThirdPersonCharacter_C|GetisOnNewGen _charref))
      (Variables|/Game/ThirdPersonBP/Blueprints/ThirdPersonCharacter.ThirdPersonCharacter_C|SetcurrentNewNewGeneratorRef _charref 0))))

(event Custom|SpawnEnemies
  ;[0 0 0] SpawnEnemies
  (for _array_element (Variables|Default|GetenemiesToSpawn)
    (bind _outactors (Actor|GetAllActorsOfClass (.enemyClass (Utilities|Struct|BreakGenEnemiesSpawn_struct _array_element))))
    (if (Utilities|Array|IsEmpty _outactors)
      _
      (else
        (for _array_element_2 _outactors
          (Actor|DestroyActor _array_element_2))))
    (for _index (range 1 (.amount (Utilities|Struct|BreakGenEnemiesSpawn_struct _array_element)))
      (if (.isSpawned (CallFunction|CanSpawnEnemy (.radius (Utilities|Struct|BreakGenEnemiesSpawn_struct _array_element))))
        (bind _returnvalue (Game|SpawnActorfromClass (.enemyClass (Utilities|Struct|BreakGenEnemiesSpawn_struct _array_element)) (Math|Transform|MakeTransform (.place (CallFunction|CanSpawnEnemy (.radius (Utilities|Struct|BreakGenEnemiesSpawn_struct _array_element)))) (.rotation (CallFunction|CanSpawnEnemy (.radius (Utilities|Struct|BreakGenEnemiesSpawn_struct _array_element)))) "1.000000,1.000000,1.000000") "AdjustIfPossibleButAlwaysSpawn" 0 0))
        (Variables|/Game/Blueprints/Enemies/BaseEnemy/BP_BaseEnemy.BP_BaseEnemy_C|SetbattleEndRef _returnvalue (Variables|Default|GetbattleEndRef))
        (Variables|/Game/Blueprints/Enemies/BaseEnemy/BP_BaseEnemy.BP_BaseEnemy_C|SetDropAbility _returnvalue (Utilities|Select :Index (Math|Random|RandomIntegerinRange 0 1) :Option%200 "NewEnumerator0" :Option%201 "NewEnumerator1"))
        (if (== (Variables|Default|GetPackInt) 0)
          (bind _output_get (Variables|/Game/Blueprints/Enemies/BaseEnemy/BP_BaseEnemy.BP_BaseEnemy_C|SetCanDropAbility _returnvalue (Math|Random|RandomBool)))
          (if _output_get
            (Math|Integer|IncrementInt (Variables|Default|GetPackInt))))))))

(event Custom|Particles
  (bind _returnvalue (Transformation|GetActorLocation))
  ;[0 0 0] Animate Particle
  (switch Utilities|FlowControl|Switch|SwitchonEnemyAspects_Enum (Variables|Default|GetenemyAspect)
    (:NewEnumerator0
      (bind _returnvalue_2 (Effects|SpawnEmitteratLocation "/Game/VFX/StylizedFX_Collection_1/Particles/StylizedFX_01/P_Lightning_Orb_01.P_Lightning_Orb_01" _returnvalue "0, 0, 0" "2.000000,2.000000,2.000000"))
      (Variables|Default|SetParticleResonate _returnvalue_2))
    (:NewEnumerator1
      (bind _returnvalue_3 (Effects|SpawnEmitteratLocation "/Game/VFX/StylizedFX_Collection_1/Particles/StylizedFX_01/P_Lightning_Orb_02.P_Lightning_Orb_02" _returnvalue "0, 0, 0" "2.000000,2.000000,2.000000"))
      (Variables|Default|SetParticleResonate _returnvalue_3))
    (:NewEnumerator2
      (bind _returnvalue_4 (Effects|SpawnEmitteratLocation "/Game/VFX/StylizedFX_Collection_1/Particles/StylizedFX_01/P_Lightning_Orb_03.P_Lightning_Orb_03" _returnvalue "0, 0, 0" "2.000000,2.000000,2.000000"))
      (Variables|Default|SetParticleResonate _returnvalue_4))
    (:NewEnumerator3
      (bind _returnvalue_5 (Effects|SpawnEmitteratLocation "/Game/VFX/StylizedFX_Collection_1/Particles/StylizedFX_01/P_Lightning_Orb_04.P_Lightning_Orb_04" _returnvalue "0, 0, 0" "2.000000,2.000000,2.000000"))
      (Variables|Default|SetParticleResonate _returnvalue_5)))
  (CallFunction|ScaleParticle))

(event Custom|ScaleParticle
  (bind _particleresonate (Variables|Default|GetParticleResonate))
  ;[0 0 0] Animate Particle
  (bind _newtrack_0 (Timeline|PerticleTimeline PlayFromStart)
    (:Update
      (Transformation|SetWorldScale3D _particleresonate (Math|Vector|MakeVector _newtrack_0 _newtrack_0 _newtrack_0)))
    (:Finished
      (Utilities|FlowControl|Delay 1.0)
      (bind _newtrack_0_2 (Timeline|Timeline_3 ReverseFromEnd)
        (:Update
          (Transformation|SetWorldScale3D _particleresonate (Math|Vector|MakeVector _newtrack_0_2 _newtrack_0_2 _newtrack_0_2)))
        (:Finished
          (Components|DestroyComponent _particleresonate))))))

(event Custom|StartTimerForSpark
  ;[0 0 0] SparkTimer
  (if (not (or (CallFunction|CheckSpark) (Variables|Default|GetgaveSpark)))
    (bind _returnvalue (Utilities|Time|SetTimerbyEvent (delegate Custom|GetSpark) (.timeSpark (Utilities|Struct|BreakNewNewGen_struct (Variables|Default|GetgenStruct)))))
    (Variables|Default|SetsparkTimer _returnvalue)
    (Rendering|SetVisibility (Variables|Default|GetWidget) true false)))

(event Custom|GetSpark
  ;[0 0 0] SparkTimer
  (Default|SetSpark (Variables|Default|GetcharRef) (Variables|Default|GetenemyAspect))
  (CallFunction|ClearSparkTimer)
  (Variables|Default|SetgaveSpark true))

(event Custom|SetCharSkill
  (params (isAspect :type Boolean))
  (bind _charref (Variables|Default|GetcharRef))
  (bind _charref_2 (Variables|Default|GetcharRef))
  ;[0 0 0] SetCharSkill
  (Variables|/Game/ThirdPersonBP/Blueprints/ThirdPersonCharacter.ThirdPersonCharacter_C|SetisOnNewGen _charref false)
  (Default|ResetBoosts _charref)
  (if isAspect
    (Variables|/Game/ThirdPersonBP/Blueprints/ThirdPersonCharacter.ThirdPersonCharacter_C|SetisOnNewGen _charref true)
    (Variables|/Game/ThirdPersonBP/Blueprints/ThirdPersonCharacter.ThirdPersonCharacter_C|SetcurrentNewNewGeneratorRef _charref self)
    (switch Utilities|FlowControl|Switch|SwitchonEnemyAspects_Enum (Variables|Default|GetenemyAspect)
      (:NewEnumerator0
        (Default|SetFaithBoost _charref_2))
      (:NewEnumerator1
        (Default|SetDestructionBoost _charref_2))
      (:NewEnumerator2
        (Default|SetBondBoost _charref_2))
      (:NewEnumerator3
        (Default|SetRenewalBoost _charref_2)))))

(event Custom|SetAreasActivation
  (params (isOn :type Boolean))
  (bind _genareas (Variables|Default|GetgenAreas))
  ;[0 0 0] AreaActivationAndDeactivation
  (if isOn
    (for _array_element _genareas
      (Default|Activate _array_element))
    (else
      (for _array_element_2 _genareas
        (Default|Disable _array_element_2)))))

(event Custom|GenEndOverlap
  (bind _charref (Variables|Default|GetcharRef))
  ;[0 0 0] StopResonating
  (if (not (CallFunction|CheckOverlappingZones))
    (Utilities|Array|Clear (Variables|Default|GetoverlappingAreas))
    (if (CallFunction|CheckSamePower)
      (CallFunction|SetCharSkill false))
    (CallFunction|ClearSparkTimer)
    (if (not (Variables|/Game/ThirdPersonBP/Blueprints/ThirdPersonCharacter.ThirdPersonCharacter_C|GetisOnNewGen _charref))
      (Variables|/Game/ThirdPersonBP/Blueprints/ThirdPersonCharacter.ThirdPersonCharacter_C|SetcurrentNewNewGeneratorRef _charref 0))))

(event Custom|FindOverlappingAreas
  ;[0 0 0] StartResonate
  (for _array_element (Variables|Default|GetgenAreas)
    (bind _array_element_2 (Utilities|Array|ForEachLoopwithBreak (Collision|GetOverlappingActors (Variables|/Game/Blueprints/Generator/Gen3/areas/BP_resArea.BP_resArea_C|GetBox _array_element) 0 :!class /Script/Engine.PrimitiveComponent) :!label _label)
      (:LoopBody
        (if (== (Game|GetPlayerCharacter 0) _array_element_2)
          (Utilities|Array|AddUnique (Variables|Default|GetoverlappingAreas) _array_element)
          (goto _label Break))))))

(event Custom|GivePower
  ;[0 0 0] StartResonate
  ;;[0 0 0] StartAfterExit
  (if (Variables|Default|GetisActive)
    (if (Variables|/Game/ThirdPersonBP/Blueprints/ThirdPersonCharacter.ThirdPersonCharacter_C|GetisOnNewGen (Variables|Default|GetcharRef))
      (if (not (CallFunction|CheckSamePower))
        (bind _returnvalue (Utilities|Time|SetTimerbyEvent (EventDispatchers|CreateEvent :!event Custom|CheckAndGiveAbility) 0.05 true))
        (Variables|Default|SettimerForGiveAbility _returnvalue))
      (else
        (CallFunction|SetCharSkill true)
        (CallFunction|StartTimerforSpark)))))

(event Custom|CheckAndGiveAbility
  (bind _charref (Variables|Default|GetcharRef))
  ;[0 0 0] SetCharSkill
  (Utilities|IsValid (Variables|/Game/ThirdPersonBP/Blueprints/ThirdPersonCharacter.ThirdPersonCharacter_C|GetcurrentNewNewGeneratorRef _charref)
    (:Is%20Not%20Valid
      (if (not (and (CallFunction|CheckOverlappingZones) (Variables|/Game/ThirdPersonBP/Blueprints/ThirdPersonCharacter.ThirdPersonCharacter_C|GetisOnNewGen _charref)))
        (Utilities|Time|ClearandInvalidateTimerbyHandle (Variables|Default|GettimerForGiveAbility))
        (if (CallFunction|CheckOverlappingZones)
          (CallFunction|SetCharSkill true)
          (CallFunction|StartTimerforSpark)
          (else
            (CallFunction|SetCharSkill false)))))))

(event Custom|PrintOverlappingAreas
  ;[0 0 0] forDebug
  (for _array_element (Variables|Default|GetoverlappingAreas)
    (Development|PrintString (Utilities|GetDisplayName _array_element))))

(event Custom|ClearSparkTimer
  ;[0 0 0] SparkTimer
  (Rendering|SetVisibility (Variables|Default|GetWidget) false false)
  (Utilities|Time|ClearandInvalidateTimerbyHandle (Variables|Default|GetsparkTimer)))

(event EventBeginPlay
  (bind _1 (Variables|Default|Get1))
  (bind _2 (Variables|Default|Get2))
  (bind _3 (Variables|Default|Get3))
  (bind _4 (Variables|Default|Get4))
  (bind _relativelocation (Variables|/Script/Engine.SceneComponent|GetRelativeLocation _1))
  (bind _relativelocation_2 (Variables|/Script/Engine.SceneComponent|GetRelativeLocation _2))
  (bind _relativelocation_3 (Variables|/Script/Engine.SceneComponent|GetRelativeLocation _3))
  (bind _relativelocation_4 (Variables|/Script/Engine.SceneComponent|GetRelativeLocation _4))
  ;[0 0 0] BeginPlay
  (CallFunction|SetWidget)
  (Utilities|FlowControl|Sequence
    (:then_0
      (bind _asthird_person_character (Utilities|Casting|CastToThirdPersonCharacter (Game|GetPlayerCharacter 0)))
      (Variables|Default|SetcharRef _asthird_person_character)
      (bind _asw_test_gen (Utilities|Casting|CastToW_TestGen (UserInterface|GetUserWidgetObject (Variables|Default|GetWidget))))
      (Variables|/Game/Widgets/W_TestGen.W_TestGen_C|SetnewNewGenRef _asw_test_gen self))
    (:then_1
      (bind _newtrack_0 (Timeline|Rotation Play)
        (:Update
          (Transformation|SetRelativeLocation _1 (Math|Vector|MakeVector (.x _relativelocation) (.y _relativelocation) _newtrack_0) false false))))
    (:then_2
      (bind _newtrack_0_2 (Timeline|Rotation_2 Play)
        (:Update
          (Transformation|SetRelativeLocation _2 (Math|Vector|MakeVector (.x _relativelocation_2) (.y _relativelocation_2) _newtrack_0_2) false false))))
    (:then_3
      (bind _newtrack_0_3 (Timeline|Timeline_0 Play)
        (:Update
          (Transformation|SetRelativeLocation _3 (Math|Vector|MakeVector (.x _relativelocation_3) (.y _relativelocation_3) _newtrack_0_3) false false))))
    (:then_4
      (bind _newtrack_0_4 (Timeline|Timeline_1 Play)
        (:Update
          (Transformation|SetRelativeLocation _4 (Math|Vector|MakeVector (.x _relativelocation_4) (.y _relativelocation_4) _newtrack_0_4) false false))))))

(event EventTick
  (params (DeltaSeconds :type Float%20%28single-precision%29)))

(event EventInteract
  ;[0 0 0] StartResonate
  (if (not (Variables|Default|GetisActive))
    (CallFunction|Particles)
    (CallFunction|Start)
    (Audio|Components|Audio|Play (Variables|Default|GetEffect_on) 0.5)))

(fn ConstructionScript)

(fn CheckOverlappingZones
  (return (not (== (Utilities|Array|Length (Variables|Default|GetoverlappingAreas)) 0))))

(fn CheckSamePower
  (bind _charref (Variables|Default|GetcharRef))
  (return (and (Utilities|Enum|Equal(Enum) (Utilities|String|EnumtoString (Variables|Default|GetenemyAspect)) (Utilities|String|EnumtoString (Variables|/Game/ThirdPersonBP/Blueprints/ThirdPersonCharacter.ThirdPersonCharacter_C|GetCurrentAspects _charref))) (== (Variables|/Game/ThirdPersonBP/Blueprints/ThirdPersonCharacter.ThirdPersonCharacter_C|GetcurrentNewNewGeneratorRef _charref) self))))

(fn CanSpawnEnemy
  (params (radius :type Float%20%28double-precision%29))
  (bind _charref (Variables|Default|GetcharRef))
  (bind _charref_2 (Variables|Default|GetcharRef))
  (bind _returnvalue (Transformation|GetActorLocation _charref_2))
  (bind _returnvalue_2 (Transformation|GetActorLocation _charref))
  (bind _randomlocation (AI|Navigation|GetRandomReachablePointinRadius _returnvalue radius 0 0))
  (bind (_x _y) (Class|KismetMathLibrary|BreakVector3f _returnvalue_2))
  (Utilities|FlowControl|ForLoopwithBreak 0 5
    (:LoopBody
      (bind (_outhit _returnvalue_3) (Collision|LineTraceByChannel _returnvalue (Math|Vector|MakeVector (.x _randomlocation) (.y _randomlocation) (.Z (Class|KismetMathLibrary|BreakVector3f _returnvalue))) "TraceTypeQuery1" false (Utilities|Array|MakeArray (Variables|Default|GetcharRef)) "None"))
      (if (not _returnvalue_3)
        (return true (.TraceEnd (Collision|BreakHitResult _outhit)) (Math|Rotator|FindLookatRotation (Math|Vector|MakeVector (.X (Math|Vector|BreakVector (.TraceEnd (Collision|BreakHitResult _outhit)))) (.Y (Math|Vector|BreakVector (.TraceEnd (Collision|BreakHitResult _outhit)))) 0.0) (Math|Vector|MakeVector _x _y 0.0)))))))

(fn CheckSpark
  (bind _charref (Variables|Default|GetcharRef))
  (switch Utilities|FlowControl|Switch|SwitchonEnemyAspects_Enum (Variables|Default|GetenemyAspect)
    (:NewEnumerator0
      (return (Variables|/Game/ThirdPersonBP/Blueprints/ThirdPersonCharacter.ThirdPersonCharacter_C|GetsparkFaith _charref)))
    (:NewEnumerator1
      (return (Variables|/Game/ThirdPersonBP/Blueprints/ThirdPersonCharacter.ThirdPersonCharacter_C|GetsparkDestruction _charref)))
    (:NewEnumerator2
      (return (Variables|/Game/ThirdPersonBP/Blueprints/ThirdPersonCharacter.ThirdPersonCharacter_C|GetsparkBond _charref)))
    (:NewEnumerator3
      (return (Variables|/Game/ThirdPersonBP/Blueprints/ThirdPersonCharacter.ThirdPersonCharacter_C|GetsparkRenewal _charref)))))

(fn SetWidget
  (Class|Image|SetBrushfromMaterial (Variables|/Game/Widgets/W_Aspect_Generator.W_Aspect_Generator_C|GetImage_36 (.AsW%20Aspect%20Generator (Utilities|Casting|CastToW_Aspect_Generator (UserInterface|GetWidget (Variables|Default|GetW_Aspect))))) (Utilities|Select :Index (Variables|Default|GetenemyAspect) :NewEnumerator0 "/Game/Widgets/Pictures/Aspects/MI_Blue_Aspect.MI_Blue_Aspect" :NewEnumerator1 "/Game/Widgets/Pictures/Aspects/MI_Red_Aspect.MI_Red_Aspect" :NewEnumerator2 "/Game/Widgets/Pictures/Aspects/MI_Purple_Aspect.MI_Purple_Aspect" :NewEnumerator3 "/Game/Widgets/Pictures/Aspects/MI_Yellow_Aspect.MI_Yellow_Aspect")))