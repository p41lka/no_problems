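; Trigger area for a Gen3 generator that lets the player character supply power by standing inside it while it is active.
; It registers with its generator on BeginPlay, and activation toggles its plane between solid and transparent materials matching the generator's EnemyAspect.
; Entering adds it to the generator's overlap list and calls GivePower.
; Leaving removes it and starts a MistakeTime grace timer, which re-entering that area cancels.
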(event OnComponentBeginOverlap(Box)
  (params (OverlappedComponent :type Primitive%20Component%20Object%20Reference) (OtherActor :type Actor%20Object%20Reference) (OtherComp :type Primitive%20Component%20Object%20Reference) (OtherBodyIndex :type Integer) (bFromSweep :type Boolean) (SweepResult :type Hit%20Result%20Structure%20%28by%20ref%29))
  ;[0 0 0] overlapEvents
  (if (Variables|Default|GetisActive)
    (Utilities|Casting|CastToThirdPersonCharacter OtherActor)
    (Utilities|Array|AddUnique (Variables|/Game/Blueprints/Generator/Gen3/BP_NewNewGenerator.BP_NewNewGenerator_C|GetoverlappingAreas (Variables|Default|GetgenRef)) self)
    (Utilities|Time|ClearandInvalidateTimerbyHandle (Variables|Default|GetEndOverlapTimer))
    (Default|GivePower (Variables|Default|GetgenRef))))

(event OnComponentEndOverlap(Box)
  (params (OverlappedComponent :type Primitive%20Component%20Object%20Reference) (OtherActor :type Actor%20Object%20Reference) (OtherComp :type Primitive%20Component%20Object%20Reference) (OtherBodyIndex :type Integer))
  (bind _genref (Variables|Default|GetgenRef))
  (bind _overlappingareas (Variables|/Game/Blueprints/Generator/Gen3/BP_NewNewGenerator.BP_NewNewGenerator_C|GetoverlappingAreas _genref))
  ;[0 0 0] overlapEvents
  (if (Variables|Default|GetisActive)
    (Utilities|Casting|CastToThirdPersonCharacter OtherActor)
    (Utilities|Array|RemoveIndex _overlappingareas (Utilities|Array|FindItem _overlappingareas self))
    (bind _returnvalue (Utilities|Time|SetTimerbyEvent (EventDispatchers|CreateEvent :!event Custom|AreaEndOverlap) (.mistakeTime (Utilities|Struct|BreakNewNewGen_struct (Variables|/Game/Blueprints/Generator/Gen3/BP_NewNewGenerator.BP_NewNewGenerator_C|GetgenStruct _genref)))))
    (Variables|Default|SetEndOverlapTimer _returnvalue)))

(event Custom|Activate
  ;[0 0 0] On/Off
  (CallFunction|SetLightMaterial)
  (Variables|Default|SetisActive true))

(event Custom|Disable
  ;[0 0 0] On/Off
  (CallFunction|SetDarkMaterial)
  (Variables|Default|SetisActive false))

(event Custom|AreaEndOverlap
  ;[0 0 0] overlapEvents
  (Default|GenEndOverlap (Variables|Default|GetgenRef)))

(event Custom|SetLightMaterial
  ;[0 0 0] SetMaterialToAspect
  (Rendering|Material|SetMaterial (Variables|Default|GetPlane) 0 (Utilities|Select :Index (Variables|/Game/Blueprints/Generator/Gen3/BP_NewNewGenerator.BP_NewNewGenerator_C|GetenemyAspect (Variables|Default|GetgenRef)) :NewEnumerator0 "/Game/Materials/M_Unlit/MI_Faith.MI_Faith" :NewEnumerator1 "/Game/Materials/M_Unlit/MI_Destruction.MI_Destruction" :NewEnumerator2 "/Game/Materials/M_Unlit/MI_Bond.MI_Bond" :NewEnumerator3 "/Game/Materials/M_Unlit/MI_Renewal.MI_Renewal")))

(event Custom|SetDarkMaterial
  ;[0 0 0] SetMaterialToAspect
  (Rendering|Material|SetMaterial (Variables|Default|GetPlane) 0 (Utilities|Select :Index (Variables|/Game/Blueprints/Generator/Gen3/BP_NewNewGenerator.BP_NewNewGenerator_C|GetenemyAspect (Variables|Default|GetgenRef)) :NewEnumerator0 "/Game/Materials/M_Transparent/MI_Faith_Transparent.MI_Faith_Transparent" :NewEnumerator1 "/Game/Materials/M_Transparent/MI_Destruction_Transparent.MI_Destruction_Transparent" :NewEnumerator2 "/Game/Materials/M_Transparent/MI_Bond_Transparent.MI_Bond_Transparent" :NewEnumerator3 "/Game/Materials/M_Transparent/M_Renewal_Transparent.M_Renewal_Transparent")))

(event EventBeginPlay
  ;[0 0 0] beginPlay
  (Utilities|Array|Add (Variables|/Game/Blueprints/Generator/Gen3/BP_NewNewGenerator.BP_NewNewGenerator_C|GetgenAreas (Variables|Default|GetgenRef)) self)
  (CallFunction|SetDarkMaterial))

(fn ConstructionScript
  (CallFunction|SetDarkMaterial))