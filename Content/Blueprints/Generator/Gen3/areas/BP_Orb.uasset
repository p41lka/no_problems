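; BP_Orb is a projectile actor that pops upward on spawn and then homes toward a target component.
; On BeginPlay it launches fast along Z, then after a short delay drops to a slow rise and sets Target as the homing target.
; When its sphere overlaps a BP_resArea, it destroys itself after a brief delay.
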(event OnComponentBeginOverlap(Sphere1)
  (params (OverlappedComponent :type Primitive%20Component%20Object%20Reference) (OtherActor :type Actor%20Object%20Reference) (OtherComp :type Primitive%20Component%20Object%20Reference) (OtherBodyIndex :type Integer) (bFromSweep :type Boolean) (SweepResult :type Hit%20Result%20Structure%20%28by%20ref%29))
  (Utilities|Casting|CastToBP_resArea OtherActor)
  (Utilities|FlowControl|Delay 0.2)
  (Actor|DestroyActor))

(event EventBeginPlay
  (bind _projectilemovement (Variables|Default|GetProjectileMovement))
  (Variables|/Script/Engine.MovementComponent|SetVelocity _projectilemovement "0, 0,500.000000")
  (Utilities|FlowControl|Delay 0.2)
  (Variables|/Script/Engine.MovementComponent|SetVelocity _projectilemovement "0, 0,10.000000")
  (Variables|/Script/Engine.ProjectileMovementComponent|SetHomingTargetComponent (Variables|Default|GetProjectileMovement) (Variables|Default|GetTarget)))

(fn ConstructionScript)