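; Resonance figure character for a generator, taking the shape of a Circle, Line or Cross that reacts to the player.
; SpawnFigure shows the chosen shape and enables its overlap collision; only the Circle moves, looping through six generator points via AIMoveTo.
; ThirdPersonCharacter overlaps tell the Generator to start or end resonating.
; Separate figure events swap in an emissive material and run timelines that scale the Circle or spin the Line and Cross.
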(event OnComponentBeginOverlap(CircleCollision)
  (params (OverlappedComponent :type Primitive%20Component%20Object%20Reference) (OtherActor :type Actor%20Object%20Reference) (OtherComp :type Primitive%20Component%20Object%20Reference) (OtherBodyIndex :type Integer) (bFromSweep :type Boolean) (SweepResult :type Hit%20Result%20Structure%20%28by%20ref%29))
  (Utilities|Casting|CastToThirdPersonCharacter OtherActor)
  (Default|StartResonating (Variables|Default|GetGenerator)))

(event OnComponentEndOverlap(CircleCollision)
  (params (OverlappedComponent :type Primitive%20Component%20Object%20Reference) (OtherActor :type Actor%20Object%20Reference) (OtherComp :type Primitive%20Component%20Object%20Reference) (OtherBodyIndex :type Integer))
  (Utilities|Casting|CastToThirdPersonCharacter OtherActor)
  (Default|EndResonating (Variables|Default|GetGenerator)))

(event OnComponentBeginOverlap(LineCollision)
  (params (OverlappedComponent :type Primitive%20Component%20Object%20Reference) (OtherActor :type Actor%20Object%20Reference) (OtherComp :type Primitive%20Component%20Object%20Reference) (OtherBodyIndex :type Integer) (bFromSweep :type Boolean) (SweepResult :type Hit%20Result%20Structure%20%28by%20ref%29))
  (Utilities|Casting|CastToThirdPersonCharacter OtherActor)
  (Default|StartResonating (Variables|Default|GetGenerator)))

(event OnComponentEndOverlap(LineCollision)
  (params (OverlappedComponent :type Primitive%20Component%20Object%20Reference) (OtherActor :type Actor%20Object%20Reference) (OtherComp :type Primitive%20Component%20Object%20Reference) (OtherBodyIndex :type Integer))
  (Utilities|Casting|CastToThirdPersonCharacter OtherActor)
  (Default|EndResonating (Variables|Default|GetGenerator)))

(event OnComponentBeginOverlap(Cross1_Collision)
  (params (OverlappedComponent :type Primitive%20Component%20Object%20Reference) (OtherActor :type Actor%20Object%20Reference) (OtherComp :type Primitive%20Component%20Object%20Reference) (OtherBodyIndex :type Integer) (bFromSweep :type Boolean) (SweepResult :type Hit%20Result%20Structure%20%28by%20ref%29))
  (Utilities|Casting|CastToThirdPersonCharacter OtherActor)
  (Default|StartResonating (Variables|Default|GetGenerator)))

(event OnComponentEndOverlap(Cross1_Collision)
  (params (OverlappedComponent :type Primitive%20Component%20Object%20Reference) (OtherActor :type Actor%20Object%20Reference) (OtherComp :type Primitive%20Component%20Object%20Reference) (OtherBodyIndex :type Integer))
  (Utilities|Casting|CastToThirdPersonCharacter OtherActor)
  (Default|EndResonating (Variables|Default|GetGenerator)))

(event OnComponentBeginOverlap(Cross2_Collision)
  (params (OverlappedComponent :type Primitive%20Component%20Object%20Reference) (OtherActor :type Actor%20Object%20Reference) (OtherComp :type Primitive%20Component%20Object%20Reference) (OtherBodyIndex :type Integer) (bFromSweep :type Boolean) (SweepResult :type Hit%20Result%20Structure%20%28by%20ref%29))
  (Utilities|Casting|CastToThirdPersonCharacter OtherActor)
  (Default|StartResonating (Variables|Default|GetGenerator)))

(event OnComponentEndOverlap(Cross2_Collision)
  (params (OverlappedComponent :type Primitive%20Component%20Object%20Reference) (OtherActor :type Actor%20Object%20Reference) (OtherComp :type Primitive%20Component%20Object%20Reference) (OtherBodyIndex :type Integer))
  (Utilities|Casting|CastToThirdPersonCharacter OtherActor)
  (Default|EndResonating (Variables|Default|GetGenerator)))

(event Collision|EventActorBeginOverlap
  (params (OtherActor :type Actor%20Object%20Reference)))

(event EventSpawnFigure
  (params (Figure :type ResonanceFigures_Enum%20Enum :default "NewEnumerator0") (Generator :type BP%20New%20Generator%20Object%20Reference))
  (bind _self self)
  (bind _self_2 self)
  (Variables|Default|SetGenerator Generator)
  (bind _output_get (Variables|Default|SetCurrentFigure Figure))
  (switch Utilities|FlowControl|Switch|SwitchonResonanceFigures_Enum _output_get
    (:NewEnumerator0
      (Rendering|SetVisibility (Variables|Default|GetCircle) true false)
      (Rendering|SetVisibility (Variables|Default|GetLine) false false)
      (Rendering|SetVisibility (Variables|Default|GetCross) false true)
      (Variables|/Script/Engine.PrimitiveComponent|SetbGenerateOverlapEvents (Variables|Default|GetCircleCollision) true)
      (Variables|/Script/Engine.PrimitiveComponent|SetbGenerateOverlapEvents (Variables|Default|GetLineCollision) false)
      (Variables|/Script/Engine.PrimitiveComponent|SetbGenerateOverlapEvents (Variables|Default|GetCross1_Collision) false)
      (Variables|/Script/Engine.PrimitiveComponent|SetbGenerateOverlapEvents (Variables|Default|GetCross2_Collision) false)
      (AI|AIMoveTo _self_2 (Variables|/Game/Blueprints/Generator/BP_NewGenerator.BP_NewGenerator_C|GetPoint1 (Variables|Default|GetGenerator)) 0 5.0 false :!label _label
        (:OnSuccess
          (AI|AIMoveTo _self_2 (Variables|/Game/Blueprints/Generator/BP_NewGenerator.BP_NewGenerator_C|GetPoint2 (Variables|Default|GetGenerator)) 0 5.0 false
            (:OnSuccess
              (AI|AIMoveTo _self_2 (Variables|/Game/Blueprints/Generator/BP_NewGenerator.BP_NewGenerator_C|GetPoint3 (Variables|Default|GetGenerator)) 0 5.0 false
                (:OnSuccess
                  (AI|AIMoveTo _self (Variables|/Game/Blueprints/Generator/BP_NewGenerator.BP_NewGenerator_C|GetPoint4 (Variables|Default|GetGenerator)) 0 5.0 false
                    (:OnSuccess
                      (AI|AIMoveTo _self (Variables|/Game/Blueprints/Generator/BP_NewGenerator.BP_NewGenerator_C|GetPoint5 (Variables|Default|GetGenerator)) 0 5.0 false
                        (:OnSuccess
                          (AI|AIMoveTo _self (Variables|/Game/Blueprints/Generator/BP_NewGenerator.BP_NewGenerator_C|GetPoint6 (Variables|Default|GetGenerator)) 0 5.0 false
                            (:OnSuccess
                              (goto _label))))))))))))))
    (:NewEnumerator1
      (Rendering|SetVisibility (Variables|Default|GetCircle) false false)
      (Rendering|SetVisibility (Variables|Default|GetLine) true false)
      (Rendering|SetVisibility (Variables|Default|GetCross) false true)
      (Variables|/Script/Engine.PrimitiveComponent|SetbGenerateOverlapEvents (Variables|Default|GetCircleCollision) false)
      (Variables|/Script/Engine.PrimitiveComponent|SetbGenerateOverlapEvents (Variables|Default|GetLineCollision) true)
      (Variables|/Script/Engine.PrimitiveComponent|SetbGenerateOverlapEvents (Variables|Default|GetCross1_Collision) false)
      (Variables|/Script/Engine.PrimitiveComponent|SetbGenerateOverlapEvents (Variables|Default|GetCross2_Collision) false))
    (:NewEnumerator2
      (Rendering|SetVisibility (Variables|Default|GetCircle) false false)
      (Rendering|SetVisibility (Variables|Default|GetLine) false false)
      (Rendering|SetVisibility (Variables|Default|GetCross) true true)
      (Variables|/Script/Engine.PrimitiveComponent|SetbGenerateOverlapEvents (Variables|Default|GetCircleCollision) false)
      (Variables|/Script/Engine.PrimitiveComponent|SetbGenerateOverlapEvents (Variables|Default|GetLineCollision) false)
      (Variables|/Script/Engine.PrimitiveComponent|SetbGenerateOverlapEvents (Variables|Default|GetCross1_Collision) true)
      (Variables|/Script/Engine.PrimitiveComponent|SetbGenerateOverlapEvents (Variables|Default|GetCross2_Collision) true))))

(event EventStartResonatingFigure
  (switch Utilities|FlowControl|Switch|SwitchonResonanceFigures_Enum (Variables|Default|GetCurrentFigure)
    (:NewEnumerator0
      (Rendering|Material|SetMaterial (Variables|Default|GetCircle) 0 "/Game/Meshes/M_Blue_Emissive.M_Blue_Emissive")
      (bind _scalecircle (Timeline|Timeline_0 Play)
        (:Update
          (Transformation|SetWorldScale3D (Variables|Default|GetCircle) _scalecircle))))
    (:NewEnumerator1
      (Rendering|Material|SetMaterial (Variables|Default|GetLine) 0 "/Game/Meshes/M_Blue_Emissive.M_Blue_Emissive")
      (bind _addrotation (Timeline|Timeline_1 Play)
        (:Update
          (Transformation|AddWorldRotation (Variables|Default|GetLine) (Math|Rotator|MakeRotator 0.0 0.0 _addrotation) false false))))
    (:NewEnumerator2
      (Rendering|Material|SetMaterial (Variables|Default|GetCross1) 0 "/Game/Meshes/M_Blue_Emissive.M_Blue_Emissive")
      (bind _addrotation_2 (Timeline|Timeline_2 Play)
        (:Update
          (Transformation|AddWorldRotation (Variables|Default|GetCross) (Math|Rotator|MakeRotator 0.0 0.0 _addrotation_2) false false))))))

(event EventEndResonatingFigure
  (switch Utilities|FlowControl|Switch|SwitchonResonanceFigures_Enum (Variables|Default|GetCurrentFigure)
    (:NewEnumerator0
      (Rendering|Material|SetMaterial (Variables|Default|GetCircle) 0 "/Game/Materials/M_Enemies/M_Circle.M_Circle")
      (bind _scalecircle (Timeline|Timeline_0 Stop)
        (:Update
          (Transformation|SetWorldScale3D (Variables|Default|GetCircle) _scalecircle))))
    (:NewEnumerator1
      (Rendering|Material|SetMaterial (Variables|Default|GetLine) 0 "/Game/Materials/M_Enemies/M_Circle.M_Circle")
      (bind _addrotation (Timeline|Timeline_1 Stop)
        (:Update
          (Transformation|AddWorldRotation (Variables|Default|GetLine) (Math|Rotator|MakeRotator 0.0 0.0 _addrotation) false false))))
    (:NewEnumerator2
      (Rendering|Material|SetMaterial (Variables|Default|GetCross1) 0 "/Game/Materials/M_Enemies/M_Circle.M_Circle")
      (bind _addrotation_2 (Timeline|Timeline_2 Stop)
        (:Update
          (Transformation|AddWorldRotation (Variables|Default|GetCross) (Math|Rotator|MakeRotator 0.0 0.0 _addrotation_2) false false))))))

(fn ConstructionScript)

(fn IsGeneratorReloading
  (params (IsReloading :type Boolean))
  (return false))