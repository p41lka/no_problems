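; Generator that grants the player a Faith, Destruction or Renewal ability, chosen by its enemy aspect, after they resonate inside its collision.
; It spawns a resonance figure below itself, which starts and stops with the resonance.
; A looping timer fills the interface's progress only while a per-tick downward trace under the player hits a Resonance physical surface.
; Granting the ability triggers a reload counted in ticks; leaving the collision resets progress.
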(event OnComponentBeginOverlap(ResonanceCollision)
  (params (OverlappedComponent :type Primitive%20Component%20Object%20Reference) (OtherActor :type Actor%20Object%20Reference) (OtherComp :type Primitive%20Component%20Object%20Reference) (OtherBodyIndex :type Integer) (bFromSweep :type Boolean) (SweepResult :type Hit%20Result%20Structure%20%28by%20ref%29))
  (bind _asthird_person_character (Utilities|Casting|CastToThirdPersonCharacter OtherActor))
  (if (not (Variables|/Game/ThirdPersonBP/Blueprints/ThirdPersonCharacter.ThirdPersonCharacter_C|GetIsUsingAbility (Variables|Default|GetCharacterREF)))
    (Default|SetLatestGenerator _asthird_person_character (Variables|Default|GetEnemyAspects))
    (Variables|Default|SetIsOverlapped true)
    (if (not (Variables|Default|GetIsGeneratorReloading_0))
      (CallFunction|StartResonationg)
      ;[0 0 0] Resonance Timer
      (bind _returnvalue (Utilities|Time|SetTimerbyEvent (delegate Custom|Resonance) 0.5 true))
      (Variables|Default|SetResTimer _returnvalue))))

(event OnComponentEndOverlap(ResonanceCollision)
  (params (OverlappedComponent :type Primitive%20Component%20Object%20Reference) (OtherActor :type Actor%20Object%20Reference) (OtherComp :type Primitive%20Component%20Object%20Reference) (OtherBodyIndex :type Integer))
  (Variables|Default|SetIsOverlapped false)
  (CallFunction|EndResonating))

(event Custom|Resonance
  (bind _characterref (Variables|Default|GetCharacterREF))
  ;[0 0 0] Resonance Timer
  (if (Variables|Default|GetIsGeneratorResonating)
    (if (< (Variables|Default|GetCurrentTime) (Variables|Default|GetResonanceTime))
      (bind _result (Math|Float|IncrementFloat (Variables|Default|GetCurrentTime))
        (:%20%20
          (Variables|/Game/Widgets/W_CharacterInterface.W_CharacterInterface_C|SetCurrentResonanceTime (Variables|/Game/ThirdPersonBP/Blueprints/ThirdPersonCharacter.ThirdPersonCharacter_C|GetInterfaceREF (Variables|Default|GetCharacterREF)) _result)
          (if (>= (Variables|Default|GetCurrentTime) (Variables|Default|GetResonanceTime))
            (Variables|/Game/ThirdPersonBP/Blueprints/ThirdPersonCharacter.ThirdPersonCharacter_C|SetIsUsingAbility (Variables|Default|GetCharacterREF) true)
            ;;[0 0 0] Set ability from enemy aspect
            (switch Utilities|FlowControl|Switch|SwitchonEnemyAspects_Enum (Variables|Default|GetEnemyAspects)
              (:NewEnumerator0
                (Default|SetFaithAbility _characterref))
              (:NewEnumerator1
                (Default|SetDestructionAbility _characterref))
              (:NewEnumerator3
                (Default|SetRenewalAbility _characterref)))
            (CallFunction|EndResonating)
            (Variables|Default|SetIsGeneratorReloading_0 true)))))))

(event Custom|StartResonationg
  ;[0 0 0] Start and End Resonating
  (Default|StartResonatingFigure (Variables|Default|GetResonanceREF)))

(event Custom|EndResonating
  ;[0 0 0] Start and End Resonating
  (Default|EndResonatingFigure (Variables|Default|GetResonanceREF))
  (Utilities|Time|ClearandInvalidateTimerbyHandle (Variables|Default|GetResTimer))
  (Variables|Default|SetCurrentTime 0.0)
  (Variables|/Game/Widgets/W_CharacterInterface.W_CharacterInterface_C|SetCurrentResonanceTime (Variables|/Game/ThirdPersonBP/Blueprints/ThirdPersonCharacter.ThirdPersonCharacter_C|GetInterfaceREF (Variables|Default|GetCharacterREF)) 0.0))

(event Custom|CheckMaterial
  (bind _characterref (Variables|Default|GetCharacterREF))
  (bind _returnvalue (Transformation|GetActorLocation _characterref))
  ;[0 0 0] Check Step on Material
  (bind _outhit (Collision|LineTraceByChannel _returnvalue (- _returnvalue "0,0.000000,300.000000") "TraceTypeQuery1" false 0 "None" true "(R=1.000000,G=0.000000,B=0.000000,A=1.000000)" "(R=0.000000,G=1.000000,B=0.000000,A=1.000000)" 1.0))
  (Variables|Default|SetIsGeneratorResonating (Utilities|Select :Index (Variables|/Script/PhysicsCore.PhysicalMaterial|GetSurfaceType (.PhysMat (Collision|BreakHitResult _outhit))) :SurfaceType_Default false :SurfaceType1 true)))

(event EventTick
  (params (DeltaSeconds :type Float%20%28single-precision%29))
  ;[0 0 0] Reloading
  (CallFunction|CheckMaterial)
  (if (Variables|Default|GetIsGeneratorReloading_0)
    (bind _output_get (Variables|Default|SetCurrentGeneratorReloadTime (+ (Variables|Default|GetCurrentGeneratorReloadTime) 1.0)))
    (Development|PrintString (Utilities|String|Append "Generator reload: " (Utilities|String|ToString(Float) _output_get)) true true "(R=1.000000,G=0.784818,B=0.000000,A=1.000000)" 0.0)
    (if (< _output_get (Variables|Default|GetGeneratorReloadTime))
      (Variables|Default|SetIsGeneratorReloading_0 true)
      (else
        (Variables|Default|SetIsGeneratorReloading_0 false)
        (Variables|Default|SetCurrentGeneratorReloadTime 0.0)))
    (else
      (Variables|Default|SetCurrentGeneratorReloadTime 0.0))))

(event EventBeginPlay
  (bind _returnvalue (Transformation|GetActorLocation))
  (bind _asthird_person_character (Utilities|Casting|CastToThirdPersonCharacter (Game|GetPlayerCharacter 0)))
  (Variables|Default|SetCharacterREF _asthird_person_character)
  ;[0 0 0] Spawn Resonate Figure
  (bind _returnvalue_2 (Game|SpawnActorfromClass "/Game/Blueprints/Generator/BP_ResonanceFigure.BP_ResonanceFigure_C" (Math|Transform|MakeTransform (Math|Vector|MakeVector (.x _returnvalue) (.y _returnvalue) (- (.z _returnvalue) 9e+01)) "0, 0, 0" "1.000000,1.000000,1.000000") "Undefined" 0 0))
  (bind _output_get (Variables|Default|SetResonanceREF _returnvalue_2))
  (Default|SpawnFigure _output_get (Variables|Default|GetResonanceFigure)))

(fn ConstructionScript)

(fn IsGeneratorReloading
  (params (IsReloading :type Boolean))
  (return false))