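; BP_Platform is a level prop that moves vertically between its start location and the height of Position2 when the ThirdPersonCharacter overlaps it.
; The Down timeline lerps only Z from the location cached at BeginPlay.
; An IsDown flag, toggled when the timeline finishes, selects reverse or forward playback.
; Each trigger plays the Glass_eye sound, with a one-second delay before forward moves only.
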(event EventBeginPlay
  (Variables|Default|SetNewVar_0 (Transformation|GetActorLocation)))

(event Collision|EventActorBeginOverlap
  (params (OtherActor :type Actor%20Object%20Reference))
  (bind _newvar_0 (Variables|Default|GetNewVar_0))
  (Utilities|Casting|CastToThirdPersonCharacter OtherActor)
  (if (Variables|Default|GetIsDown)
    (Audio|PlaySound2D "/Game/Sound/Enviroment/glass_eye.glass_eye" 1.0 1.0 0.0 0 0)
    (bind _newtrack_0 (Timeline|down Reverse)
      (:Update
        (Transformation|SetActorLocation (Math|Vector|MakeVector (.x _newvar_0) (.y _newvar_0) (Math|Float|Lerp (.z _newvar_0) (.z (Variables|Default|Getposition%202)) _newtrack_0)) false false))
      (:Finished
        (if (Variables|Default|GetIsDown)
          (Variables|Default|SetIsDown false)
          (else
            (Variables|Default|SetIsDown true)))))
    (else
      (Utilities|FlowControl|Delay 1.0)
      (Audio|PlaySound2D "/Game/Sound/Enviroment/glass_eye.glass_eye" 1.0 1.0 0.0 0 0)
      (Timeline|down Play))))

(fn ConstructionScript)