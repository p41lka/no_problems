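; BP_Teleport is a level prop that moves an overlapping ThirdPersonCharacter to the Arrow of its linked BPoint, with zero rotation.
; Box overlap starts a timeline that scales the particle system's Z axis, then teleports the character when it finishes.
; Both points are then flagged active for the Reload delay, blocking retriggering while both flags are set, before the flags clear and the particle's Z scale resets.
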(event OnComponentBeginOverlap(Box)
  (params (OverlappedComponent :type Primitive%20Component%20Object%20Reference) (OtherActor :type Actor%20Object%20Reference) (OtherComp :type Primitive%20Component%20Object%20Reference) (OtherBodyIndex :type Integer) (bFromSweep :type Boolean) (SweepResult :type Hit%20Result%20Structure%20%28by%20ref%29))
  (bind _bpoint (Variables|Default|GetBPoint))
  (bind _particlesystem (Variables|Default|GetParticleSystem))
  (bind _particlesystem_2 (Variables|Default|GetParticleSystem))
  (bind _returnvalue (Transformation|GetWorldScale _particlesystem_2))
  (bind _returnvalue_2 (Transformation|GetWorldScale _particlesystem))
  (bind _asthird_person_character (Utilities|Casting|CastToThirdPersonCharacter OtherActor))
  (if (not (and (Variables|Default|GetIsActive) (Variables|BP_Teleport_C|GetIsActive _bpoint)))
    (Utilities|IsValid _bpoint
      (:Is%20Valid
        (bind _newtrack_0 (Timeline|scale%20particle PlayFromStart)
          (:Update
            (Transformation|SetWorldScale3D _particlesystem_2 (Math|Vector|MakeVector (.x _returnvalue) (.y _returnvalue) _newtrack_0)))
          (:Finished
            (Transformation|Teleport _asthird_person_character (Transformation|GetWorldLocation (Variables|BP_Teleport_C|GetArrow _bpoint)) "0, 0, 0")
            (Variables|Default|SetIsActive true)
            (Variables|BP_Teleport_C|SetIsActive _bpoint true)
            (Utilities|FlowControl|Delay (Variables|Default|GetReload))
            (Variables|Default|SetIsActive false)
            (Variables|BP_Teleport_C|SetIsActive _bpoint false)
            (Transformation|SetWorldScale3D _particlesystem (Math|Vector|MakeVector (.x _returnvalue_2) (.y _returnvalue_2) 0.0))))))))

(event EventBeginPlay
  (Rendering|Material|SetMaterial (Variables|Default|GetTeleport) 1 (Variables|Default|GetMaterial)))

(fn ConstructionScript)