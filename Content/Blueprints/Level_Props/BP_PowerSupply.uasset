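; BP_PowerSupply is a station prop that refills a ThirdPersonCharacter's DopAmmo when it enters the box trigger, then recharges.
; A pickup only happens when the station is ready and the character is below max, adding a clamped amount with particles and audio.
; PowerSupplyStruct sets the amount and cooldown.
; A dynamic emissive material shows state: a timeline dims it on use, and the end-of-recharge timer snaps it back to bright.
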(event OnComponentBeginOverlap(Box)
  (params (OverlappedComponent :type Primitive%20Component%20Object%20Reference) (OtherActor :type Actor%20Object%20Reference) (OtherComp :type Primitive%20Component%20Object%20Reference) (OtherBodyIndex :type Integer) (bFromSweep :type Boolean) (SweepResult :type Hit%20Result%20Structure%20%28by%20ref%29))
  (if (not (Variables|Default|GetIsRecharging))
    (bind _asthird_person_character (Utilities|Casting|CastToThirdPersonCharacter OtherActor))
    (if (< (Variables|/Game/ThirdPersonBP/Blueprints/ThirdPersonCharacter.ThirdPersonCharacter_C|GetCurrentDopAmmo _asthird_person_character) (Variables|/Game/ThirdPersonBP/Blueprints/ThirdPersonCharacter.ThirdPersonCharacter_C|GetMaxDopAmmo _asthird_person_character))
      (CallFunction|AddAmmo _asthird_person_character)
      (Audio|Components|Audio|Play (Variables|Default|GetAudio) 0.0))))

(event Custom|StartRecharge
  (Variables|Default|SetIsRecharging true)
  (Components|Activation|Activate (Variables|Default|GetParticleSystem) true)
  (Utilities|Time|SetTimerbyEvent (delegate Custom|EndRecharge) (Utilities|Struct|BreakPowerSupply_Struct (Variables|Default|GetpowerSupplyStruct)))
  (bind _alpha (Timeline|SoftChangeAlpha PlayFromStart)
    (:Update
      (Rendering|Material|SetScalarParameterValue (Variables|Default|GetMaterial) "Emissive" (Math|Float|Lerp 3e+02 0.03 _alpha) :!class /Script/Engine.MaterialInstanceDynamic))))

(event Custom|EndRecharge
  (Variables|Default|SetIsRecharging false)
  (Rendering|Material|SetScalarParameterValue (Variables|Default|GetMaterial) "Emissive" 3e+02 :!class /Script/Engine.MaterialInstanceDynamic))

(event Custom|AddAmmo
  (params (charRef :type Third%20Person%20Character%20Object%20Reference))
  (Variables|/Game/ThirdPersonBP/Blueprints/ThirdPersonCharacter.ThirdPersonCharacter_C|SetCurrentDopAmmo charRef (Math|Integer|Clamp(Integer) (+ (Utilities|Struct|BreakPowerSupply_Struct (Variables|Default|GetpowerSupplyStruct)) (Variables|/Game/ThirdPersonBP/Blueprints/ThirdPersonCharacter.ThirdPersonCharacter_C|GetCurrentDopAmmo charRef)) 0 (Variables|/Game/ThirdPersonBP/Blueprints/ThirdPersonCharacter.ThirdPersonCharacter_C|GetMaxDopAmmo charRef)))
  (CallFunction|StartRecharge))

(event EventBeginPlay
  (bind _station (Variables|Default|GetStation))
  (bind _returnvalue (Rendering|Material|CreateDynamicMaterialInstance _station 2 "/Game/Materials/M_Enemies/M_Emissive_Blue_Enemy.M_Emissive_Blue_Enemy" "None" :!class /Script/Engine.PrimitiveComponent))
  (bind _output_get (Variables|Default|SetMaterial _returnvalue))
  (Rendering|Material|SetMaterial _station 2 _output_get))

(fn ConstructionScript)