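; BP_Camera_Change is a level prop that changes the third-person character's camera framing, setting the boom socket offset and follow camera rotation to level-specific values.
; With SetOnOverlap off, it applies them instantly on BeginPlay.
; With it on, entering its Box blends from the current values via a timeline scaled by TimeChange.
; IsOverlapping blocks retriggering until the blend finishes; leaving the box restores nothing.
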(event OnComponentBeginOverlap(Box)
  (params (OverlappedComponent :type Primitive%20Component%20Object%20Reference) (OtherActor :type Actor%20Object%20Reference) (OtherComp :type Primitive%20Component%20Object%20Reference) (OtherBodyIndex :type Integer) (bFromSweep :type Boolean) (SweepResult :type Hit%20Result%20Structure%20%28by%20ref%29))
  (bind _asthird_person_character (Utilities|Casting|CastToThirdPersonCharacter OtherActor))
  (bind _output_get (Variables|Default|SetCharacterREF _asthird_person_character))
  (if (Variables|Editable|GetSetOnOverlap)
    (if (not (Variables|Default|GetIsOverlapping))
      (Variables|Default|SetIsOverlapping true)
      (Variables|Default|SetPreviousSocketOffset (Variables|/Script/Engine.SpringArmComponent|GetSocketOffset (Variables|/Game/ThirdPersonBP/Blueprints/ThirdPersonCharacter.ThirdPersonCharacter_C|GetCameraBoom _output_get)))
      (Variables|Default|SetPreviousCameraRotation (Variables|/Script/Engine.SceneComponent|GetRelativeRotation (Variables|/Game/ThirdPersonBP/Blueprints/ThirdPersonCharacter.ThirdPersonCharacter_C|GetFollowCamera _output_get)))
      (Components|Timeline|SetPlayRate (Variables|Default|GetChangeAlpha) (/ 1.0 (Variables|Default|GetTimeChange)))
      (bind _alpha (Timeline|ChangeAlpha PlayFromStart)
        (:Update
          (Variables|/Script/Engine.SpringArmComponent|SetSocketOffset (Variables|/Game/ThirdPersonBP/Blueprints/ThirdPersonCharacter.ThirdPersonCharacter_C|GetCameraBoom _output_get) (Math|Vector|Lerp(Vector) (Variables|Default|GetPreviousSocketOffset) (Variables|Editable|GetLevelSocketOffset) _alpha))
          (Transformation|SetRelativeRotation (Variables|/Game/ThirdPersonBP/Blueprints/ThirdPersonCharacter.ThirdPersonCharacter_C|GetFollowCamera _output_get) (Math|Rotator|Lerp(Rotator) (Variables|Default|GetPreviousCameraRotation) (Variables|Editable|GetLevelCameraRotation) _alpha) false false))
        (:Finished
          (Variables|Default|SetIsOverlapping false))))))

(event EventBeginPlay
  (bind _asthird_person_character (Utilities|Casting|CastToThirdPersonCharacter (Game|GetPlayerCharacter 0)))
  (bind _output_get (Variables|Default|SetCharacterREF _asthird_person_character))
  (if (not (Variables|Editable|GetSetOnOverlap))
    (Variables|/Script/Engine.SpringArmComponent|SetSocketOffset (Variables|/Game/ThirdPersonBP/Blueprints/ThirdPersonCharacter.ThirdPersonCharacter_C|GetCameraBoom _output_get) (Variables|Editable|GetLevelSocketOffset))
    (Transformation|SetRelativeRotation (Variables|/Game/ThirdPersonBP/Blueprints/ThirdPersonCharacter.ThirdPersonCharacter_C|GetFollowCamera _output_get) (Variables|Editable|GetLevelCameraRotation) false false)))

(fn ConstructionScript)