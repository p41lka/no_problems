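; BP_Tram is a level prop tram that departs when the player's ThirdPersonCharacter enters its trigger box.
; It records its start location on BeginPlay, then on overlap plays a transition sound and a timeline that lerps the actor toward Location2.
; Two seconds after the overlap, it plays fade animations on the character's fade widget and interface widget.
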(event OnComponentBeginOverlap(Box)
  (params (OverlappedComponent :type Primitive%20Component%20Object%20Reference) (OtherActor :type Actor%20Object%20Reference) (OtherComp :type Primitive%20Component%20Object%20Reference) (OtherBodyIndex :type Integer) (bFromSweep :type Boolean) (SweepResult :type Hit%20Result%20Structure%20%28by%20ref%29))
  (bind _asthird_person_character (Utilities|Casting|CastToThirdPersonCharacter OtherActor))
  (Utilities|FlowControl|Sequence
    (:then_0
      (Audio|PlaySound2D "/Game/Sound/transition.transition" 1.0 1.0 0.0 0 0)
      (bind _newtrack_0 (Timeline|MovementTram Play)
        (:Update
          (Transformation|SetActorLocation (Math|Vector|Lerp(Vector) (Variables|Default|GetLocation) (Variables|Default|Getlocation2) _newtrack_0) false false))))
    (:then_1
      (Utilities|FlowControl|Delay 2.0)
      (UserInterface|Animation|PlayAnimation (Variables|/Game/ThirdPersonBP/Blueprints/ThirdPersonCharacter.ThirdPersonCharacter_C|GetFadeWidget _asthird_person_character) (Variables|/Game/Widgets/W_FadeOut.W_FadeOut_C|GetFade (Variables|/Game/ThirdPersonBP/Blueprints/ThirdPersonCharacter.ThirdPersonCharacter_C|GetFadeWidget _asthird_person_character)) 0.0 1 "Forward" 1.0 false)
      (UserInterface|Animation|PlayAnimation (Variables|/Game/ThirdPersonBP/Blueprints/ThirdPersonCharacter.ThirdPersonCharacter_C|GetInterfaceREF _asthird_person_character) (Variables|/Game/Widgets/W_CharacterInterface.W_CharacterInterface_C|GetFade (Variables|/Game/ThirdPersonBP/Blueprints/ThirdPersonCharacter.ThirdPersonCharacter_C|GetInterfaceREF _asthird_person_character)) 0.0 1 "Forward" 1.0 false))))

(event EventBeginPlay
  (Variables|Default|SetLocation (Transformation|GetActorLocation)))

(fn ConstructionScript)