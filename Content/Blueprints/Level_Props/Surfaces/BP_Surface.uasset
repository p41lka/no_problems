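; BP_Surface is a level prop surface that speeds up or slows down the player character while it stands inside its box trigger.
; On begin play it caches the player's normal run and walk speeds and applies its material to the plane.
; On overlap, the Surface setting (Fast or Slow) selects speeds from the Speed struct, updating both the character's stored speeds and current max walk speed.
; Leaving the box restores the cached speeds.
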(event OnComponentBeginOverlap(Box)
  (params (OverlappedComponent :type Primitive%20Component%20Object%20Reference) (OtherActor :type Actor%20Object%20Reference) (OtherComp :type Primitive%20Component%20Object%20Reference) (OtherBodyIndex :type Integer) (bFromSweep :type Boolean) (SweepResult :type Hit%20Result%20Structure%20%28by%20ref%29))
  (bind _speed (Variables|Default|GetSpeed))
  (bind _speed_2 (Variables|Default|GetSpeed))
  (bind (_fastrun _fastwalk _slowrun _slowwalk) (Utilities|Struct|BreakSurfaces_S _speed))
  (bind (_fastrun_2 _fastwalk_2 _slowrun_2 _slowwalk_2) (Utilities|Struct|BreakSurfaces_S _speed_2))
  (bind _asthird_person_character (Utilities|Casting|CastToThirdPersonCharacter OtherActor))
  (Variables|Default|SetCharREF _asthird_person_character)
  (switch Utilities|FlowControl|Switch|SwitchonSurfaces_Enum (Variables|Default|GetSurface)
    (:NewEnumerator0
      (Variables|/Game/ThirdPersonBP/Blueprints/ThirdPersonCharacter.ThirdPersonCharacter_C|SetRunSpeed (Variables|Default|GetCharREF) _fastrun)
      (Variables|/Game/ThirdPersonBP/Blueprints/ThirdPersonCharacter.ThirdPersonCharacter_C|SetWalk%20Speed (Variables|Default|GetCharREF) _fastwalk)
      (if (Variables|/Game/ThirdPersonBP/Blueprints/ThirdPersonCharacter.ThirdPersonCharacter_C|GetIsRunning (Variables|Default|GetCharREF))
        (Variables|/Script/Engine.CharacterMovementComponent|SetMaxWalkSpeed (Variables|/Script/Engine.Character|GetCharacterMovement (Variables|Default|GetCharREF)) _fastrun_2)
        (else
          (Variables|/Script/Engine.CharacterMovementComponent|SetMaxWalkSpeed (Variables|/Script/Engine.Character|GetCharacterMovement (Variables|Default|GetCharREF)) _fastwalk_2))))
    (:NewEnumerator1
      (Variables|/Game/ThirdPersonBP/Blueprints/ThirdPersonCharacter.ThirdPersonCharacter_C|SetRunSpeed (Variables|Default|GetCharREF) _slowrun)
      (Variables|/Game/ThirdPersonBP/Blueprints/ThirdPersonCharacter.ThirdPersonCharacter_C|SetWalk%20Speed (Variables|Default|GetCharREF) _slowwalk)
      (if (Variables|/Game/ThirdPersonBP/Blueprints/ThirdPersonCharacter.ThirdPersonCharacter_C|GetIsRunning (Variables|Default|GetCharREF))
        (Variables|/Script/Engine.CharacterMovementComponent|SetMaxWalkSpeed (Variables|/Script/Engine.Character|GetCharacterMovement (Variables|Default|GetCharREF)) _slowrun_2)
        (else
          (Variables|/Script/Engine.CharacterMovementComponent|SetMaxWalkSpeed (Variables|/Script/Engine.Character|GetCharacterMovement (Variables|Default|GetCharREF)) _slowwalk_2))))))

(event OnComponentEndOverlap(Box)
  (params (OverlappedComponent :type Primitive%20Component%20Object%20Reference) (OtherActor :type Actor%20Object%20Reference) (OtherComp :type Primitive%20Component%20Object%20Reference) (OtherBodyIndex :type Integer))
  (bind _asthird_person_character (Utilities|Casting|CastToThirdPersonCharacter OtherActor))
  (Variables|/Game/ThirdPersonBP/Blueprints/ThirdPersonCharacter.ThirdPersonCharacter_C|SetRunSpeed _asthird_person_character (Variables|Default|GetNormRunSpeed))
  (Variables|/Game/ThirdPersonBP/Blueprints/ThirdPersonCharacter.ThirdPersonCharacter_C|SetWalk%20Speed _asthird_person_character (Variables|Default|GetNormWalkSpeed))
  (if (Variables|/Game/ThirdPersonBP/Blueprints/ThirdPersonCharacter.ThirdPersonCharacter_C|GetIsRunning _asthird_person_character)
    (Variables|/Script/Engine.CharacterMovementComponent|SetMaxWalkSpeed (Variables|/Script/Engine.Character|GetCharacterMovement _asthird_person_character) (Variables|Default|GetNormRunSpeed))
    (else
      (Variables|/Script/Engine.CharacterMovementComponent|SetMaxWalkSpeed (Variables|/Script/Engine.Character|GetCharacterMovement _asthird_person_character) (Variables|Default|GetNormWalkSpeed)))))

(event EventBeginPlay
  (bind _asthird_person_character (Utilities|Casting|CastToThirdPersonCharacter (Game|GetPlayerCharacter 0)))
  (Variables|Default|SetNormRunSpeed (Variables|/Game/ThirdPersonBP/Blueprints/ThirdPersonCharacter.ThirdPersonCharacter_C|GetRunSpeed _asthird_person_character))
  (Variables|Default|SetNormWalkSpeed (Variables|/Game/ThirdPersonBP/Blueprints/ThirdPersonCharacter.ThirdPersonCharacter_C|GetWalk%20Speed _asthird_person_character))
  (Rendering|Material|SetMaterial (Variables|Default|GetPlane) 0 (Variables|Default|GetMaterial)))

(fn ConstructionScript)