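; BP_Spikes is a trap prop that rises and deals damage after the ThirdPersonCharacter enters its box.
; After a delay, timelines lerp the spikes to the Up marker, then back to Down, with a DoOnce gating each cycle.
; Radial damage, ignoring all BP_BaseEnemy actors, fires when fully raised.
; Entering while raised also triggers damage, throttled by a briefly delayed DoOnce reset.
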(event OnComponentBeginOverlap(Box)
  (params (OverlappedComponent :type Primitive%20Component%20Object%20Reference) (OtherActor :type Actor%20Object%20Reference) (OtherComp :type Primitive%20Component%20Object%20Reference) (OtherBodyIndex :type Integer) (bFromSweep :type Boolean) (SweepResult :type Hit%20Result%20Structure%20%28by%20ref%29))
  (bind _asthird_person_character (Utilities|Casting|CastToThirdPersonCharacter OtherActor))
  (Variables|Default|SetCharREF _asthird_person_character)
  (if (Variables|Default|GetIsActive)
    (Utilities|FlowControl|DoOnce false :!label _label
      (:Completed
        (bind _outactors (Actor|GetAllActorsOfClass "/Game/Blueprints/Enemies/BaseEnemy/BP_BaseEnemy.BP_BaseEnemy_C"))
        (Game|Damage|ApplyRadialDamage (Variables|Default|GetDamage) (Transformation|GetWorldLocation (Variables|Default|GetSpikes)) 1e+02 0 _outactors self 0 true "ECC_Visibility")
        (Utilities|FlowControl|Delay 0.1)
        (goto _label Reset)))
    (else
      (CallFunction|Activate))))

(event Custom|Activate
  (bind _spikes (Variables|Default|GetSpikes))
  (bind _spikes_2 (Variables|Default|GetSpikes))
  (bind _returnvalue (Transformation|GetWorldLocation _spikes_2))
  (bind _returnvalue_2 (Transformation|GetWorldLocation _spikes))
  (Utilities|FlowControl|Delay 1.0)
  (Utilities|FlowControl|DoOnce false :!label _label
    (:Completed
      (bind _alpha (Timeline|MoveSpikes PlayFromStart)
        (:Update
          (Transformation|SetWorldLocation _spikes_2 (Math|Vector|MakeVector (.x _returnvalue) (.y _returnvalue) (Math|Float|Lerp (.z _returnvalue) (.z (Transformation|GetWorldLocation (Variables|Default|GetUp))) _alpha)) false false))
        (:Finished
          (Variables|Default|SetIsActive true)
          (bind _outactors (Actor|GetAllActorsOfClass "/Game/Blueprints/Enemies/BaseEnemy/BP_BaseEnemy.BP_BaseEnemy_C"))
          (Game|Damage|ApplyRadialDamage (Variables|Default|GetDamage) (Transformation|GetWorldLocation (Variables|Default|GetSpikes)) 1e+02 0 _outactors self 0 true "ECC_Visibility")
          (Utilities|FlowControl|Delay 1.0)
          (bind _alpha_2 (Timeline|MoveAway PlayFromStart)
            (:Update
              (Transformation|SetWorldLocation _spikes (Math|Vector|MakeVector (.x _returnvalue_2) (.y _returnvalue_2) (Math|Float|Lerp (.z _returnvalue_2) (.z (Transformation|GetWorldLocation (Variables|Default|GetDown))) _alpha_2)) false false))
            (:Finished
              (Variables|Default|SetIsActive false)
              (goto _label Reset))))))))

(fn ConstructionScript)