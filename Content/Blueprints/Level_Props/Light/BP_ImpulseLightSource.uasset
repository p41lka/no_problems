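; A light prop that sends a light pulse travelling between two points, either once or on a repeating loop.
; BeginPlay turns the start and end offsets into world positions at the actor's height, fires SendLight and scales the timeline's play rate to last the configured seconds.
; SendLight, also meant for triggers, shows the light, lerps LightRadius along the path, then hides it and, if looped, pauses before repeating.
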(event Custom|SendLight
  ;[0 0 0] Move timeline (call this event for light on triggers)
  (CallFunction|AppearDisappear true)
  (bind _alpha (Timeline|MoveLight PlayFromStart)
    (:Update
      (Transformation|SetWorldLocation (Variables|Default|GetLightRadius) (Math|Vector|Lerp(Vector) (Variables|Default|GetStartLocation) (Variables|Default|GetEndLocation) _alpha) false false))
    (:Finished
      (Utilities|FlowControl|Delay 0.1)
      (CallFunction|AppearDisappear false)
      (if (Variables|Default|Getislooped)
        (Utilities|FlowControl|Delay (Variables|Default|GetpauseTime))
        (CallFunction|SendLight)))))

(event EventBeginPlay
  (bind _returnvalue (Transformation|GetActorLocation))
  (bind _z (Math|Vector|BreakVector _returnvalue))
  (|CallParentFunction)
  (Variables|Default|SetStartLocation (Math|Vector|MakeVector (.x (+ _returnvalue (Variables|Default|GetStartLocation))) (.y (+ _returnvalue (Variables|Default|GetStartLocation))) _z))
  (Variables|Default|SetEndLocation (Math|Vector|MakeVector (.x (+ _returnvalue (Variables|Default|GetEndLocation))) (.y (+ _returnvalue (Variables|Default|GetEndLocation))) _z))
  (CallFunction|SendLight)
  (Components|Timeline|SetPlayRate (Variables|Default|GetMoveLight) (/ (Components|Timeline|GetTimelineLength (Variables|Default|GetMoveLight)) (Variables|Default|Getseconds))))

(fn ConstructionScript
  (|CallParentFunction))