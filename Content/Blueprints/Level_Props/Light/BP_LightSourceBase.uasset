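; Base light source prop that periodically damages enemies in its radius and can be drained by the player for extra ammo.
; LightBaseStruct drives the radius scale, a looping damage timer over overlapping BP_BaseEnemy actors, and the charge amount.
; InteractionRadius toggles the prompt widget; Interact adds clamped ammo, then permanently turns the light off, stopping damage.
; Isolated lights still deal damage but disable interaction.
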(event OnComponentBeginOverlap(InteractionRadius)
  (params (OverlappedComponent :type Primitive%20Component%20Object%20Reference) (OtherActor :type Actor%20Object%20Reference) (OtherComp :type Primitive%20Component%20Object%20Reference) (OtherBodyIndex :type Integer) (bFromSweep :type Boolean) (SweepResult :type Hit%20Result%20Structure%20%28by%20ref%29))
  ;[0 0 0] Interaction and isolation
  (if (Variables|Default|GetisActive)
    (Utilities|Casting|CastToThirdPersonCharacter OtherActor)
    (Rendering|SetVisibility (Variables|Default|GetInteractionWidget) true false)))

(event OnComponentEndOverlap(InteractionRadius)
  (params (OverlappedComponent :type Primitive%20Component%20Object%20Reference) (OtherActor :type Actor%20Object%20Reference) (OtherComp :type Primitive%20Component%20Object%20Reference) (OtherBodyIndex :type Integer))
  ;[0 0 0] Interaction and isolation
  (if (Variables|Default|GetisActive)
    (Utilities|Casting|CastToThirdPersonCharacter OtherActor)
    (Rendering|SetVisibility (Variables|Default|GetInteractionWidget) false false)))

(event Custom|DamageEnemies
  ;[0 0 0] Damage enemies with light
  (for _array_element (Collision|GetOverlappingActors (Variables|Default|GetLightRadius) "/Game/Blueprints/Enemies/BaseEnemy/BP_BaseEnemy.BP_BaseEnemy_C" :!class /Script/Engine.PrimitiveComponent)
    (Game|Damage|ApplyDamage _array_element (.damage (Utilities|Struct|BreakLightSourcesInfo_Struct (Variables|Default|GetlightBaseStruct))) 0 0)))

(event Custom|TurnOff
  ;[0 0 0] Interaction and isolation
  (Variables|Default|SetisActive false)
  (Rendering|Material|SetMaterial (Variables|Default|GetStaticMesh) 0 "/Game/Materials/M_Unlit/M_Blue.M_Blue")
  (Utilities|Time|ClearandInvalidateTimerbyHandle (Variables|Default|GetlightDamageTimer))
  (Rendering|SetVisibility (Variables|Default|GetInteractionWidget) false false)
  (CallFunction|AppearDisappear false))

(event Custom|StartDamageEnemies
  ;[0 0 0] Damage enemies with light
  (bind _returnvalue (Utilities|Time|SetTimerbyEvent (delegate Custom|DamageEnemies) (.damageTime (Utilities|Struct|BreakLightSourcesInfo_Struct (Variables|Default|GetlightBaseStruct))) true))
  (Variables|Default|SetlightDamageTimer _returnvalue))

(event Custom|AppearDisappear
  (params (is%20working :type Boolean))
  ;[0 0 0] Disable or enable light for time
  (Collision|SetCollisionEnabled (Variables|Default|GetLightRadius) (select is%20working "QueryOnly" "NoCollision"))
  (Rendering|SetVisibility (Variables|Default|GetLightRadius) is%20working true))

(event Custom|AddAmmo
  (bind _charref (Variables|Default|GetcharRef))
  ;[0 0 0] ammo for char (probably should create this in character)
  (Variables|/Game/ThirdPersonBP/Blueprints/ThirdPersonCharacter.ThirdPersonCharacter_C|SetCurrentDopAmmo _charref (Math|Integer|Clamp(Integer) (+ (.chargeAmount (Utilities|Struct|BreakLightSourcesInfo_Struct (Variables|Default|GetlightBaseStruct))) (Variables|/Game/ThirdPersonBP/Blueprints/ThirdPersonCharacter.ThirdPersonCharacter_C|GetCurrentDopAmmo _charref)) 0 (Variables|/Game/ThirdPersonBP/Blueprints/ThirdPersonCharacter.ThirdPersonCharacter_C|GetMaxDopAmmo _charref))))

(event EventBeginPlay
  (bind _lightbasestruct (Variables|Default|GetlightBaseStruct))
  (bind (_isisolated _damageradius) (Utilities|Struct|BreakLightSourcesInfo_Struct _lightbasestruct))
  (Transformation|SetWorldScale3D (Variables|Default|GetLightRadius) (Math|Conversions|ToVector(Float) _damageradius))
  (Variables|Default|SetisActive (not _isisolated))
  (CallFunction|StartDamageEnemies)
  (if (.isIsolated (Utilities|Struct|BreakLightSourcesInfo_Struct (Variables|Default|GetlightBaseStruct)))
    (Collision|SetCollisionEnabled (Variables|Default|GetInteractionRadius) "NoCollision") ; no interaction if isolated
    (else
      (bind _asthird_person_character (Utilities|Casting|CastToThirdPersonCharacter (Game|GetPlayerCharacter 0)))
      (Variables|Default|SetcharRef _asthird_person_character))))

(fn ConstructionScript)

(fn Interact
  (bind _charref (Variables|Default|GetcharRef))
  (if (Math|Boolean|ANDBoolean (Collision|IsOverlappingActor (Variables|Default|GetInteractionRadius) (Game|GetPlayerCharacter 0) :!class /Script/Engine.PrimitiveComponent) (Variables|Default|GetisActive) (< (Variables|/Game/ThirdPersonBP/Blueprints/ThirdPersonCharacter.ThirdPersonCharacter_C|GetCurrentDopAmmo _charref) (Variables|/Game/ThirdPersonBP/Blueprints/ThirdPersonCharacter.ThirdPersonCharacter_C|GetMaxDopAmmo _charref)))
    (CallFunction|AddAmmo)
    (CallFunction|TurnOff)
    (return true)
    (else
      (return false))))