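; Laser light source prop that fires a stretching beam to damage what it touches.
; The Attack timeline scales and shifts the Plane to grow the beam, dealing attack damage to any actor entering LightLine meanwhile.
; Once extended, a looping timer damages overlapping BP_BaseEnemy actors, and a second timer limits the beam's lifetime.
; Ending disables collision and visibility, then either refires after a delay when looping and active, or turns off.
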(event OnComponentBeginOverlap(LightLine)
  (params (OverlappedComponent :type Primitive%20Component%20Object%20Reference) (OtherActor :type Actor%20Object%20Reference) (OtherComp :type Primitive%20Component%20Object%20Reference) (OtherBodyIndex :type Integer) (bFromSweep :type Boolean) (SweepResult :type Hit%20Result%20Structure%20%28by%20ref%29))
  ;[0 0 0] Draw light line
  (if (Variables|Default|GetisAttacking)
    (Game|Damage|ApplyDamage OtherActor (.DamageAttack (Utilities|Struct|BreakLazerLightSourcesInfo_Struct (Variables|Default|GetlazerLightStruct))) 0 0)))

(event Custom|LazerAttack
  (bind _lazerlightstruct (Variables|Default|GetlazerLightStruct))
  (bind _plane (Variables|Default|GetPlane))
  (bind (_damageattack _width _height _length) (Utilities|Struct|BreakLazerLightSourcesInfo_Struct _lazerlightstruct))
  ;[0 0 0] Start Lazer
  (if (Variables|Default|GetisActive)
    (CallFunction|AppearDisappear true)
    (Variables|Default|SetisAttacking true)
    (Rendering|SetVisibility (Variables|Default|GetPlane) true false)
    (bind _lerpe (Timeline|Attack PlayFromStart)
      (:Update
        (Transformation|SetRelativeScale3D _plane (Math|Vector|MakeVector (Math|Float|Lerp 0.0 _length _lerpe) _width _height))
        (Transformation|SetRelativeLocation _plane (Math|Vector|MakeVector (* (Math|Float|Lerp 0.0 _length _lerpe) 5e+01) 0.0 0.0) false false))
      (:Finished
        (CallFunction|StartDamageEnemies)
        (Variables|Default|SetisAttacking false)))))

(event Custom|Ending
  (bind _lazerlightstruct (Variables|Default|GetlazerLightStruct))
  (bind (_damageattack _width _height _length _timelightexist _isloop _delay) (Utilities|Struct|BreakLazerLightSourcesInfo_Struct _lazerlightstruct))
  ;[0 0 0] stop or continue work
  (CallFunction|AppearDisappear false)
  (if (and _isloop (Variables|Default|GetisActive))
    (Utilities|FlowControl|Delay _delay)
    (CallFunction|LazerAttack)
    (else
      (CallFunction|TurnOff))))

(event EventTurnOff
  ;[0 0 0] stop or continue work
  (Audio|Components|Audio|Stop (Variables|Default|GetAttack))
  (|CallParentFunction))

(event EventBeginPlay
  (|CallParentFunction)
  (CallFunction|LazerAttack))

(event EventStartDamageEnemies
  ;[0 0 0] Draw light line
  (bind _returnvalue (Utilities|Time|SetTimerbyEvent (delegate EventDamageEnemies) (.damageTime (Utilities|Struct|BreakLightSourcesInfo_Struct (Variables|Default|GetlightBaseStruct))) true))
  (Variables|Default|SetlightDamageTimer _returnvalue)
  (Utilities|Time|SetTimerbyEvent (EventDispatchers|CreateEvent :!event Custom|Ending) (.timelightexist (Utilities|Struct|BreakLazerLightSourcesInfo_Struct (Variables|Default|GetlazerLightStruct)))))

(event EventDamageEnemies
  ;[0 0 0] Draw light line
  (for _array_element (Collision|GetOverlappingActors (Variables|Default|GetLightLine) "/Game/Blueprints/Enemies/BaseEnemy/BP_BaseEnemy.BP_BaseEnemy_C" :!class /Script/Engine.PrimitiveComponent)
    (Game|Damage|ApplyDamage _array_element (.damage (Utilities|Struct|BreakLightSourcesInfo_Struct (Variables|Default|GetlightBaseStruct))) 0 0)))

(event EventAppearDisappear
  (params (is%20working :type Boolean))
  ;[0 0 0] stop or continue work
  (Collision|SetCollisionEnabled (Variables|Default|GetLightLine) (select is%20working "QueryOnly" "NoCollision"))
  (Rendering|SetVisibility (Variables|Default|GetPlane) false false))

(fn ConstructionScript
  (|CallParentFunction))