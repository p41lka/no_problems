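; A destructible light source prop that loses health to nearby enemies and regenerates over time, extending a parent light class.
; Looping timers drain health per BP_BaseEnemy overlapping its damage sphere and restore a set amount, using struct-driven tuning.
; Health percentage scales the LightRadius component, and below half a Flash timeline flip-flops the mesh material as a warning.
; At zero health it turns off, clearing its timers and setting the blue material.
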(event Custom|GetDamage
  ;[0 0 0] Damage and regeneration
  (CallFunction|ChangeHealth (* (* (Utilities|Array|Length (Collision|GetOverlappingActors (Variables|Default|GetGetDamageSphere) "/Game/Blueprints/Enemies/BaseEnemy/BP_BaseEnemy.BP_BaseEnemy_C" :!class /Script/Engine.PrimitiveComponent)) (.getDamageAmount (Utilities|Struct|BreakLightSourcesNormalInfo_Struct (Variables|Default|GetnormalLightStruct)))) -1.0))
  (CallFunction|ChangeLightRadius)
  (CallFunction|CheckHealth))

(event Custom|Regenerate
  ;[0 0 0] Damage and regeneration
  (CallFunction|ChangeHealth (.RegenerationAmount (Utilities|Struct|BreakLightSourcesNormalInfo_Struct (Variables|Default|GetnormalLightStruct))))
  (CallFunction|ChangeLightRadius)
  (CallFunction|CheckHealth))

(event Custom|ChangeLightRadius
  ;[0 0 0] Change forms and effects
  (Transformation|SetWorldScale3D (Variables|Default|GetLightRadius) (Math|Conversions|ToVector(Float) (* (+ 0.5 (/ (CallFunction|GetHealthPercent) 2.0)) (.damageRadius (Utilities|Struct|BreakLightSourcesInfo_Struct (Variables|Default|GetlightBaseStruct)))))))

(event Custom|ChangeHealth
  (params (amount :type Float%20%28double-precision%29))
  ;[0 0 0] Damage and regeneration
  (Variables|Default|Sethealth (Math|Float|Clamp(Float) (+ amount (Variables|Default|Gethealth)) 0.0 (.MaxHealth (Utilities|Struct|BreakLightSourcesNormalInfo_Struct (Variables|Default|GetnormalLightStruct))))))

(event Custom|CheckHealth
  (bind _healtpercent (CallFunction|GetHealthPercent))
  ;[0 0 0] Change forms and effects
  (if (== _healtpercent 0.0)
    (CallFunction|TurnOff)
    (elif (>= _healtpercent 0.5)
      (Audio|Components|Audio|Stop (Variables|Default|GetFlash))
      (Rendering|Material|SetMaterial (Variables|Default|GetStaticMesh) 0 "/Game/Materials/M_Blockouts/MATERIALS/GLOWY_WIRES.GLOWY_WIRES")
      (else
        (Timeline|Flash PlayFromStart
          (:Flash
            (Utilities|FlowControl|FlipFlop
              (:A
                (Rendering|Material|SetMaterial (Variables|Default|GetStaticMesh) 0 "/Game/Materials/M_Unlit/M_Blue.M_Blue"))
              (:B
                (Rendering|Material|SetMaterial (Variables|Default|GetStaticMesh) 0 "/Game/Materials/M_Blockouts/MATERIALS/GLOWY_WIRES.GLOWY_WIRES")))))))))

(event EventBeginPlay
  (bind _normallightstruct (Variables|Default|GetnormalLightStruct))
  (bind (_maxhealth _getdamageradius _getdamageamount _getdamagetime _regenerationamount _regenerationtime) (Utilities|Struct|BreakLightSourcesNormalInfo_Struct _normallightstruct))
  (|CallParentFunction)
  (Transformation|SetWorldScale3D (Variables|Default|GetGetDamageSphere) (Math|Conversions|ToVector(Float) _getdamageradius))
  (Variables|Default|Sethealth _maxhealth)
  (bind _returnvalue (Utilities|Time|SetTimerbyEvent (EventDispatchers|CreateEvent :!event Custom|GetDamage) _getdamagetime true))
  (Variables|Default|SetgetDamageTimer _returnvalue)
  (bind _returnvalue_2 (Utilities|Time|SetTimerbyEvent (EventDispatchers|CreateEvent :!event Custom|Regenerate) _regenerationtime true))
  (Variables|Default|SetregenTimer _returnvalue_2))

(event EventTurnOff
  (bind _flash (Variables|Default|GetFlash))
  ;[0 0 0] Change forms and effects
  (|CallParentFunction)
  (for _array_element (Utilities|Array|MakeArray (Variables|Default|GetlightDamageTimer) (Variables|Default|GetregenTimer) (Variables|Default|GetgetDamageTimer))
    (Utilities|Time|ClearandInvalidateTimerbyHandle _array_element)
    (Rendering|Material|SetMaterial (Variables|Default|GetStaticMesh) 0 "/Game/Materials/M_Unlit/M_Blue.M_Blue")
    (Utilities|IsValid _flash
      (:Is%20Valid
        (Audio|Components|Audio|Stop _flash)))))

(fn ConstructionScript
  (|CallParentFunction))

(fn GetHealthPercent
  (return (/ (Variables|Default|Gethealth) (.MaxHealth (Utilities|Struct|BreakLightSourcesNormalInfo_Struct (Variables|Default|GetnormalLightStruct))))))