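; Enemy with a Faith aspect that lends the player an aspect-based ability through proximity resonance.
; Entering its collision lights the radius and starts a looping timer that, once charged, grants the matching ability.
; Leaving resets the player's abilities, starting a Tick-driven reload if one was earned.
; Damage can destroy it; a timer-driven projectile attack exists but its call is disconnected.
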(event OnComponentBeginOverlap(ResonanceCollision)
  (params (OverlappedComponent :type Primitive%20Component%20Object%20Reference) (OtherActor :type Actor%20Object%20Reference) (OtherComp :type Primitive%20Component%20Object%20Reference) (OtherBodyIndex :type Integer) (bFromSweep :type Boolean) (SweepResult :type Hit%20Result%20Structure%20%28by%20ref%29))
  (bind _asthird_person_character (Utilities|Casting|CastToThirdPersonCharacter OtherActor))
  (Variables|Default|SetCharacterREF _asthird_person_character)
  (Rendering|Material|SetMaterial (Variables|Default|GetResonanceRadius) 0 "/Game/Materials/M_Enemies/M_Circle_Emissive.M_Circle_Emissive")
  (Variables|Default|SetIsResonating true)
  ;[0 0 0] Resonance Timer
  (bind _returnvalue (Utilities|Time|SetTimerbyEvent (delegate Custom|Resonance) 0.5 true))
  (Variables|Default|SetResTimer _returnvalue))

(event OnComponentEndOverlap(ResonanceCollision)
  (params (OverlappedComponent :type Primitive%20Component%20Object%20Reference) (OtherActor :type Actor%20Object%20Reference) (OtherComp :type Primitive%20Component%20Object%20Reference) (OtherBodyIndex :type Integer))
  (Utilities|Casting|CastToThirdPersonCharacter OtherActor)
  (Rendering|Material|SetMaterial (Variables|Default|GetResonanceRadius) 0 "/Game/Materials/M_Enemies/M_Circle.M_Circle")
  (Variables|Default|SetIsResonating false)
  (if (Variables|Default|GetCanUseAbility)
    (Variables|Default|SetIsReloading true))
  (Default|ResetAbilities (Variables|Default|GetCharacterREF)))

(event Custom|Resonance
  (bind _characterref (Variables|Default|GetCharacterREF))
  ;[0 0 0] Resonance Timer
  (if (not (Variables|Default|GetIsReloading))
    (if (< (Variables|Default|GetCurrentTime) (Variables|Default|GetResonanceTime))
      (bind _result (Math|Float|IncrementFloat (Variables|Default|GetCurrentTime))
        (:%20%20
          (Development|PrintString (Utilities|String|ToString(Float) _result) true true "(R=0.051790,G=0.608333,B=0.000000,A=1.000000)" 0.1)
          (if (>= (Variables|Default|GetCurrentTime) (Variables|Default|GetResonanceTime))
            (Variables|Default|SetCanUseAbility true)
            ;;[0 0 0] Set ability from enemy aspect
            (switch Utilities|FlowControl|Switch|SwitchonEnemyAspects_Enum (Variables|Aspects|GetEnemyAspects)
              (:NewEnumerator0
                (Default|SetFaithAbility _characterref))
              (:NewEnumerator1
                (Default|SetDestructionAbility _characterref))
              (:NewEnumerator2
                (Default|SetBondAbility _characterref))
              (:NewEnumerator3
                (Default|SetRenewalAbility _characterref))))))
      (else
        (Utilities|Time|ClearandInvalidateTimerbyHandle (Variables|Default|GetResTimer))
        (Variables|Default|SetCurrentTime 0.0)
        (Variables|Default|SetCanUseAbility false)))))

(event Custom|PassiveAttack
  ;[0 0 0] Spawn Projectiles
  (bind _returnvalue (Utilities|Time|SetTimerbyEvent (delegate Custom|PassiveAttackSpawn) 0.4 true))
  (Variables|Default|SetAttackTimer _returnvalue))

(event Custom|PassiveAttackSpawn
  (bind _attackspawn (Variables|Default|GetAttackSpawn))
  ;[0 0 0] Spawn Projectiles
  (Game|SpawnActorfromClass "/Game/Blueprints/Projectiles/BP_EnemyProjectiles.BP_EnemyProjectiles_C" (Math|Transform|MakeTransform (Transformation|GetWorldLocation _attackspawn) (Transformation|GetWorldRotation _attackspawn) "0.500000,0.500000,0.500000") "Undefined" 0 0))

(event EventTick
  (params (DeltaSeconds :type Float%20%28single-precision%29))
  ;[0 0 0] Reload Timer
  (if (Variables|Default|GetIsReloading)
    (bind _output_get (Variables|Default|SetCurrentReloadTime (+ (Variables|Default|GetCurrentReloadTime) DeltaSeconds)))
    (Development|PrintString (Utilities|String|ToString(Float) _output_get) true true "(R=1.000000,G=0.784818,B=0.000000,A=1.000000)" 0.0)
    (if (< _output_get (Variables|Default|GetReloadTime))
      (Variables|Default|SetIsReloading true)
      (else
        (Variables|Default|SetIsReloading false)
        (Variables|Default|SetCurrentReloadTime 0.0)))
    (else
      (Variables|Default|SetCurrentReloadTime 0.0))))

(event Game|Damage|EventAnyDamage
  (params (Damage :type Float%20%28single-precision%29) (DamageType :type Damage%20Type%20Object%20Reference) (InstigatedBy :type Controller%20Object%20Reference) (DamageCauser :type Actor%20Object%20Reference))
  ;[0 0 0] Damage
  (bind _output_get (Variables|Default|SetCurrentHealth (- (Variables|Default|GetCurrentHealth) Damage)))
  (if (not (> _output_get 0.0))
    (Actor|DestroyActor)
    (Variables|/Game/ThirdPersonBP/Blueprints/ThirdPersonCharacter.ThirdPersonCharacter_C|SetCurrentAbility (Variables|Default|GetCharacterREF) "NewEnumerator4")))

(event EventBeginPlay
  (Variables|Default|SetCurrentHealth (Variables|Default|GetMaxHealth))
  ;[1 1 1] Set Enemy Aspect
  (Variables|Aspects|SetEnemyAspects "NewEnumerator0"))

(fn ConstructionScript)